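; BP_Payload_Stop_Trigger is a one-shot trigger that halts the co-op payload once enough actors have left its volume.
; Shortly after BeginPlay it caches the player list from BP_ThirdPersonGameMode.
; Each unique actor ending overlap is recorded, without a player filter.
; When that count equals the player count, it zeroes BP_Payload's speed through SlowPayload, deactivates it and destroys itself.
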(event `self.ReceiveBeginPlay`
  (`KismetSystemLibrary.Delay` 0.2)
  (bind _asbp_third_person_game_mode (cast `/Game/Modes_Instances/Modes/BP_ThirdPersonGameMode` (`GameplayStatics.GetGameMode`)))
  (bind _output_get (set `self.As BP Third Person Game Mode` _asbp_third_person_game_mode))
  (set `self.Players` (`/Game/Modes_Instances/Modes/BP_ThirdPersonGameMode.Players` _output_get)))

(event `self.Trigger.OnComponentEndOverlap`
  (params (OverlappedComponent :type "PrimitiveComponent Object Reference") (OtherActor :type "Actor Object Reference") (OtherComp :type "PrimitiveComponent Object Reference") (OtherBodyIndex :type Integer))
  (if (not (`KismetArrayLibrary.Array_Contains` (`self.Players Triggered`) OtherActor))
    (`KismetArrayLibrary.Array_Add` (`self.Players Triggered`) OtherActor)
    (if (== (`KismetArrayLibrary.Array_Length` (`self.Players Triggered`)) (`KismetArrayLibrary.Array_Length` (`self.Players`)))
      (bind _returnvalue (`GameplayStatics.GetActorOfClass` "/Game/Co-op/Payload/BP_Payload.BP_Payload_C"))
      (`/Game/Co-op/Payload/BP_Payload.Slow Payload` _returnvalue false 0.0 0.0)
      (`/Game/Co-op/Payload/BP_Payload.Update Active` _returnvalue false)
      (`self.K2_DestroyActor`))))

(fn `UserConstructionScript`)