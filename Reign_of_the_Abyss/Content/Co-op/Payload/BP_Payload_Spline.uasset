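; Spline path actor for the co-op payload, exposing world-space queries for placing and orienting actors along the route.
; It finds an actor's closest spline location and rounded point index, or its distance along the spline.
; Other helpers convert a distance to location or rotation and an index to a point location.
; The index updater increments, returning zero only when the current index already exceeds the point count.
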(fn `Find Starting Loc`
  (params (Actor :type "Actor Object Reference"))
  (returns (`Starting Loc` :type "Vector Structure") (`Spline Index` :type Integer))
  (return (`SplineComponent.FindLocationClosestToWorldLocation` (`self.Spline`) (`self.K2_GetActorLocation` Actor) "World") (`KismetMathLibrary.Round` (`SplineComponent.FindInputKeyClosestToWorldLocation` (`self.Spline`) (`self.K2_GetActorLocation` (`local.Actor`))))))

(fn `Get Distance Along Spline`
  (params (Actor :type "Actor Object Reference"))
  (returns (`Distance Along Spline` :type "Float (double-precision)"))
  (return (`SplineComponent.GetDistanceAlongSplineAtLocation` (`self.Spline`) (`self.K2_GetActorLocation` Actor) "World")))

(fn `Get Nearest Location`
  (params (`Distance Along Spline` :type "Float (double-precision)"))
  (returns (`Tarrget Loc` :type "Vector Structure"))
  (return (`SplineComponent.GetLocationAtDistanceAlongSpline` (`self.Spline`) `Distance Along Spline` "World")))

(fn `Get Nearest Spline Point`
  (params (`Current Spline Index` :type Integer))
  (returns (Location :type "Vector Structure"))
  (return (`SplineComponent.GetLocationAtSplinePoint` (`self.Spline`) `Current Spline Index` "World")))

(fn `Get Rotation At Distance`
  (params (Distance :type "Float (double-precision)"))
  (returns (Rotation :type "Rotator Structure"))
  (return (`SplineComponent.GetRotationAtDistanceAlongSpline` (`self.Spline`) Distance "World")))

(fn `Update Spline Index`
  (params (`Current Spline Index` :type Integer))
  (returns (`New Spline Index` :type Integer))
  (return (`KismetMathLibrary.SelectInt` 0 (+ `Current Spline Index` 1) (> `Current Spline Index` (`SplineComponent.GetNumberOfSplinePoints` (`self.Spline`))))))

(fn `UserConstructionScript`)