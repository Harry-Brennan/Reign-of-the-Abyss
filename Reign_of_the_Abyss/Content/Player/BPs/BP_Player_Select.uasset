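; Player pawn for the main menu character select, previewing one player's character and weapons into one of four render targets chosen by actor tag.
; The capture's show-only list isolates the pawn and its weapons, and look input yaws the spring arm.
; Join input registers the player with the select widget once until reset.
; UpdateCharacter reloads mesh and weapons from the character data table and refreshes that list.
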(event `self.ReceiveBeginPlay`
  (`KismetSystemLibrary.Delay` 0.2)
  (switch `name` (`|GetArrayItem` (`self.Tags`))
    (:`0`
      (set `SceneCaptureComponent2D.TextureTarget` "/Game/UI/Screens/Character_Select/Render_Targets/RT_Player_Select_1.RT_Player_Select_1" (`self.Render Target`)))
    (:`1`
      (set `SceneCaptureComponent2D.TextureTarget` "/Game/UI/Screens/Character_Select/Render_Targets/RT_Player_Select_2.RT_Player_Select_2" (`self.Render Target`)))
    (:`2`
      (set `SceneCaptureComponent2D.TextureTarget` "/Game/UI/Screens/Character_Select/Render_Targets/RT_Player_Select_3.RT_Player_Select_3" (`self.Render Target`)))
    (:`3`
      (set `SceneCaptureComponent2D.TextureTarget` "/Game/UI/Screens/Character_Select/Render_Targets/RT_Player_Select_4.RT_Player_Select_4" (`self.Render Target`))))
  (bind _output_get (set `SceneCaptureComponent.ShowOnlyActors` (`|MakeArray` self :!type "Actor Object Reference") (`self.Render Target`)))
  (set `self.Show Only List` _output_get)
  (`self.Update Show Only List` (`|MakeArray` (`self.Equipped Ranged Weapon`) (`self.Equipped Melee Weapon`) :!type "Actor Object Reference"))
  (bind _asplayer_controller (cast `PlayerController` (`self.GetController`)))
  (bind _returnvalue (pcsubsystem `EnhancedInputLocalPlayerSubsystem` _asplayer_controller))
  (`/Engine/EditorBlueprintResources/StandardMacros.IsValid` _returnvalue
    (:`Is Valid`
      (`EnhancedInputSubsystemInterface.AddMappingContext` _returnvalue "/Game/Player/Input/IMCs/IMC_Character_Select.IMC_Character_Select" 0 (struct)))))

(event `EnhancedInput|/Game/Player/Input/Actions/IA_Look_Controller`
  (params (ActionValue :type "Vector2D Structure") (ElapsedSeconds :type "Float (double-precision)") (TriggeredSeconds :type "Float (double-precision)") (InputAction :type "InputAction Object Reference" :default "/Game/Player/Input/Actions/IA_Look_Controller.IA_Look_Controller"))
  (:`Triggered`
    (`SceneComponent.K2_AddRelativeRotation` (`self.SpringArm`) (`KismetMathLibrary.MakeRotator` 0.0 0.0 (* ActionValue_X 3.0)) false false)))

(event `EnhancedInput|/Game/Player/Input/Actions/IA_Look`
  (params (ActionValue :type "Vector2D Structure") (ElapsedSeconds :type "Float (double-precision)") (TriggeredSeconds :type "Float (double-precision)") (InputAction :type "InputAction Object Reference" :default "/Game/Player/Input/Actions/IA_Look.IA_Look"))
  (:`Triggered`
    (`SceneComponent.K2_AddRelativeRotation` (`self.SpringArm`) (`KismetMathLibrary.MakeRotator` 0.0 0.0 (* ActionValue_X 3.0)) false false)))

(event `/Game/Combat/Interfaces/BPI_Has_Weapon.Set_Equipped_Melee_Weapon`
  (params (`Weapon Parent` :type "/Game/Combat/Weapons/BPs/BP_WeaponParent Object Reference"))
  (set `self.Equipped Melee Weapon` `Weapon Parent`))

(event `EnhancedInput|/Game/Player/Input/Actions/UI/IA_Join`
  (params (ActionValue :type Boolean) (ElapsedSeconds :type "Float (double-precision)") (TriggeredSeconds :type "Float (double-precision)") (InputAction :type "InputAction Object Reference" :default "/Game/Player/Input/Actions/UI/IA_Join.IA_Join"))
  (:`Triggered`
    (`/Engine/EditorBlueprintResources/StandardMacros.DoOnce` false :!label _label
      (:`Completed`
        (bind _asbp_main_menu_gm (cast `/Game/Modes_Instances/Modes/BP_Main_Menu_GM` (`GameplayStatics.GetGameMode`)))
        (bind _character_select_widget_ref (`/Game/Modes_Instances/Modes/BP_Main_Menu_GM.Character Select Widget Ref` _asbp_main_menu_gm))
        (bind _returnvalue (`KismetArrayLibrary.Array_Find` (`/Game/Modes_Instances/Modes/BP_Main_Menu_GM.Players` _asbp_main_menu_gm) self))
        (`/Game/UI/Screens/Character_Select/Widgets/WBP_Character_Select.Join` _character_select_widget_ref _returnvalue)
        (`WidgetBlueprintLibrary.SetInputMode_GameAndUIEx` (`GameplayStatics.GetPlayerController` _returnvalue) (select `int` _returnvalue :`0` (`/Game/UI/Screens/Character_Select/Widgets/WBP_Character_Select.ReadyCharacter1` _character_select_widget_ref) :`1` (`/Game/UI/Screens/Character_Select/Widgets/WBP_Character_Select.ReadyCharacter2` _character_select_widget_ref) :`2` (`/Game/UI/Screens/Character_Select/Widgets/WBP_Character_Select.ReadyCharacter3` _character_select_widget_ref) :`3` (`/Game/UI/Screens/Character_Select/Widgets/WBP_Character_Select.ReadyCharacter4` _character_select_widget_ref) :!type "Widget Object Reference"))))))

(event `/Game/Combat/Interfaces/BPI_Has_Weapon.Set_Equipped_Ranged_Weapon`
  (params (`Weapon Parent` :type "/Game/Combat/Weapons/BPs/BP_WeaponParent Object Reference"))
  (set `self.Equipped Ranged Weapon` `Weapon Parent`))

(event `Reset Join`
  (goto _label :!via `Reset`))

(event `Update Character`
  (params (`New Character Name` :type "/Game/General_Character_Things/Enums/Enum_Character_Names Enum" :default "NewEnumerator0"))
  (bind _equipped_melee_weapon (`self.Equipped Melee Weapon`))
  (bind _show_only_list (`self.Show Only List`))
  (bind _equipped_ranged_weapon (`self.Equipped Ranged Weapon`))
  (`KismetSystemLibrary.PrintString` (`KismetStringLibrary.Concat_StrStr` (`KismetSystemLibrary.GetDisplayName` self) " IS BEING UPDATED."))
  (`KismetArrayLibrary.Array_RemoveItem` _show_only_list _equipped_ranged_weapon)
  (`KismetArrayLibrary.Array_RemoveItem` _show_only_list _equipped_melee_weapon)
  (`self.K2_DestroyActor` _equipped_melee_weapon)
  (`self.K2_DestroyActor` _equipped_ranged_weapon)
  (bind _returnvalue (`|GetDataTableRow` "/Game/Player/Structs_Tables/DT_Player_Character_Info.DT_Player_Character_Info" (`KismetStringLibrary.Conv_StringToName` (`|GetEnumeratorNameAsString` `New Character Name`)))
    (:`then`
      (bind _output_get (set `self.Character Info` _returnvalue))
      (`SkeletalMeshComponent.SetSkeletalMeshAsset` (`self.Mesh`) (`.CharacterMesh_45_C007CBB34910AA62B182F98A1917FF26` (break `/Game/General_Character_Things/Structs_Tables/Struct_Character_Info` _output_get)))
      (`/Game/Combat/Weapons/Components/BPC_AttachWeapon.Set Weapons` (`self.BPC_AttachWeapon`))
      (`self.Update Show Only List` (`|MakeArray` (`self.Equipped Ranged Weapon`) (`self.Equipped Melee Weapon`) :!type "Actor Object Reference")))))

(event `Update Show Only List`
  (params (`New Actors` :type "Array of Actor Object Reference"))
  (for _array_element `New Actors`
    (`KismetArrayLibrary.Array_Add` (`self.Show Only List`) _array_element))
  (set `SceneCaptureComponent.ShowOnlyActors` (`self.Show Only List`) (`self.Render Target`)))

(fn `Get Character Info`
  (returns (`Character Info` :type "/Game/General_Character_Things/Structs_Tables/Struct_Character_Info Structure"))
  (return (`self.Character Info`)))

(fn `Get Spells`
  (returns (`Character's Spells` :type "Array of /Game/Combat/Ranged/Projectiles/Enums/Enum_Spell_Names Enum"))
  (return))

(fn `Get_Character_Mesh`
  (returns (Mesh :type "SkeletalMeshComponent Object Reference"))
  (return (`self.Mesh`)))

(fn `Get_Equipped_Melee_Weapon`
  (returns (`Weapon Parent` :type "/Game/Combat/Weapons/BPs/BP_WeaponParent Object Reference"))
  (return (`self.Equipped Melee Weapon`)))

(fn `Get_Equipped_Ranged_Weapon`
  (returns (Weapon_Parent :type "/Game/Combat/Weapons/BPs/BP_WeaponParent Object Reference"))
  (return (`self.Equipped Ranged Weapon`)))

(fn `UserConstructionScript`
  (bind _returnvalue (`|GetDataTableRow` "/Game/Player/Structs_Tables/DT_Player_Character_Info.DT_Player_Character_Info" (`KismetStringLibrary.Conv_StringToName` (`|GetEnumeratorNameAsString` (`.CharacterName_25_3138D50F4790E86DA8C67587FF681575` (break `/Game/General_Character_Things/Structs_Tables/Struct_Character_Info` (`self.Character Info`))))))
    (:`then`
      (bind _output_get (set `self.Character Info` _returnvalue))
      (`SkeletalMeshComponent.SetSkeletalMeshAsset` (`self.Mesh`) (`.CharacterMesh_45_C007CBB34910AA62B182F98A1917FF26` (break `/Game/General_Character_Things/Structs_Tables/Struct_Character_Info` _output_get))))))