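; BP_Camera is a shared multiplayer camera that follows either the players' average position or the BP_Payload actor.
; GameStarted stores the active players and enables Tick, which lerps a Sphere component toward the FollowingPlayers-selected focus and a target rotation.
; Each tick also finds the player furthest from the sphere and eases spring arm length by that distance, clamped to a zoom range.
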(event `self.ReceiveBeginPlay`
  (bind _returnvalue (`GameplayStatics.GetActorOfClass` "/Game/Co-op/BPs/BP_Payload.BP_Payload_C"))
  (set `self.Payload` _returnvalue))

(event `self.ReceiveTick`
  (params (DeltaSeconds :type "Float (single-precision)"))
  (bind _springarm (`self.SpringArm`))
  (if (`self.Following_Players`)
    (bind _output_get (set `self.Previous_Loc` (`SceneComponent.K2_GetComponentLocation` (`self.Sphere`))))
    (bind _returnvalue (`GameplayStatics.GetActorArrayAverageLocation` (`self.Active Players`)))
    (`SceneComponent.K2_SetWorldLocation` (`self.Sphere`) (`KismetMathLibrary.VLerp` _output_get _returnvalue (`self.Pos_Lerp_Speed`)) false false)
    (else
      (bind _output_get_2 (set `self.Previous_Loc` (`SceneComponent.K2_GetComponentLocation` (`self.Sphere`))))
      (`SceneComponent.K2_SetWorldLocation` (`self.Sphere`) (`KismetMathLibrary.VLerp` _output_get_2 (`self.K2_GetActorLocation` (`self.Payload`)) (`self.Pos_Lerp_Speed`)) false false)))
  (`SceneComponent.K2_SetWorldRotation` (`self.Sphere`) (`KismetMathLibrary.RLerp` (`SceneComponent.K2_GetComponentRotation` (`self.Sphere`)) (`self.Target_Rotation`) (`self.Rot_Lerp_Speed`)) false false)
  (for (_array_element _array_index) (`self.Active Players`)
    (if (== _array_index 0)
      (bind _returnvalue_2 (`KismetMathLibrary.Vector_Distance` (`self.K2_GetActorLocation` _array_element) (`SceneComponent.K2_GetComponentLocation` (`self.Sphere`))))
      (set `self.Furthest_Player_Distance` _returnvalue_2)
      (elif (< (`self.Furthest_Player_Distance`) _returnvalue_2)
        (set `self.Furthest_Player_Distance` _returnvalue_2))))
  (set `SpringArmComponent.TargetArmLength` (`KismetMathLibrary.FClamp` (`KismetMathLibrary.Lerp` (`SpringArmComponent.TargetArmLength` _springarm) (* (`self.Max_Zoom_Amount`) (/ (`self.Furthest_Player_Distance`) 1500.0)) (`self.Zoom_Lerp_Speed`)) 1250.0 6500.0) _springarm))

(fn `Game Started`
  (params (`Active Players` :type "Array of Actor Object Reference"))
  (set `self.Active Players` `Active Players`)
  (`self.SetActorTickEnabled` true))

(fn `UserConstructionScript`)