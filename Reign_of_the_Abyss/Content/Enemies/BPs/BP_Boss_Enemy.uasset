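; Boss enemy character that loads its stats and mesh from DT_Enemy_Info, attaches extra socketed meshes and exposes weapon, spell and health getters.
; Activate2ndPhase runs once, swapping to the Lyssanthys row with blood explosion, camera shake and refreshed spells.
; A cutscene then pauses the AI, focuses the camera, scales up the boss and shows dialogue timed by character count.
; Afterward combat resumes with updated minion spawning and a large heal.
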(event `self.ReceiveBeginPlay`
  (bind ((`AdditionalSkeletalMeshes-NameofSocketAttachment_55_D31D802C4CC41EFB12CC23AEBA551BB2` _additionalskeletalmeshes_nameofsocketattachment)) (break `/Game/General_Character_Things/Structs_Tables/Struct_Character_Info` (`.CharacterInfo_34_7E88B37C48A144D82062C88B20F20CD8` (break `/Game/Enemies/Structs_Tables/Struct_Enemy_Info` (`self.Enemy Info`)))))
  (bind _keys (`BlueprintMapLibrary.Map_Keys` _additionalskeletalmeshes_nameofsocketattachment))
  (bind _values (`BlueprintMapLibrary.Map_Values` _additionalskeletalmeshes_nameofsocketattachment))
  (for (_array_element _array_index) _keys
    (bind _returnvalue (`AddComponent|NODE_AddSkeletalMeshComponent-0` :`bManualAttachment` true))
    (`SkeletalMeshComponent.SetSkeletalMeshAsset` _returnvalue _array_element)
    (`SceneComponent.K2_AttachToComponent` _returnvalue (`self.Mesh`) (`|GetArrayItem` _values _array_index) "SnapToTarget" "SnapToTarget" "KeepRelative" true)))

(event `self.Set_Equipped_Melee_Weapon`
  (params (`Weapon Parent` :type "/Game/Combat/Weapons/BPs/BP_WeaponParent Object Reference"))
  (set `self.EquippedMeleeWeapon` `Weapon Parent`))

(event `self.Set_Equipped_Ranged_Weapon`
  (params (`Weapon Parent` :type "/Game/Combat/Weapons/BPs/BP_WeaponParent Object Reference"))
  (set `self.EquippedRangedWeapon` `Weapon Parent`))

(event `/Game/Enemies/Interfaces/BPI_Boss.Activate 2nd Phase`
  (bind _bpc_enemy_spawning_director (`self.BPC_Enemy_Spawning_Director`))
  (`/Engine/EditorBlueprintResources/StandardMacros.DoOnce` false
    (:`Completed`
      (`|SpawnActorFromClass` "/Game/VFX/Bloodsplosion/BPs/BP_BloodSplosion.BP_BloodSplosion_C" (`KismetMathLibrary.MakeTransform` (`self.K2_GetActorLocation`)) "Undefined" "MultiplyWithRoot" null 500 null)
      (`GameplayStatics.PlayWorldCameraShake` "/Game/VFX/Bloodsplosion/BPs/BP_Bloodsplosion_Camera_Shake.BP_Bloodsplosion_Camera_Shake_C" (`self.K2_GetActorLocation`) 0.0 99999.0)
      (bind _returnvalue (`|GetDataTableRow` "/Game/Enemies/Structs_Tables/DT_Enemy_Info.DT_Enemy_Info" "Lyssanthys")
        (:`then`
          (set `self.Enemy Info` _returnvalue)
          (`SkeletalMeshComponent.SetSkeletalMeshAsset` (`self.Mesh`) (`.CharacterMesh_45_C007CBB34910AA62B182F98A1917FF26` (break `/Game/General_Character_Things/Structs_Tables/Struct_Character_Info` (`.CharacterInfo_34_7E88B37C48A144D82062C88B20F20CD8` (break `/Game/Enemies/Structs_Tables/Struct_Enemy_Info` _returnvalue)))))
          (`/Game/Combat/Ranged/Components/BPC_Spells.Update Spells` (`self.BPC_Spells`))
          (bind _asac_enemy (cast `/Game/Enemies/AI/Controllers/AC_Enemy` (`self.GetController`)))
          (set `/Game/Enemies/AI/Controllers/AC_Enemy.Active` false _asac_enemy)
          (`/Game/Movement/Basic_Movement/BPC_Movement_Manager.Set Speed Multiplier` (`self.BPC_Movement_Manager`) 1.0)
          (set `/Game/Combat/Components/BPC_AttackHandler.In Boss Cutscene` true (`self.BPC_AttackHandler`))
          (bind _returnvalue_2 (`GameplayStatics.GetActorOfClass` "/Game/Co-op/Camera/BP_Camera.BP_Camera_C"))
          (set `/Game/Co-op/Camera/BP_Camera.Focus Boss` true _returnvalue_2)
          (bind _asbp_third_person_game_mode (cast `/Game/Modes_Instances/Modes/BP_ThirdPersonGameMode` (`GameplayStatics.GetGameMode`)))
          (bind _wbp_boss_health (`/Game/UI/HUD/Widgets/WBP_HUD.WBP_Boss_Health` (`/Game/Modes_Instances/Modes/BP_ThirdPersonGameMode.HUD Ref` _asbp_third_person_game_mode)))
          (`/Game/UI/HUD/Widgets/WBP_Boss_Health.Deactivate` _wbp_boss_health)
          (`/Game/UI/HUD/Widgets/WBP_Boss_Health.Activate` _wbp_boss_health)
          (for _array_element (`/Game/Modes_Instances/Modes/BP_ThirdPersonGameMode.Players` _asbp_third_person_game_mode)
            (`/Game/Movement/Basic_Movement/BPC_Movement_Manager.Set Speed Multiplier` (`self.GetComponentByClass` _array_element "/Game/Movement/Basic_Movement/BPC_Movement_Manager.BPC_Movement_Manager_C") 1.0)
            (set `/Game/Combat/Components/BPC_AttackHandler.In Boss Cutscene` true (`self.GetComponentByClass` _array_element "/Game/Combat/Components/BPC_AttackHandler.BPC_AttackHandler_C")))
          (bind (_direction _alpha) (`Timeline|Lerp Boss Scale` :!via `PlayFromStart`)
            (:`Update`
              (`SceneComponent.SetWorldScale3D` (`self.CapsuleComponent`) (`KismetMathLibrary.VLerp` (1.5 1.5 1.5) (2.0 2.0 2.0) _alpha)))
            (:`Finished`
              (bind _returnvalue_3 (`|CreateWidget` "/Game/UI/Screens/Dialogue/WBP_Boss_Dialogue.WBP_Boss_Dialogue_C" null (`self.Second Phase Dialogue Dialogue`) (`self.Second Phase Dialogue Speed`)))
              (`UserWidget.AddToViewport` _returnvalue_3 0)
              (set `self.Second Phase Dialogue Complete Time` 0.0)
              (for _array_element_2 (`self.Second Phase Dialogue Dialogue`)
                (set `self.Second Phase Dialogue Complete Time` (+ (`self.Second Phase Dialogue Complete Time`) (+ (* (`KismetArrayLibrary.Array_Length` (`KismetStringLibrary.GetCharacterArrayFromString` (`KismetTextLibrary.Conv_TextToString` _array_element_2))) (`self.Second Phase Dialogue Speed`)) 1.0))))
              (`KismetSystemLibrary.Delay` (`self.Second Phase Dialogue Complete Time`))
              (set `/Game/Co-op/Camera/BP_Camera.Focus Boss` false _returnvalue_2)
              (set `/Game/Enemies/AI/Controllers/AC_Enemy.Active` true _asac_enemy)
              (set `/Game/Combat/Components/BPC_AttackHandler.In Boss Cutscene` false (`self.BPC_AttackHandler`))
              (`/Game/Enemies/Components/BPC_Enemy_Spawning_Director.Update Spawn Amount` _bpc_enemy_spawning_director (`|MakeMap` "NewEnumerator6" 5 "NewEnumerator10" 3 :!type "/Game/Enemies/Enums/Enum_Enemies Enum"))
              (`/Game/Enemies/Components/BPC_Enemy_Spawning_Director.Update Spawn Rate` _bpc_enemy_spawning_director 10.0)
              (`/Game/Movement/Basic_Movement/BPC_Movement_Manager.Set Speed Multiplier` (`self.BPC_Movement_Manager`) -1.0)
              (bind _asbp_third_person_game_mode_2 (cast `/Game/Modes_Instances/Modes/BP_ThirdPersonGameMode` (`GameplayStatics.GetGameMode`)))
              (for _array_element_3 (`/Game/Modes_Instances/Modes/BP_ThirdPersonGameMode.Players` _asbp_third_person_game_mode_2)
                (`/Game/Movement/Basic_Movement/BPC_Movement_Manager.Set Speed Multiplier` (`self.GetComponentByClass` _array_element_3 "/Game/Movement/Basic_Movement/BPC_Movement_Manager.BPC_Movement_Manager_C") -1.0)
                (set `/Game/Combat/Components/BPC_AttackHandler.In Boss Cutscene` false (`self.GetComponentByClass` _array_element_3 "/Game/Combat/Components/BPC_AttackHandler.BPC_AttackHandler_C")))
              (`/Game/Health/Components/BPC_Health_V2.Heal` (`self.BPC_Health_V2`) 9999.0))))))))

(fn `Get Character Info`
  (returns (`Character Info` :type "/Game/General_Character_Things/Structs_Tables/Struct_Character_Info Structure"))
  (return (`.CharacterInfo_34_7E88B37C48A144D82062C88B20F20CD8` (break `/Game/Enemies/Structs_Tables/Struct_Enemy_Info` (`self.Enemy Info`)))))

(fn `Get Current Spell`
  (returns (Spell :type "/Game/Combat/Ranged/Projectiles/Structs_Tables/Struct_Spell_Info Structure"))
  (return (`/Game/Combat/Ranged/Components/BPC_Spells.Current Spell` (`self.BPC_Spells`))))

(fn `Get Enemy Info`
  (returns (`Enemy Info` :type "/Game/Enemies/Structs_Tables/Struct_Enemy_Info Structure"))
  (return (`self.Enemy Info`)))

(fn `Get Health Info`
  (returns (`Health Info` :type "/Game/Health/Structs_Tables/Struct_Health_Info Structure"))
  (return (`.HealthInfo_27_FE8889204233D713A8392D9FFC4FA5F5` (break `/Game/General_Character_Things/Structs_Tables/Struct_Character_Info` (`.CharacterInfo_34_7E88B37C48A144D82062C88B20F20CD8` (break `/Game/Enemies/Structs_Tables/Struct_Enemy_Info` (`self.Enemy Info`)))))))

(fn `Get Main Skeletal Mesh`
  (returns (`Skeletal Mesh Component` :type "SkeletalMeshComponent Object Reference"))
  (return (`self.Mesh`)))

(fn `Get Ranged Weapon Mesh`
  (returns (`Static Mesh` :type "StaticMeshComponent Object Reference"))
  (return (`/Game/Combat/Weapons/BPs/BP_WeaponParent.WeaponMesh` (`self.EquippedRangedWeapon`))))

(fn `Get Spells`
  (returns (`Character's Spells` :type "Array of /Game/Combat/Ranged/Projectiles/Enums/Enum_Spell_Names Enum"))
  (return (`.SpellNames_31_03D6700A43242027BE70A18A6486F183` (break `/Game/General_Character_Things/Structs_Tables/Struct_Character_Info` (`.CharacterInfo_34_7E88B37C48A144D82062C88B20F20CD8` (break `/Game/Enemies/Structs_Tables/Struct_Enemy_Info` (`self.Enemy Info`)))))))

(fn `Get_Character_Mesh`
  (returns (Mesh :type "SkeletalMeshComponent Object Reference"))
  (return (`self.Mesh`)))

(fn `Get_Equipped_Melee_Weapon`
  (returns (`Weapon Parent` :type "/Game/Combat/Weapons/BPs/BP_WeaponParent Object Reference"))
  (return (`self.EquippedMeleeWeapon`)))

(fn `Get_Equipped_Ranged_Weapon`
  (returns (Weapon_Parent :type "/Game/Combat/Weapons/BPs/BP_WeaponParent Object Reference"))
  (bind _equippedrangedweapon (`self.EquippedRangedWeapon`))
  (`/Engine/EditorBlueprintResources/StandardMacros.IsValid` _equippedrangedweapon
    (:`Is Valid`
      (return _equippedrangedweapon))
    (:`Is Not Valid`
      (return null))))

(fn `Get_Hand_Cast_Loc`
  (returns (Vector :type "Vector Structure"))
  (return (`SceneComponent.GetSocketLocation` (`self.Mesh`) "Hand_Cast_Loc_R")))

(fn `UserConstructionScript`
  (bind _returnvalue (`|GetDataTableRow` "/Game/Enemies/Structs_Tables/DT_Enemy_Info.DT_Enemy_Info" (`KismetStringLibrary.Conv_StringToName` (`|GetEnumeratorNameAsString` (`.EnemyName_5_1AED7F654B2F73F405EA7EAD4C01CE55` (break `/Game/Enemies/Structs_Tables/Struct_Enemy_Info` (`self.Enemy Info`))))))
    (:`then`
      (set `self.Enemy Info` _returnvalue)
      (`SkeletalMeshComponent.SetSkeletalMeshAsset` (`self.Mesh`) (`.CharacterMesh_45_C007CBB34910AA62B182F98A1917FF26` (break `/Game/General_Character_Things/Structs_Tables/Struct_Character_Info` (`.CharacterInfo_34_7E88B37C48A144D82062C88B20F20CD8` (break `/Game/Enemies/Structs_Tables/Struct_Enemy_Info` _returnvalue))))))))