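; Trigger actor that runs the boss intro cutscene once every player has exited its volume, then destroys itself.
; It flags players as in-cutscene, changes their speed multiplier, focuses BP_Camera on the boss and shows a dialogue widget.
; After a delay computed from dialogue character counts, the camera orbits while the HUD shows the boss image and health bar.
; After FocusDuration, it resets camera and players, clears the boss's cutscene flag and activates its AI.
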(event `self.ReceiveBeginPlay`
  (`KismetSystemLibrary.Delay` 0.3)
  (bind _asbp_third_person_game_mode (cast `/Game/Modes_Instances/Modes/BP_ThirdPersonGameMode` (`GameplayStatics.GetGameMode`)))
  (bind _output_get (set `self.As BP Third Person Game Mode` _asbp_third_person_game_mode))
  (set `self.Players` (`/Game/Modes_Instances/Modes/BP_ThirdPersonGameMode.Players` _output_get)))

(event `self.Trigger.OnComponentEndOverlap`
  (params (OverlappedComponent :type "PrimitiveComponent Object Reference") (OtherActor :type "Actor Object Reference") (OtherComp :type "PrimitiveComponent Object Reference") (OtherBodyIndex :type Integer))
  (bind _dialogue_complete_time (`self.Dialogue Complete Time`))
  (if (not (`KismetArrayLibrary.Array_Contains` (`self.Players Triggered`) OtherActor))
    (`KismetArrayLibrary.Array_Add` (`self.Players Triggered`) OtherActor)
    (if (== (`KismetArrayLibrary.Array_Length` (`self.Players Triggered`)) (`KismetArrayLibrary.Array_Length` (`self.Players`)))
      (for _array_element (`self.Players`)
        (`/Game/Movement/Basic_Movement/BPC_Movement_Manager.Set Speed Multiplier` (`self.GetComponentByClass` _array_element "/Game/Movement/Basic_Movement/BPC_Movement_Manager.BPC_Movement_Manager_C") 1.0)
        (set `/Game/Combat/Components/BPC_AttackHandler.In Boss Cutscene` true (`self.GetComponentByClass` _array_element "/Game/Combat/Components/BPC_AttackHandler.BPC_AttackHandler_C")))
      (bind _returnvalue (`GameplayStatics.GetActorOfClass` "/Game/Co-op/Camera/BP_Camera.BP_Camera_C"))
      (set `/Game/Co-op/Camera/BP_Camera.Focus Boss` true _returnvalue)
      (bind _returnvalue_2 (`|CreateWidget` "/Game/UI/Screens/Dialogue/WBP_Boss_Dialogue.WBP_Boss_Dialogue_C" null (`self.Dialogue`) (`self.Dialogue Speed`)))
      (`UserWidget.AddToViewport` _returnvalue_2 0)
      (set `self.Dialogue Complete Time` 0.0)
      (for _array_element_2 (`self.Dialogue`)
        (set `self.Dialogue Complete Time` (+ (`self.Dialogue Complete Time`) (+ (* (`KismetArrayLibrary.Array_Length` (`KismetStringLibrary.GetCharacterArrayFromString` (`KismetTextLibrary.Conv_TextToString` _array_element_2))) (`self.Dialogue Speed`)) 1.0))))
      (`KismetSystemLibrary.PrintString` (`KismetStringLibrary.Conv_DoubleToString` _dialogue_complete_time))
      (`KismetSystemLibrary.Delay` _dialogue_complete_time)
      (set `/Game/Co-op/Camera/BP_Camera.Rotating Around Boss` true _returnvalue)
      (bind _asbp_third_person_game_mode (cast `/Game/Modes_Instances/Modes/BP_ThirdPersonGameMode` (`GameplayStatics.GetGameMode`)))
      (`/Game/UI/HUD/Widgets/WBP_HUD.Play Boss Image ` (`/Game/Modes_Instances/Modes/BP_ThirdPersonGameMode.HUD Ref` _asbp_third_person_game_mode))
      (`/Game/UI/HUD/Widgets/WBP_HUD.Activate Boss Health Bar` (`/Game/Modes_Instances/Modes/BP_ThirdPersonGameMode.HUD Ref` _asbp_third_person_game_mode))
      (`KismetSystemLibrary.Delay` (`self.Focus Duration`))
      (set `/Game/Co-op/Camera/BP_Camera.Focus Boss` false _returnvalue)
      (set `/Game/Co-op/Camera/BP_Camera.Rotating Around Boss` false _returnvalue)
      (bind _returnvalue_3 (`GameplayStatics.GetActorOfClass` "/Game/Enemies/BPs/BP_Boss_Enemy.BP_Boss_Enemy_C"))
      (set `/Game/Combat/Components/BPC_AttackHandler.In Boss Cutscene` false (`self.GetComponentByClass` _returnvalue_3 "/Game/Combat/Components/BPC_AttackHandler.BPC_AttackHandler_C"))
      (bind _asbp_third_person_game_mode_2 (cast `/Game/Modes_Instances/Modes/BP_ThirdPersonGameMode` (`GameplayStatics.GetGameMode`)))
      (for _array_element_3 (`/Game/Modes_Instances/Modes/BP_ThirdPersonGameMode.Players` _asbp_third_person_game_mode_2)
        (`/Game/Movement/Basic_Movement/BPC_Movement_Manager.Set Speed Multiplier` (`self.GetComponentByClass` _array_element_3 "/Game/Movement/Basic_Movement/BPC_Movement_Manager.BPC_Movement_Manager_C") -1.0)
        (set `/Game/Combat/Components/BPC_AttackHandler.In Boss Cutscene` false (`self.GetComponentByClass` _array_element_3 "/Game/Combat/Components/BPC_AttackHandler.BPC_AttackHandler_C")))
      (bind _returnvalue_4 (`GameplayStatics.GetActorOfClass` "/Game/Enemies/BPs/BP_Boss_Enemy.BP_Boss_Enemy_C"))
      (bind _asac_enemy (cast `/Game/Enemies/AI/Controllers/AC_Enemy` (`Pawn.GetController` _returnvalue_4)))
      (`/Game/Enemies/AI/Controllers/AC_Enemy.Activate Enemy` _asac_enemy)
      (`self.K2_DestroyActor`))))

(fn `UserConstructionScript`)