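; BP_TestEnemy is an enemy character that holds its info, equipped weapons and spell component, and exposes them through getters.
; The construction script replaces EnemyInfo with the DT_Enemy_Info row named after its EnemyName enum, if found.
; Events store melee and ranged weapon references.
; Getters return character and health info, mesh, weapons and the current spell from BPCSpells, validity-checking only the ranged weapon getter.
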(event `/Game/Combat/Interfaces/BPI_Has_Weapon.Set_Equipped_Melee_Weapon`
  (params (`Weapon Parent` :type "/Game/Combat/Weapons/BPs/BP_WeaponParent Object Reference"))
  (set `self.EquippedMeleeWeapon` `Weapon Parent`))

(event `/Game/Combat/Interfaces/BPI_Has_Weapon.Set_Equipped_Ranged_Weapon`
  (params (`Weapon Parent` :type "/Game/Combat/Weapons/BPs/BP_WeaponParent Object Reference"))
  (set `self.EquippedRangedWeapon` `Weapon Parent`))

(fn `Get Character Info`
  (returns (`Character Info` :type "/Game/General_Character_Things/Structs_Tables/Struct_Character_Info Structure"))
  (return (`.CharacterInfo_26_7E88B37C48A144D82062C88B20F20CD8` (break `/Game/Enemies/Structs_Tables/Struct_Enemy_Info` (`self.Enemy Info`)))))

(fn `Get Current Spell`
  (returns (Spell :type "/Game/Combat/Ranged/Projectiles/Structs_Tables/Struct_Spell_Info Structure"))
  (return (`/Game/Combat/Ranged/Components/BPC_Spells.Current Spell` (`self.BPC_Spells`))))

(fn `Get Enemy Info`
  (returns (`Enemy Info` :type "/Game/Enemies/Structs_Tables/Struct_Enemy_Info Structure"))
  (return (`self.Enemy Info`)))

(fn `Get Health Info`
  (returns (`Health Info` :type "/Game/Health/Structs_Tables/Struct_Health_Info Structure"))
  (return (`.HealthInfo_27_FE8889204233D713A8392D9FFC4FA5F5` (break `/Game/General_Character_Things/Structs_Tables/Struct_Character_Info` (`.CharacterInfo_26_7E88B37C48A144D82062C88B20F20CD8` (break `/Game/Enemies/Structs_Tables/Struct_Enemy_Info` (`self.Enemy Info`)))))))

(fn `Get Ranged Weapon Mesh`
  (returns (`Static Mesh` :type "StaticMeshComponent Object Reference"))
  (return (`/Game/Combat/Weapons/BPs/BP_WeaponParent.WeaponMesh` (`self.EquippedRangedWeapon`))))

(fn `Get_Character_Mesh`
  (returns (Mesh :type "SkeletalMeshComponent Object Reference"))
  (return (`self.Mesh`)))

(fn `Get_Equipped_Melee_Weapon`
  (returns (`Weapon Parent` :type "/Game/Combat/Weapons/BPs/BP_WeaponParent Object Reference"))
  (return (`self.EquippedMeleeWeapon`)))

(fn `Get_Equipped_Ranged_Weapon`
  (returns (Weapon_Parent :type "/Game/Combat/Weapons/BPs/BP_WeaponParent Object Reference"))
  (bind _equippedrangedweapon (`self.EquippedRangedWeapon`))
  (`/Engine/EditorBlueprintResources/StandardMacros.IsValid` _equippedrangedweapon
    (:`Is Valid`
      (return _equippedrangedweapon))
    (:`Is Not Valid`
      (return null))))

(fn `UserConstructionScript`
  (bind _returnvalue (`|GetDataTableRow` "/Game/Enemies/Structs_Tables/DT_Enemy_Info.DT_Enemy_Info" (`KismetStringLibrary.Conv_StringToName` (`|GetEnumeratorNameAsString` (`.EnemyName_5_1AED7F654B2F73F405EA7EAD4C01CE55` (break `/Game/Enemies/Structs_Tables/Struct_Enemy_Info` (`self.Enemy Info`))))))
    (:`then`
      (set `self.Enemy Info` _returnvalue))))