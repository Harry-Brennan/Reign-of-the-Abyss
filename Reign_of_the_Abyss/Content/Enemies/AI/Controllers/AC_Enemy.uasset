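; AI controller for enemies that chooses between chasing players and the payload, starting the main enemy behavior tree only through ActivateBoss.
; Perception maintains a list of sensed targets, evaluated on each sensing update using interface, distance and player downed checks.
; These set the passive or aggressive state, chased actor and focus, with getters exposing state and target.
; When no targets remain after one is forgotten, it idles after a delay.
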(event `Activate Boss`
  (`self.RunBehaviorTree` "/Game/Enemies/AI/Trees/BT_Enemy_Main.BT_Enemy_Main"))

(event `self.ReceiveBeginPlay`
  (bind _returnvalue (`GameplayStatics.GetActorOfClass` "/Game/Co-op/Payload/BP_Payload.BP_Payload_C"))
  (set `self.Payload Ref` _returnvalue))

(event `self.AIPerception.OnTargetPerceptionInfoUpdated`
  (params (UpdateInfo :type "ActorPerceptionUpdateInfo Structure (by ref)"))
  (bind _perception_target (`self.Perception Target`))
  (bind _chasing_character (`self.Chasing_Character`))
  (bind _perception_target_2 (`self.Perception Target`))
  (bind (_age _expirationage _strength _stimuluslocation _receiverlocation _tag _bsuccessfullysensed) (break `AIStimulus` (`.Stimulus` (break `ActorPerceptionUpdateInfo` UpdateInfo))))
  (bind _returnvalue (`self.K2_GetActorLocation` (`self.K2_GetPawn`)))
  (bind _returnvalue_2 (`self.K2_GetActorLocation` (`self.K2_GetPawn`)))
  (bind _returnvalue_3 (`self.GetComponentByClass` (`self.Perception Target`) "/Game/Health/Components/BPC_Health_V2.BPC_Health_V2_C"))
  (bind _returnvalue_4 (`self.GetComponentByClass` (`self.Perception Target`) "/Game/Health/Components/BPC_Health_V2.BPC_Health_V2_C"))
  (bind _returnvalue_5 (`self.GetComponentByClass` (`self.Perception Target`) "/Game/Health/Components/BPC_Health_V2.BPC_Health_V2_C"))
  (bind _returnvalue_6 (<= (`KismetMathLibrary.Vector_Distance` (`self.K2_GetActorLocation` (`self.Perception Target`)) _returnvalue) (`KismetMathLibrary.Vector_Distance` _returnvalue (`self.K2_GetActorLocation` (`self.Chasing_Character`)))))
  (if _bsuccessfullysensed
    (for _array_element (`self.Perceived Targets`)
      (set `self.Perception Target` _array_element)
      (switch `/Game/Enemies/AI/Enums/Enum_Enemy_States` (`self.Current State`)
        (:`NewEnumerator0`
          (if (`KismetSystemLibrary.DoesImplementInterface` _perception_target_2 "/Game/Player/Interfaces/BPI_Player.BPI_Player_C")
            (if (not (or (`/Game/Health/Components/BPC_Health_V2.Downed` _returnvalue_5) (`/Game/Health/Components/BPC_Health_V2.DownedTransition` _returnvalue_5)))
              (`self.Update State` "NewEnumerator1")
              (bind _output_get (set `self.Chasing_Character` (`self.Perception Target`) :!label _label))
              (`self.K2_SetFocus` _output_get))
            (elif (`KismetSystemLibrary.DoesImplementInterface` _perception_target_2 "/Game/Co-op/Interfaces/BPI_Payload.BPI_Payload_C")
              (`self.Update State` "NewEnumerator2")
              (goto _label))))
        (:`NewEnumerator1`
          (if (and (`KismetSystemLibrary.DoesImplementInterface` _perception_target "/Game/Co-op/Interfaces/BPI_Payload.BPI_Payload_C") _returnvalue_6)
            (`self.Update State` "NewEnumerator2")
            (bind _output_get_2 (set `self.Chasing_Character` (`self.Perception Target`)))
            (`self.K2_SetFocus` _output_get_2)
            (elif (and (`KismetSystemLibrary.DoesImplementInterface` _perception_target "/Game/Player/Interfaces/BPI_Player.BPI_Player_C") _returnvalue_6)
              (`/Engine/EditorBlueprintResources/StandardMacros.IsValid` _returnvalue_4
                (:`Is Valid`
                  (if (not (or (`/Game/Health/Components/BPC_Health_V2.Downed` _returnvalue_4) (`/Game/Health/Components/BPC_Health_V2.DownedTransition` _returnvalue_4)))
                    (bind _output_get_3 (set `self.Chasing_Character` (`self.Perception Target`) :!label _label_2))
                    (`self.K2_SetFocus` _output_get_3)))
                (:`Is Not Valid`
                  (goto _label_2))))))
        (:`NewEnumerator2`
          (if (and (`KismetSystemLibrary.DoesImplementInterface` (`self.Perception Target`) "/Game/Player/Interfaces/BPI_Player.BPI_Player_C") (select `bool` (`KismetSystemLibrary.IsValid` _chasing_character) :`false` true :`true` (< (`KismetMathLibrary.Vector_Distance` _stimuluslocation _returnvalue_2) (`KismetMathLibrary.Vector_Distance` (`self.K2_GetActorLocation` _chasing_character) _returnvalue_2))))
            (`/Engine/EditorBlueprintResources/StandardMacros.IsValid` _returnvalue_3
              (:`Is Valid`
                (if (not (or (`/Game/Health/Components/BPC_Health_V2.Downed` _returnvalue_3) (`/Game/Health/Components/BPC_Health_V2.DownedTransition` _returnvalue_3)))
                  (`self.Update State` "NewEnumerator1")
                  (bind _output_get_4 (set `self.Chasing_Character` (`self.Perception Target`)))
                  (`self.K2_SetFocus` _output_get_4))))
            (else
              (`self.Update State` "NewEnumerator2")
              (bind _output_get_5 (set `self.Chasing_Character` (`self.Perception Target`)))
              (`self.K2_SetFocus` _output_get_5))))))))

(event `self.AIPerception.OnTargetPerceptionUpdated`
  (params (Actor :type "Actor Object Reference") (Stimulus :type "AIStimulus Structure"))
  (if (`.bSuccessfullySensed` (break `AIStimulus` Stimulus))
    (`KismetArrayLibrary.Array_Add` (`self.Perceived Targets`) Actor)
    (else
      (`KismetArrayLibrary.Array_RemoveItem` (`self.Perceived Targets`) Actor))))

(event `self.AIPerception.OnTargetPerceptionForgotten`
  (params (Actor :type "Actor Object Reference"))
  (`KismetArrayLibrary.Array_RemoveItem` (`self.Perceived Targets`) Actor)
  (if (`KismetArrayLibrary.Array_IsEmpty` (`self.Perceived Targets`))
    (`KismetSystemLibrary.Delay` 2.0)
    (`/Game/Enemies/Interfaces/BPI_Enemy_Controller.Update State` "NewEnumerator0")
    (`self.K2_ClearFocus`)))

(event `/Game/Enemies/Interfaces/BPI_Enemy_Controller.Update State`
  (params (`New State` :type "/Game/Enemies/AI/Enums/Enum_Enemy_States Enum" :default "NewEnumerator0"))
  (if (not (`|EnumEquality` `New State` (`self.Current State`)))
    (set `self.Current State` `New State`)))

(fn `Get Chasing Actor`
  (returns (Actor :type "Actor Object Reference"))
  (return (`self.Chasing_Character`)))

(fn `Get State`
  (returns (State :type "/Game/Enemies/AI/Enums/Enum_Enemy_States Enum"))
  (return (`self.Current State`)))

(fn `UserConstructionScript`)