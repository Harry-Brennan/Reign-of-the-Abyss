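; Enemy spawning director component that periodically spawns BP_Enemy actors around the payload, using its tick interval as the spawn rate.
; The spawn radius scales with the player camera's spring arm length and zoom ratio.
; Random navigable points are accepted only near that radius's outer edge, with no retry on failure.
; Each enemy faces the payload, receives a random DT_Enemy_Info row and gets a temporary debug box at its location.
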(event `self.ReceiveBeginPlay`
  ;[1 1 1] Setup
  (bind _returnvalue (`GameplayStatics.GetActorOfClass` "/Game/Co-op/Camera/BP_Camera.BP_Camera_C"))
  (bind _output_get (set `self.Player's Camera` _returnvalue))
  (set `self.Player's Camera Spring Arm` (`/Game/Co-op/Camera/BP_Camera.SpringArm` _output_get))
  (set `self.Max Zoom Length` (`/Game/Co-op/Camera/BP_Camera.Max Zoom Length` _output_get))
  (bind _returnvalue_2 (`GameplayStatics.GetActorOfClass` "/Game/Co-op/Payload/BP_Payload.BP_Payload_C"))
  (set `self.Payload` _returnvalue_2)
  (`self.SetComponentTickInterval` (`self.Spawn Rate`)))

(event `self.ReceiveTick`
  (params (DeltaSeconds :type "Float (single-precision)"))
  ;[1 1 1] Spawn enemy
  (`self.Spawn Enemy`))

(fn `Spawn Enemy`
  (bind _returnvalue (`Actor.K2_GetActorLocation` (`self.Payload`)))
  (bind _targetarmlength (`SpringArmComponent.TargetArmLength` (`self.Player's Camera Spring Arm`)))
  ;[1 1 1] Spawn enemy with random enemy info outisde of  a set radius and also draw a little debug cube for 5 seconds at the location as well
  (bind _output_get (set `self.Spawn Radius` (* _targetarmlength (* 2.75 (`KismetMathLibrary.FClamp` (/ _targetarmlength (`self.Max Zoom Length`)) 0.6 0.75)))))
  (bind _randomlocation (`NavigationSystemV1.K2_GetRandomLocationInNavigableRadius` (`Actor.K2_GetActorLocation` (`self.Payload`)) _output_get null null))
  (for _ (range 1 (+ (`self.Spawn Amount`) 1))
    (bind _outrownames (`DataTableFunctionLibrary.GetDataTableRowNames` "/Game/Enemies/Structs_Tables/DT_Enemy_Info.DT_Enemy_Info"))
    (bind _returnvalue_2 (`|GetDataTableRow` "/Game/Enemies/Structs_Tables/DT_Enemy_Info.DT_Enemy_Info" (`KismetArrayLibrary.Array_Random` _outrownames))
      (:`then`
        (if (> (`KismetMathLibrary.VSize` (- _returnvalue _randomlocation)) (* (`self.Spawn Radius`) 0.9))
          (bind _returnvalue_3 (`KismetMathLibrary.FindLookAtRotation` _randomlocation _returnvalue))
          (`KismetSystemLibrary.DrawDebugBox` _randomlocation (5.0 5.0 5.0) (struct) _returnvalue_3 5.0 5.0)
          (`|SpawnActorFromClass` "/Game/Enemies/BPs/BP_Enemy.BP_Enemy_C" (`KismetMathLibrary.MakeTransform` _randomlocation _returnvalue_3) "AdjustIfPossibleButAlwaysSpawn" "MultiplyWithRoot" null _returnvalue_2 null))))))