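; Movement manager component that controls its owning character's walk speed through a stackable speed multiplier.
; On BeginPlay it reads the base speed from the owner's character info, then each Tick moves MaxWalkSpeed at a constant rate toward base speed times multiplier.
; SetSpeedMultiplier subtracts the passed difference, so positive values slow the owner.
; It clamps the applied multiplier but keeps an unclamped total, so overlapping changes reverse cleanly.
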(event `self.ReceiveBeginPlay`
  ;[1 1 1] Get the owning character's info to get the base movement speed and set this to the float variable to be used for changing the speed.
  (bind _character_info (message `/Game/General_Character_Things/Interfaces/BPI_Character.Get Character Info` (`self.GetOwner`)))
  (bind _output_get (set `self.Base Movement Speed` (`.BaseMovementSpeed_2_E2CF1391418CFBD3AC4AB49080F340B8` (break `/Game/Movement/Basic_Movement/Struct_Basic_Movement_Info` (`.BasicMovementInfo_29_836C670A4CFE01D4E5C7818F9B9C661A` (break `/Game/General_Character_Things/Structs_Tables/Struct_Character_Info` _character_info))))))
  (set `CharacterMovementComponent.MaxWalkSpeed` _output_get (`Actor.GetComponentByClass` (`self.GetOwner`) "/Script/Engine.CharacterMovementComponent"))
  (`self.SetComponentTickEnabled` true))

(event `self.ReceiveTick`
  (params (DeltaSeconds :type "Float (single-precision)"))
  (bind _returnvalue (`Actor.GetComponentByClass` (`self.GetOwner`) "/Script/Engine.CharacterMovementComponent"))
  ;[1 1 1] Constantly finterping the max walk speed of the owner to be the base movement speed multiplied by the speed multiplier so that any changes to the speed multiplier happen relatively fast and smoothly with no sudden changes in speed
  (set `CharacterMovementComponent.MaxWalkSpeed` (`KismetMathLibrary.FInterpTo_Constant` (`CharacterMovementComponent.MaxWalkSpeed` _returnvalue) (* (`self.Base Movement Speed`) (`self.Speed Multiplier`)) DeltaSeconds 750.0) _returnvalue))

(fn `Set Speed Multiplier`
  (params (`Speed Multiplier Difference` :type "Float (double-precision)"))
  ;[1 1 1] This function is for changing the speed multiplier based on the passed parameter so passing a positive float will decrease the speed multiplier therefore overall decreasing the speed of the owner but passing a negative number will increase the speed multiplier and therefore increase the speed. The speed multiplier however is clamped to 0.05 and 2.0 but there is another float variable called unclamped SM value that is the unclamped varions of the speed multiplier which is what is actually used to change the speed multiplier based on the passed parameter which allows multiple changes to the speed to happen at once and the speed multiplier to be able to be set back to normal afterwards
  (set `self.Speed Multiplier` (`KismetMathLibrary.FClamp` (- (`self.Unclamped SM Value`) `Speed Multiplier Difference`) 0.01 2.0))
  (set `self.Unclamped SM Value` (- (`self.Unclamped SM Value`) `Speed Multiplier Difference`)))