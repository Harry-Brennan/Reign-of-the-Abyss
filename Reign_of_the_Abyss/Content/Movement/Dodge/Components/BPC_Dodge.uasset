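; Dodge component that handles the shared dodge/roll input for its owning character.
; Every tick it recomputes CanDodge from falling state, BPC_Roll, BPC_AttackHandler and the CharmedTurned status tag in BPC_StatusEffectHandler.
; A press sets Dodging when allowed, which the animation blueprint uses to start the dodge.
; A press while already dodging chains into BPC_Roll's roll if CanRoll, regardless of CanDodge.
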(event `self.ReceiveTick`
  (params (DeltaSeconds :type "Float (single-precision)"))
  (bind _returnvalue (`self.GetOwner`))
  ;[1 1 1] Constantly setting if can dodge based on if on the ground, if not rolling and if we can attack which is just used instead of doing all the checks for can attack since it should be simpler.
  (set `self.Can Dodge` (and (not (`NavMovementComponent.IsFalling` (`Actor.GetComponentByClass` _returnvalue "/Script/Engine.CharacterMovementComponent"))) (not (`/Game/Movement/Roll/Components/BPC_Roll.Rolling` (`Actor.GetComponentByClass` _returnvalue "/Game/Movement/Roll/Components/BPC_Roll.BPC_Roll_C"))) (`/Game/Combat/Components/BPC_AttackHandler.Can Attack` (`Actor.GetComponentByClass` _returnvalue "/Game/Combat/Components/BPC_AttackHandler.BPC_AttackHandler_C")) (not (`BlueprintGameplayTagLibrary.HasTag` (`/Game/Combat/Status_Effects/Components/BPC_StatusEffectHandler.StatusEffects` (`Actor.GetComponentByClass` (`self.GetOwner`) "/Game/Combat/Status_Effects/Components/BPC_StatusEffectHandler.BPC_StatusEffectHandler_C")) (struct :`TagName` "Charmed / Turned"))))))

(event `EnhancedInput|/Game/Player/Input/Actions/Movement/IA_Dodge_Roll`
  (params (ActionValue :type Boolean) (ElapsedSeconds :type "Float (double-precision)") (TriggeredSeconds :type "Float (double-precision)") (InputAction :type "InputAction Object Reference" :default "/Game/Player/Input/Actions/Movement/IA_Dodge_Roll.IA_Dodge_Roll"))
  (bind _returnvalue (`Actor.GetComponentByClass` (`self.GetOwner`) "/Game/Movement/Roll/Components/BPC_Roll.BPC_Roll_C"))
  ;[1 1 1] If clicked whilst being able to roll then we also have to check if we are currently dodging and if so then we will call the roll function in the roll component on the owner and if we cannot dodge but we are already dodging then we will also being the roll but if we are not dodging and we can infact dodge then the dodging bool will be set true which will then start the dodge animation in the animation blueprint
  (:`Triggered`
    (if (`self.Can Dodge`)
      (if (`self.Dodging`)
        (if (`/Game/Movement/Roll/Components/BPC_Roll.Can Roll` _returnvalue) :!label _label
          (`/Game/Movement/Roll/Components/BPC_Roll.Roll` _returnvalue))
        (else
          (set `self.Dodging` true)))
      (elif (`self.Dodging`)
        (goto _label)))))