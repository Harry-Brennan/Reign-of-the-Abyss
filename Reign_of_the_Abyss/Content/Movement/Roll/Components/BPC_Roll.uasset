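; BPC_Roll is an actor component that tracks roll availability and state for its owning actor.
; Every Tick it sets CanRoll when the owner is not falling or already rolling, and either can attack (BPC_AttackHandler) or is dodging (BPC_Dodge).
; The Roll event sets Rolling and clears the dodge state, so a roll can interrupt a dodge.
; Rolling is never reset within this graph.
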(event `self.ReceiveTick`
  (params (DeltaSeconds :type "Float (single-precision)"))
  (bind _returnvalue (`self.GetOwner`))
  (set `self.Can Roll` (and (not (`NavMovementComponent.IsFalling` (`Actor.GetComponentByClass` _returnvalue "/Script/Engine.CharacterMovementComponent"))) (or (`/Game/Combat/Components/BPC_AttackHandler.Can Attack` (`Actor.GetComponentByClass` _returnvalue "/Game/Combat/Components/BPC_AttackHandler.BPC_AttackHandler_C")) (`/Game/Movement/Dodge/Components/BPC_Dodge.Dodging` (`Actor.GetComponentByClass` _returnvalue "/Game/Movement/Dodge/Components/BPC_Dodge.BPC_Dodge_C"))) (not (`self.Rolling`)))))

(event `Roll`
  (set `self.Rolling` true)
  (set `/Game/Movement/Dodge/Components/BPC_Dodge.Dodging` false (`Actor.GetComponentByClass` (`self.GetOwner`) "/Game/Movement/Dodge/Components/BPC_Dodge.BPC_Dodge_C")))