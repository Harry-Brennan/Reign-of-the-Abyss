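; Ranged attack component that fires instant, charged and burst spells from its owning character.
; Start and Finish events track charge time, apply movement slow and store shot state for the animation blueprint.
; Shoot, not called within this graph, starts cooldown and spawns a projectile with charge-scaled stats, plus knockback, camera shake and HUD animation.
; Aim assist box-traces for the nearest valid target, falling back to a forward line trace.
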(event `Reset Charing Speed Slow`
  (goto _label_2 :!via `Reset`))

(event `Start Ranged Attack`
  (params (`Elapsed Seconds` :type "Float (double-precision)") (`Attempting Spell` :type "/Game/Combat/Ranged/Projectiles/Structs_Tables/Struct_Spell_Info Structure"))
  (bind _returnvalue (`Actor.GetComponentByClass` (`self.GetOwner`) "/Game/Movement/Basic_Movement/BPC_Movement_Manager.BPC_Movement_Manager_C"))
  (bind _returnvalue_2 (- `Elapsed Seconds` (`self.Triggered Seconds When Fired`)))
  ;[1 1 1] Starting a ranged attack with functionality for instant firing, charge firing and burst firing
  (bind _output_get (set `self.Current Attempted Spell Info` `Attempting Spell`))
  (bind (_spellname _generalinfo _uiinfo _spellcharacteristics _chargeinfo _instantinfo _burstinfo) (break `/Game/Combat/Ranged/Projectiles/Structs_Tables/Struct_Spell_Info` _output_get))
  (bind _returnvalue_3 (`KismetArrayLibrary.Array_Contains` _spellcharacteristics "NewEnumerator0"))
  (if _returnvalue_3
    (set `self.Charging Spell` true)
    (bind (_minimumchargetime _maximumchargetime _percentagemovementslow) (break `/Game/Combat/Ranged/Projectiles/Structs_Tables/Characteristics/Struct_Spell_Charge` _chargeinfo))
    ;;[1 1 1] HAVE WE EXCEEDED MAXIMUM CHARGE TIME
    (if (>= _returnvalue_2 _maximumchargetime)
      (`|ExecutionSequence`
        (:`then_0`
          (set `self.Charging Spell` false)
          (bind _returnvalue_4 (`KismetArrayLibrary.Array_Contains` _spellcharacteristics "NewEnumerator2"))
          (if _returnvalue_4
            (`self.Set Current Spell Variables` (`self.Current Attempted Spell Info`) `Elapsed Seconds` _burstinfo true :!label _label)
            (if _returnvalue_3
              (bind _returnvalue_5 (* _percentagemovementslow -1.0))
              (`/Game/Movement/Basic_Movement/BPC_Movement_Manager.Set Speed Multiplier` _returnvalue _returnvalue_5))
            (else
              (set `self.Firing Spell` true)
              (`self.Set Current Spell Variables` (`self.Current Attempted Spell Info`) `Elapsed Seconds`)
              (`/Game/Movement/Basic_Movement/BPC_Movement_Manager.Set Speed Multiplier` _returnvalue _returnvalue_5))))
        (:`then_1`
          (goto _label_2 :!via `Reset`)))
      (else
        ;;[1 1 1] Changing the speed of the character charging the charge spell that needs to be reset when the character stops charging
        (set `self.Current Charge Seconds` _returnvalue_2)
        (`/Engine/EditorBlueprintResources/StandardMacros.DoOnce` false :!label _label_2
          (:`Completed`
            (`/Game/Movement/Basic_Movement/BPC_Movement_Manager.Set Speed Multiplier` (`Actor.GetComponentByClass` (`self.GetOwner`) "/Game/Movement/Basic_Movement/BPC_Movement_Manager.BPC_Movement_Manager_C") _percentagemovementslow)))))
    (elif _returnvalue_4
      (set `self.Firing Spell` true)
      (goto _label)
      (else
        (set `self.Firing Spell` true)
        (`self.Set Current Spell Variables` (`self.Current Attempted Spell Info`) _returnvalue_2)))))

(event `Reset Charge`
  ;[1 1 1] Resets the charging time
  (set `self.Triggered Seconds When Fired` 0.0))

(event `Set Triggered Seconds When Fired`
  ;[1 1 1] In case there is a spell that has no cooldown that will be charged this allows for seamless transitions between charging -> firing -> back to charging
  (if (or (`self.Charging Spell`) (`/Game/Combat/Components/BPC_AttackHandler.Attempting to Ranged Attack` (`Actor.GetComponentByClass` (`self.GetOwner`) "/Game/Combat/Components/BPC_AttackHandler.BPC_AttackHandler_C")))
    (set `self.Triggered Seconds When Fired` (stale `Start Ranged Attack` `Elapsed Seconds`))
    (else
      (set `self.Triggered Seconds When Fired` 0.0))))

(event `Finish Ranged Attack`
  (params (`Elapsed Seconds` :type "Float (double-precision)"))
  (bind (_spellname _generalinfo _uiinfo _spellcharacteristics _chargeinfo) (break `/Game/Combat/Ranged/Projectiles/Structs_Tables/Struct_Spell_Info` (`self.Current Attempted Spell Info`)))
  (bind _returnvalue (- `Elapsed Seconds` (`self.Triggered Seconds When Fired`)))
  (bind (_minimumchargetime _maximumchargetime _percentagemovementslow) (break `/Game/Combat/Ranged/Projectiles/Structs_Tables/Characteristics/Struct_Spell_Charge` _chargeinfo))
  (bind _returnvalue_2 (* _percentagemovementslow -1.0))
  ;[1 1 1] Releasing attack mainly for charge firing
  (if (`KismetArrayLibrary.Array_Contains` _spellcharacteristics "NewEnumerator0")
    (if (>= _returnvalue _minimumchargetime)
      (set `self.Charging Spell` false)
      (if (`KismetArrayLibrary.Array_Contains` _spellcharacteristics "NewEnumerator2")
        (set `self.Firing Spell` true)
        (`self.Set Current Spell Variables` (`self.Current Attempted Spell Info`) _returnvalue (`.BurstInfo_40_BD5FFF864A13AF0BB17922806435E24A` (break `/Game/Combat/Ranged/Projectiles/Structs_Tables/Struct_Spell_Info` (`self.Current Attempted Spell Info`))) true)
        (`/Game/Movement/Basic_Movement/BPC_Movement_Manager.Set Speed Multiplier` (`Actor.GetComponentByClass` (`self.GetOwner`) "/Game/Movement/Basic_Movement/BPC_Movement_Manager.BPC_Movement_Manager_C") _returnvalue_2)
        (`self.Reset Charing Speed Slow`)
        (else
          (set `self.Firing Spell` true)
          (`self.Set Current Spell Variables` (`self.Current Attempted Spell Info`) _returnvalue)
          (`/Game/Movement/Basic_Movement/BPC_Movement_Manager.Set Speed Multiplier` (`Actor.GetComponentByClass` (`self.GetOwner`) "/Game/Movement/Basic_Movement/BPC_Movement_Manager.BPC_Movement_Manager_C") _returnvalue_2)
          (`self.Reset Charing Speed Slow`)))
      (else
        (set `self.Charging Spell` false)
        (`/Game/Movement/Basic_Movement/BPC_Movement_Manager.Set Speed Multiplier` (`Actor.GetComponentByClass` (`self.GetOwner`) "/Game/Movement/Basic_Movement/BPC_Movement_Manager.BPC_Movement_Manager_C") _returnvalue_2)
        (`self.Reset Charing Speed Slow`)))))

(event `Shoot`
  (params (`Spell Info` :type "/Game/Combat/Ranged/Projectiles/Structs_Tables/Struct_Spell_Info Structure") (`Charge Seconds` :type "Float (double-precision)") (Angle :type "Float (double-precision)") (`Original Spell Info (As in Spells Component)` :type "/Game/Combat/Ranged/Projectiles/Structs_Tables/Struct_Spell_Info Structure"))
  (bind (_spellname _generalinfo _uiinfo _spellcharacteristics _chargeinfo _instantinfo _burstinfo _piercinginfo _aoeinfo _splitinfo _hominginfo _attractinginfo) (break `/Game/Combat/Ranged/Projectiles/Structs_Tables/Struct_Spell_Info` `Spell Info`))
  (bind (_spelldamage _spellspeed _timetomaxspeed _shouldslowdown _slowdownstarttime _timeforslowdown _spellscale _spellduration _spellcooldown _spellshape _spellaimassistsize _spellcastmethod) (break `/Game/Combat/Ranged/Projectiles/Structs_Tables/Struct_Spell_General_Info` _generalinfo))
  (bind _returnvalue (`Actor.GetComponentByClass` (`self.GetOwner`) "/Game/Combat/Components/BPC_In_Combat_Checker.BPC_In_Combat_Checker_C"))
  (bind _returnvalue_2 (`|EnumEquality` (`.SpellCastMethod_35_D94EA3244382481C03E6A796F1DDE51E` (break `/Game/Combat/Ranged/Projectiles/Structs_Tables/Struct_Spell_General_Info` (`.GeneralInfo_32_E73347CC461F7538702134BFE7B28D2D` (break `/Game/Combat/Ranged/Projectiles/Structs_Tables/Struct_Spell_Info` `Spell Info`)))) "NewEnumerator0"))
  (bind _returnvalue_3 (/ `Charge Seconds` (`.MaximumChargeTime_5_4503AA2B415D7B5F1DDF069D70B7CA11` (break `/Game/Combat/Ranged/Projectiles/Structs_Tables/Characteristics/Struct_Spell_Charge` _chargeinfo))))
  (bind _returnvalue_4 (+ (.yaw (`Actor.K2_GetActorRotation` (`self.GetOwner`))) Angle))
  (bind _struct_spell_info (make `/Game/Combat/Ranged/Projectiles/Structs_Tables/Struct_Spell_Info` _spellname (select `bool` (`KismetArrayLibrary.Array_Contains` _spellcharacteristics "NewEnumerator0") :`false` _generalinfo :`true` (make `/Game/Combat/Ranged/Projectiles/Structs_Tables/Struct_Spell_General_Info` (* _spelldamage _returnvalue_3) (* _spellspeed _returnvalue_3) (* _timetomaxspeed _returnvalue_3) _shouldslowdown _slowdownstarttime _timeforslowdown (* _spellscale _returnvalue_3) (* _spellduration _returnvalue_3) _spellcooldown _spellshape _spellaimassistsize _spellcastmethod)) _uiinfo _spellcharacteristics _chargeinfo _instantinfo _burstinfo _piercinginfo _aoeinfo _splitinfo _hominginfo _attractinginfo))
  (bind ((`GeneralInfo_32_E73347CC461F7538702134BFE7B28D2D` _generalinfo_2) (`SpellCharacteristics_28_5646769B490CA7DBA8B01FB707622E22` _spellcharacteristics_2) (`ChargeInfo_36_6A627B1545A51F049C28D3B5D438A165` _chargeinfo_2) (`InstantInfo_38_B2497BF64D072E1A742E9C92ABF95903` _instantinfo_2)) (break `/Game/Combat/Ranged/Projectiles/Structs_Tables/Struct_Spell_Info` _struct_spell_info))
  ;[1 1 1] Actual firing function
  (`/Game/Combat/Ranged/Components/BPC_Spells.Start Spell Cooldown` (`Actor.GetComponentByClass` (`self.GetOwner`) "/Game/Combat/Ranged/Components/BPC_Spells.BPC_Spells_C") `Original Spell Info (As in Spells Component)`)
  (bind _static_mesh (message `/Game/Combat/Ranged/Interfaces/BPI_Has_Ranged_Attack.Get Ranged Weapon Mesh` (`self.GetOwner`)))
  (bind _vector (message `/Game/Combat/Ranged/Interfaces/BPI_Has_Ranged_Attack.Get_Hand_Cast_Loc` (`self.GetOwner`)))
  (bind _returnvalue_5 (`self.Find Look at Rotation For Spell / Aim Assist` (`KismetMathLibrary.MakeRotator` (.roll (`Actor.K2_GetActorRotation` (`self.GetOwner`))) (.pitch (`Actor.K2_GetActorRotation` (`self.GetOwner`))) (`KismetMathLibrary.SelectFloat` (- _returnvalue_4 360.0) _returnvalue_4 (>= _returnvalue_4 180.0))) _spellaimassistsize))
  (bind _returnvalue_6 (`SceneComponent.GetSocketLocation` _static_mesh "Fire Spell Socket"))
  (`|SpawnActorFromClass` "/Game/Combat/Ranged/Projectiles/BPs/BP_Spell_Projectile.BP_Spell_Projectile_C" (`KismetMathLibrary.MakeTransform` (`KismetMathLibrary.SelectVector` _returnvalue_6 _vector _returnvalue_2) (`KismetMathLibrary.FindLookAtRotation` (`KismetMathLibrary.SelectVector` _returnvalue_6 _vector _returnvalue_2) _returnvalue_5) (`.SpellScale_8_E11B722246D23D5911D27D8C60799466` (break `/Game/Combat/Ranged/Projectiles/Structs_Tables/Struct_Spell_General_Info` (`.GeneralInfo_32_E73347CC461F7538702134BFE7B28D2D` (break `/Game/Combat/Ranged/Projectiles/Structs_Tables/Struct_Spell_Info` _struct_spell_info))))) "AdjustIfPossibleButAlwaysSpawn" "MultiplyWithRoot" (`self.GetOwner`) _struct_spell_info null)
  (`self.Shoot Knockback` (`KismetMathLibrary.SelectFloat` (`.OppositionalKnockbackForce_9_AD3CFEA34179DE14729BF3A56A5AC852` (break `/Game/Combat/Ranged/Projectiles/Structs_Tables/Characteristics/Struct_Spell_Charge` _chargeinfo_2)) (`.OppositionalKnockbackForce_2_75E4E49F4092D0788D8079BF6265DA44` (break `/Game/Combat/Ranged/Projectiles/Structs_Tables/Characteristics/Struct_Spell_Instant` _instantinfo_2)) (`KismetArrayLibrary.Array_Contains` _spellcharacteristics_2 "NewEnumerator0")))
  (`self.Shoot Camera Shake` (`.SpellDamage_20_FD560B5F4CD3F0E02E8D65AC79277E69` (break `/Game/Combat/Ranged/Projectiles/Structs_Tables/Struct_Spell_General_Info` _generalinfo_2)))
  (bind _asbp_third_person_game_mode (cast `/Game/Modes_Instances/Modes/BP_ThirdPersonGameMode` (`GameplayStatics.GetGameMode`)))
  (`/Game/UI/HUD/Widgets/WBP_HUD.Play Spell Shoot Anim` (`/Game/Modes_Instances/Modes/BP_ThirdPersonGameMode.HUD Ref` _asbp_third_person_game_mode) (`KismetArrayLibrary.Array_Find` (`/Game/Modes_Instances/Modes/BP_ThirdPersonGameMode.Players` _asbp_third_person_game_mode) (`self.GetOwner`)))
  (`/Engine/EditorBlueprintResources/StandardMacros.IsValid` _returnvalue
    (:`Is Valid`
      (`/Game/Combat/Components/BPC_In_Combat_Checker.Delay In Combat Reset` _returnvalue))))

(fn `Get Current Shooting Info`
  (returns (`Spell Info` :type "/Game/Combat/Ranged/Projectiles/Structs_Tables/Struct_Spell_Info Structure") (Charge :type "Float (double-precision)") (`Burst Info` :type "/Game/Combat/Ranged/Projectiles/Structs_Tables/Characteristics/Struct_Spell_Burst Structure") (`Is Burst?` :type Boolean))
  (return (`self.Current Attempted Spell Info`) (`self.Current Charge Seconds`) (`self.Current Burst Info`) (`self.Is Burst`)))

(fn `Shoot Camera Shake`
  (params (`Spell Damage` :type "Float (double-precision)"))
  ;[1 1 1] Starts the spell shoot camera shake with the scale dependent on the spell's damage divided by 25 and clamped so it isn't too too too extreme
  (`LegacyCameraShake.StartLegacyCameraShake` (`GameplayStatics.GetPlayerCameraManager` 0) "/Game/Combat/Ranged/BPs/BP_Spell_Shoot_Camera_Shake.BP_Spell_Shoot_Camera_Shake_C" (`KismetMathLibrary.FClamp` (/ `Spell Damage` 25.0) 0.1 7.5) "World"))

(fn `Shoot Knockback`
  (params (`Knockback Amount` :type "Float (double-precision)"))
  (bind _returnvalue (`self.GetOwner`))
  ;[1 1 1] Knockbacks the character that is shooting the spell using the passed float parameter and casting from the owner of this component to launch the character
  (bind _ascharacter (cast `Character` _returnvalue))
  (`Character.LaunchCharacter` _ascharacter (* (* (`Actor.GetActorForwardVector` _returnvalue) -1.0) `Knockback Amount`) true false))