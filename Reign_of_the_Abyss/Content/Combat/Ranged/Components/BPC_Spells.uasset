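; Spell component that holds its owner's spell list, current selection and per-spell cooldowns.
; On BeginPlay it loads rows from DT_Spells: one random spell for enemies, all listed spells for other owners.
; Next/previous inputs cycle with wraparound and repeat while held, are blocked during charging, and update the player HUD.
; Cooldowns are timestamped and expired on Tick, which is enabled when one starts and disabled when none remain.
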(event `self.ReceiveBeginPlay`
  (bind _spells (`self.Spells`))
  ;[1 1 1] Small wait so that everything is setup properly
  (`KismetSystemLibrary.Delay` 0.2)
  ;[1 1 1] Precautionary clear of the spells array
  (`KismetArrayLibrary.Array_Clear` (`self.Spells`))
  ;[1 1 1] Get the characters spells
  (bind _character_s_spells (message `/Game/General_Character_Things/Interfaces/BPI_Character.Get Spells` (`self.GetOwner`)))
  ;[1 1 1] Checking if it is an enemy thjat is the owner of this component and if so we get a random spell and set that to be the spells that the enemy has so that I don't have to make a bunch of enemy rows and can just give them a number of spells and they will randomly choose one from them to use which also helps with variety
  (if (`KismetSystemLibrary.DoesImplementInterface` (`self.GetOwner`) "/Game/Enemies/Interfaces/BPI_Enemy.BPI_Enemy_C")
    (bind _returnvalue (`|GetDataTableRow` "/Game/Combat/Ranged/Projectiles/Structs_Tables/DT_Spells.DT_Spells" (`KismetStringLibrary.Conv_StringToName` (`|GetEnumeratorNameAsString` (`KismetArrayLibrary.Array_Random` _character_s_spells))))
      (:`then`
        (`KismetArrayLibrary.Array_Add` (`self.Spells`) _returnvalue)
        (`KismetArrayLibrary.Array_Add` (`self.Spell Cooldowns Active`))))
    (else
      ;[1 1 1] Loop through the character's spell names
      (for _array_element _character_s_spells
        ;[1 1 1] Find the spell info from the non-custom spells data table and add to array of spells and then also add to spell cooldowns active with false so that spell cooldowns can be tracked and the array is only the length of the number of spells that the owner of this component actually has
        (bind _returnvalue_2 (`|GetDataTableRow` "/Game/Combat/Ranged/Projectiles/Structs_Tables/DT_Spells.DT_Spells" (`KismetStringLibrary.Conv_StringToName` (`|GetEnumeratorNameAsString` _array_element)))
          (:`then`
            (`KismetArrayLibrary.Array_Add` (`self.Spells`) _returnvalue_2)
            (`KismetArrayLibrary.Array_Add` (`self.Spell Cooldowns Active`)))))))
  ;[1 1 1] Sets the current spell to be the first index of the spells array and sets the current spell index to be 0 since that is the index of the current spell
  (if (> (`KismetArrayLibrary.Array_Length` _spells) 0)
    (set `self.Current Spell` (`|GetArrayItem` _spells))
    (set `self.Current Spell Index` 0)
    (`self.Update Spell HUD`)))

(event `EnhancedInput|/Game/Player/Input/Actions/Ranged/IA_Next_Spell`
  (params (ActionValue :type Boolean) (ElapsedSeconds :type "Float (double-precision)") (TriggeredSeconds :type "Float (double-precision)") (InputAction :type "InputAction Object Reference" :default "/Game/Player/Input/Actions/Ranged/IA_Next_Spell.IA_Next_Spell"))
  ;[1 1 1] Input actions for selecting the next spell and the previous spell - this will work as long as the component is on a character with a controller and an input device - therefore if this needs to be used by NPCs then the functions just need to be called from the task to change spells
  (:`Triggered`
    (if (not (`/Game/Combat/Ranged/Components/BPC_Ranged_Attack.Charging Spell` (`Actor.GetComponentByClass` (`self.GetOwner`) "/Game/Combat/Ranged/Components/BPC_Ranged_Attack.BPC_Ranged_Attack_C")))
      (`|ExecutionSequence`
        (:`then_0`
          (`/Engine/EditorBlueprintResources/StandardMacros.DoOnce` false :!label _label
            (:`Completed`
              (`self.Next Spell`))))
        (:`then_1`
          (if (and (<= (mod TriggeredSeconds 0.3) 0.1) (>= TriggeredSeconds 0.3))
            (`/Engine/EditorBlueprintResources/StandardMacros.DoOnce` false :!label _label_2
              (:`Completed`
                (`self.Next Spell`)))
            (else
              (goto _label_2 :!via `Reset`)))))))
  (:`Canceled`
    (goto _label :!via `Reset`))
  (:`Completed`
    (goto _label :!via `Reset`)))

(event `self.ReceiveTick`
  (params (DeltaSeconds :type "Float (single-precision)"))
  ;[1 1 1] Looping through the array of spell cooldown infos that are on cooldown
  (for (_array_element _array_index) (`self.Spell Cooldowns`)
    (bind (_timecooldownstarted _cooldownduration _spellindex) (break `/Game/Combat/Ranged/Projectiles/Structs_Tables/Struct_Spell_Cooldown` _array_element))
    (if (>= (`KismetSystemLibrary.GetGameTimeInSeconds`) (+ _timecooldownstarted _cooldownduration))
      ;[1 1 1] Set the index at the spell cooldowns active bool array to false and then add to the spell cooldowns to remove index array with the current array's index
      (`KismetArrayLibrary.Array_Set` (`self.Spell Cooldowns Active`) _spellindex)
      (`KismetArrayLibrary.Array_Add` (`self.Spell Cooldowns To Remove`) _array_index)))
  ;[1 1 1] Looping through the indexes of spells that need to have their cooldowns stopped and then removing them from the spell info array and then removing from the array that is also being looped through
  (for (_array_element_2 _array_index_2) (`self.Spell Cooldowns To Remove`)
    (`KismetArrayLibrary.Array_Remove` (`self.Spell Cooldowns`) _array_element_2)
    (`KismetArrayLibrary.Array_Remove` (`self.Spell Cooldowns To Remove`) _array_index_2)
    (if (== (`self.Current Spell Index`) _array_index_2)
      (bind _asbp_third_person_game_mode (cast `/Game/Modes_Instances/Modes/BP_ThirdPersonGameMode` (`GameplayStatics.GetGameMode`)))
      (`/Game/UI/HUD/Widgets/WBP_HUD.Play Spell Cooldown End Anim` (`/Game/Modes_Instances/Modes/BP_ThirdPersonGameMode.HUD Ref` _asbp_third_person_game_mode) (`KismetArrayLibrary.Array_Find` (`/Game/Modes_Instances/Modes/BP_ThirdPersonGameMode.Players` _asbp_third_person_game_mode) (`self.GetOwner`)))))
  ;[1 1 1] If there are no spells that are on cooldown then the tick of this component will be disabled
  (if (`KismetArrayLibrary.Array_IsEmpty` (`self.Spell Cooldowns`))
    (`self.SetComponentTickEnabled` false)))

(event `EnhancedInput|/Game/Player/Input/Actions/Ranged/IA_Previous_Spell`
  (params (ActionValue :type Boolean) (ElapsedSeconds :type "Float (double-precision)") (TriggeredSeconds :type "Float (double-precision)") (InputAction :type "InputAction Object Reference" :default "/Game/Player/Input/Actions/Ranged/IA_Previous_Spell.IA_Previous_Spell"))
  ;[1 1 1] Input actions for selecting the next spell and the previous spell - this will work as long as the component is on a character with a controller and an input device - therefore if this needs to be used by NPCs then the functions just need to be called from the task to change spells
  (:`Triggered`
    (if (not (`/Game/Combat/Ranged/Components/BPC_Ranged_Attack.Charging Spell` (`Actor.GetComponentByClass` (`self.GetOwner`) "/Game/Combat/Ranged/Components/BPC_Ranged_Attack.BPC_Ranged_Attack_C")))
      (`|ExecutionSequence`
        (:`then_0`
          (`/Engine/EditorBlueprintResources/StandardMacros.DoOnce` false :!label _label_3
            (:`Completed`
              (`self.Previous Spell`))))
        (:`then_1`
          (if (and (<= (mod TriggeredSeconds 0.3) 0.1) (>= TriggeredSeconds 0.3))
            (`/Engine/EditorBlueprintResources/StandardMacros.DoOnce` false :!label _label_4
              (:`Completed`
                (`self.Previous Spell`)))
            (else
              (goto _label_4 :!via `Reset`)))))))
  (:`Ongoing`
    (goto _label_3 :!via `Reset`))
  (:`Canceled`
    (goto _label_3 :!via `Reset`)))

(fn `Next Spell`
  (bind _returnvalue (`KismetMathLibrary.SelectInt` 0 (+ (`self.Current Spell Index`) 1) (>= (`self.Current Spell Index`) (- (`KismetArrayLibrary.Array_Length` (`self.Spells`)) 1))))
  ;[1 1 1] Sets the current spell index and current spell info variable to be either the next spell index or to 0 if we have reached the end of the array / the length of the array - 1
  (set `self.Current Spell` (`|GetArrayItem` (`self.Spells`) _returnvalue))
  (set `self.Current Spell Index` _returnvalue)
  (`self.Update Spell HUD`))

(fn `Previous Spell`
  (bind _returnvalue (`KismetMathLibrary.SelectInt` (- (`KismetArrayLibrary.Array_Length` (`self.Spells`)) 1) (- (`self.Current Spell Index`) 1) (<= (`self.Current Spell Index`) 0)))
  ;[1 1 1] Select the int of the next spell index based on if we have reached 0 or less for the current spell index and if so then loop back to the end of the array if not then the current spell index is set to one less of the current spell index also sets the current spell info based on the selected int from the array of spells
  (set `self.Current Spell` (`|GetArrayItem` (`self.Spells`) _returnvalue))
  (set `self.Current Spell Index` _returnvalue)
  (`self.Update Spell HUD`))

(fn `Start Spell Cooldown`
  (params (`Spell Info` :type "/Game/Combat/Ranged/Projectiles/Structs_Tables/Struct_Spell_Info Structure"))
  (bind _spells (`self.Spells`))
  (bind _returnvalue (`KismetArrayLibrary.Array_Find` _spells `Spell Info`))
  ;[1 1 1] Passing the spell that should have its cooldown started
  (if (`KismetArrayLibrary.Array_IsValidIndex` _spells _returnvalue)
    ;[1 1 1] Set the passed spell's index in the spell cooldowns active bool array to be true
    ;;[1 1 1] Add this struct to the spell cooldown array
    (`KismetArrayLibrary.Array_Add` (`self.Spell Cooldowns`) (make `/Game/Combat/Ranged/Projectiles/Structs_Tables/Struct_Spell_Cooldown` (`KismetSystemLibrary.GetGameTimeInSeconds`) (`.SpellCooldown_17_D857444B4AF40445F837C6A34351379E` (break `/Game/Combat/Ranged/Projectiles/Structs_Tables/Struct_Spell_General_Info` (`.GeneralInfo_32_E73347CC461F7538702134BFE7B28D2D` (break `/Game/Combat/Ranged/Projectiles/Structs_Tables/Struct_Spell_Info` (`|GetArrayItem` (`self.Spells`) _returnvalue))))) _returnvalue))
    (`KismetArrayLibrary.Array_Set` (`self.Spell Cooldowns Active`) _returnvalue true)
    ;[1 1 1] Start the cooldown by setting the tick of the component active
    (`self.SetComponentTickEnabled` true)))

(fn `Update Spell HUD`
  (if (`KismetSystemLibrary.DoesImplementInterface` (`self.GetOwner`) "/Game/Player/Interfaces/BPI_Player.BPI_Player_C")
    (bind _asbp_third_person_game_mode (cast `/Game/Modes_Instances/Modes/BP_ThirdPersonGameMode` (`GameplayStatics.GetGameMode`)))
    (`/Game/UI/HUD/Widgets/WBP_HUD.Update Spell` (`/Game/Modes_Instances/Modes/BP_ThirdPersonGameMode.HUD Ref` _asbp_third_person_game_mode) (`.SpellName_27_5665ABAF49EC6DACF2667599D030ED83` (break `/Game/Combat/Ranged/Projectiles/Structs_Tables/Struct_Spell_Info` (`self.Current Spell`))) (`KismetArrayLibrary.Array_Find` (`/Game/Modes_Instances/Modes/BP_ThirdPersonGameMode.Players` _asbp_third_person_game_mode) (`self.GetOwner`)))))