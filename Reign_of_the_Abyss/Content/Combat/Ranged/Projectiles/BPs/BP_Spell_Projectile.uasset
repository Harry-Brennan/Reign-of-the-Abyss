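; Spell projectile actor whose speed, mesh, scale and behavior come from SpellInfo, filled from DT_NonCustom_Spells for non-custom spells.
; BeginPlay adds AOE, Homing and Split components according to the spell's characteristics.
; On impact or lifetime expiry, a sphere trace damages and knocks back pawns via BPC_Health and sends physics bodies a zero-valued impulse.
; It then triggers AOE and any unused Split before destroying itself.
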(event `self.ReceiveBeginPlay`
  (bind ((`SpellCharacteristics_28_5646769B490CA7DBA8B01FB707622E22` _spellcharacteristics)) (break `/Game/Combat/Ranged/Projectiles/Structs_Tables/Struct_Spell` (`self.Spell Info`)))
  (bind (_spelldamage _spellspeed _timetomaxspeed _spellscale _spellduration _spellcooldown _spellshape) (break `/Game/Combat/Ranged/Projectiles/Structs_Tables/Struct_Spell_General_Info` (`.GeneralInfo_32_E73347CC461F7538702134BFE7B28D2D` (break `/Game/Combat/Ranged/Projectiles/Structs_Tables/Struct_Spell` (`self.Spell Info`)))))
  (for _array_element (`.SpellCharacteristics_28_5646769B490CA7DBA8B01FB707622E22` (break `/Game/Combat/Ranged/Projectiles/Structs_Tables/Struct_Spell` (`self.Spell Info`)))
    (`KismetSystemLibrary.PrintString` (`|GetEnumeratorNameAsString` _array_element)))
  (set `ProjectileMovementComponent.InitialSpeed` _spellspeed (`self.ProjectileMovement`))
  (`StaticMeshComponent.SetStaticMesh` (`self.StaticMesh`) _spellshape)
  (`self.SetActorScale3D` _spellscale)
  (`|ExecutionSequence`
    (:`then_0`
      ;[1 1 1] Adding corresponding components based on the characteristics of the spell including AOE, Split, and Homing
      (if (`KismetArrayLibrary.Array_Contains` _spellcharacteristics "NewEnumerator4")
        (bind _returnvalue (`AddComponent|NODE_AddBPC_AOE-0`))
        (set `self.AOE Component` _returnvalue))
      (if (`KismetArrayLibrary.Array_Contains` _spellcharacteristics "NewEnumerator6")
        (bind _returnvalue_2 (`AddComponent|NODE_AddBPC_Homing-0`))
        (set `self.Homing Component` _returnvalue_2))
      (if (`KismetArrayLibrary.Array_Contains` _spellcharacteristics "NewEnumerator5")
        (bind _returnvalue_3 (`AddComponent|NODE_AddBPC_Split-0`))
        (set `self.Split Component` _returnvalue_3))
      ;[1 1 1] Delay for the spell duration which will then activate the correct component functions based on the spell characteristics only activating if the spell projectile is valid after the dela / lifetime of the spell
      (`KismetSystemLibrary.Delay` (`.SpellDuration_11_024EB84E4B15A3F12FF2B1BEB85D9F0D` (break `/Game/Combat/Ranged/Projectiles/Structs_Tables/Struct_Spell_General_Info` (`.GeneralInfo_32_E73347CC461F7538702134BFE7B28D2D` (break `/Game/Combat/Ranged/Projectiles/Structs_Tables/Struct_Spell` (`self.Spell Info`))))))
      (`self.Spell EOL`))
    (:`then_1`
      (`KismetSystemLibrary.Delay` 0.1)
      (`PrimitiveComponent.SetCollisionProfileName` (`self.StaticMesh`) "BlockAllDynamic" true))))

(event `Spell EOL`
  (bind _split_component (`self.Split Component`))
  ;[1 1 1] Spell End Of Life
  (set `self.Natural EOL` true)
  (bind _returnvalue (`KismetMathLibrary.SelectVector` (`self.K2_GetActorLocation`) (`.Location` (`GameplayStatics.BreakHitResult` (stale `self.ProjectileMovement.OnProjectileStop` ImpactResult))) (`self.Natural EOL`)))
  ;[1 1 1] Multi sphere trace detecting characters hit and physics bodies hit at the stopped location
  (bind (_outhits _returnvalue_2) (`KismetSystemLibrary.SphereTraceMultiForObjects` :`Start` _returnvalue :`End` _returnvalue :`Radius` (* (`.SphereRadius` (`KismetSystemLibrary.GetComponentBounds` (`self.StaticMesh`))) 1.5) :`ObjectTypes` (`|MakeArray` "ObjectTypeQuery3" "ObjectTypeQuery4" :!type "EObjectTypeQuery Enum") :`DrawDebugType` "ForDuration" :!label _label))
  ;[1 1 1] Only check if actually hit something
  (if _returnvalue_2
    ;[1 1 1] Looping through hit targets both pawns and physiocs bodies and then applying damage to hit characters and knockback to hit characters and knockback to hit physics objects
    (for _array_element _outhits
      (bind (_bblockinghit _binitialoverlap _time _distance _location _impactpoint _normal _impactnormal _physmat _hitactor _hitcomponent) (`GameplayStatics.BreakHitResult` _array_element))
      (if (not (`KismetArrayLibrary.Array_Contains` (`self.Hit Characters`) _hitactor))
        (`KismetArrayLibrary.Array_Add` (`self.Hit Characters`) _hitactor)
        (switch `ECollisionChannel` (`PrimitiveComponent.GetCollisionObjectType` _hitcomponent)
          (:`ECC_Pawn`
            (`/Game/Health/Components/BPC_Health.Take Damage` (`self.GetComponentByClass` _hitactor "/Game/Health/Components/BPC_Health.BPC_Health_C") (`.SpellDamage_20_FD560B5F4CD3F0E02E8D65AC79277E69` (break `/Game/Combat/Ranged/Projectiles/Structs_Tables/Struct_Spell_General_Info` (`.GeneralInfo_32_E73347CC461F7538702134BFE7B28D2D` (break `/Game/Combat/Ranged/Projectiles/Structs_Tables/Struct_Spell` (`self.Spell Info`))))) (`self.GetOwner`) _impactnormal _location 1000.0 650.0))
          (:`ECC_PhysicsBody`
            (`PrimitiveComponent.AddImpulse` _hitcomponent (0.0 0.0 0.0) "None" true))))))
  ;[1 1 1] Activating AOE and/or split depending on the validity of the corresponding components and then destroying the spell projectile
  (`|ExecutionSequence`
    (:`then_0`
      (`/Engine/EditorBlueprintResources/StandardMacros.IsValid` (`self.AOE Component`)
        (:`Is Valid`
          (`/Game/Combat/Ranged/Projectiles/Components/BPC_AOE.AOE` (`self.AOE Component`)))))
    (:`then_1`
      (`/Engine/EditorBlueprintResources/StandardMacros.IsValid` _split_component
        (:`Is Valid`
          (if (not (`/Game/Combat/Ranged/Projectiles/Components/BPC_Split.Have Split` _split_component))
            (`/Game/Combat/Ranged/Projectiles/Components/BPC_Split.Split` (`self.Split Component`))))))
    (:`then_2`
      (`self.K2_DestroyActor`))))

(event `self.ProjectileMovement.OnProjectileStop`
  (params (ImpactResult :type "HitResult Structure (by ref)"))
  ;[1 1 1] When projectile hits something
  (`KismetArrayLibrary.Array_Clear` (`self.Hit Characters`))
  (set `self.Natural EOL` false)
  (`KismetSystemLibrary.PrintString` (`KismetStringLibrary.Concat_StrStr` "HIT: " (`KismetSystemLibrary.GetDisplayName` (`.HitActor` (`GameplayStatics.BreakHitResult` ImpactResult)))))
  (goto _label))

(fn `Get Spell Info`
  (returns (`Spell Info` :type "/Game/Combat/Ranged/Projectiles/Structs_Tables/Struct_Spell Structure"))
  (return (`self.Spell Info`)))

(fn `UserConstructionScript`
  (bind ((`SpellName_27_5665ABAF49EC6DACF2667599D030ED83` _spellname) (`CustomSpell_34_144D0638476B4E35E3FC448C67567152` _customspell)) (break `/Game/Combat/Ranged/Projectiles/Structs_Tables/Struct_Spell` (`self.Spell Info`)))
  (bind (_spelldamage _spellspeed _timetomaxspeed _spellscale _spellduration _spellcooldown _spellshape) (break `/Game/Combat/Ranged/Projectiles/Structs_Tables/Struct_Spell_General_Info` (`.GeneralInfo_32_E73347CC461F7538702134BFE7B28D2D` (break `/Game/Combat/Ranged/Projectiles/Structs_Tables/Struct_Spell` (`self.Spell Info`)))))
  (if (not _customspell)
    (bind _returnvalue (`|GetDataTableRow` "/Game/Combat/Ranged/Projectiles/Structs_Tables/DT_Non-Custom_Spells.DT_Non-Custom_Spells" (`KismetStringLibrary.Conv_StringToName` (`|GetEnumeratorNameAsString` _spellname)))
      (:`then`
        (set `self.Spell Info` _returnvalue))))
  (set `ProjectileMovementComponent.InitialSpeed` _spellspeed (`self.ProjectileMovement`))
  (`StaticMeshComponent.SetStaticMesh` (`self.StaticMesh`) _spellshape)
  (`self.SetActorScale3D` _spellscale))