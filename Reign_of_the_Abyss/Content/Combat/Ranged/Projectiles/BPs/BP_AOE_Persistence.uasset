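; Lingering area-of-effect left by an exploded projectile that slows characters standing inside it for a set duration.
; BeginPlay sizes the overlap sphere from Radius and spawns a fading, tinted blood decal using a dynamic material.
; Overlaps pass the slow to each BPI_Character's movement manager and its negation on exit, tracking actors to avoid duplicates.
; The actor destroys itself at 90% of Duration to match the visual fade.
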(event `self.ReceiveBeginPlay`
  (bind _returnvalue (* (`self.Radius`) 1.5))
  ;[1 1 1] Spawn the bllood decal at the projectile's location when it exploded and set its size to be 128, and then 1.5 * the radius of the actual AOE with the rotation as -90.
  (bind _returnvalue_2 (`GameplayStatics.SpawnDecalAtLocation` "/Game/VFX/Blood_Splatter/Materials/MI_Blood_Decal_Advanced.MI_Blood_Decal_Advanced" (`KismetMathLibrary.MakeVector` 128.0 _returnvalue _returnvalue) (`self.K2_GetActorLocation`)))
  ;[1 1 1] Set the fadeout duration of the decal to be the duration of the AOE persistence
  (`DecalComponent.SetFadeOut` _returnvalue_2 0.0 (`self.Duration`) true)
  ;[1 1 1] Create a dynamic material instance of the blood
  (bind _returnvalue_3 (`DecalComponent.CreateDynamicMaterialInstance` _returnvalue_2))
  ;[1 1 1] Set the radius parameter of the blood material to be 1.5 * the radius of the AOE
  (`MaterialInstanceDynamic.SetScalarParameterValue` _returnvalue_3 "Radius" (* (`self.Radius`) 1.5))
  ;[1 1 1] Set the sphere radius of the collision to be the radius of the AOE
  (`SphereComponent.SetSphereRadius` (`self.Sphere`) (`self.Radius`) true)
  ;[1 1 1] Set the colour of the blood material - currently just blue to be distinguishable
  (`MaterialInstanceDynamic.SetVectorParameterValue` _returnvalue_3 "Colour" (struct :`G` 0.541019 :`B` 1.0 :`A` 1.0))
  ;[1 1 1] Start a delay with the length of the duration of the AOE persistence but silghtly less since the fadeout makes it look like the AOE persistence is gone before it actually is and then after the delay destroy this actor
  (`KismetSystemLibrary.Delay` (* (`self.Duration`) 0.9))
  (`self.K2_DestroyActor`))

(event `self.Sphere.OnComponentBeginOverlap`
  (params (OverlappedComponent :type "PrimitiveComponent Object Reference") (OtherActor :type "Actor Object Reference") (OtherComp :type "PrimitiveComponent Object Reference") (OtherBodyIndex :type Integer) (bFromSweep :type Boolean) (SweepResult :type "HitResult Structure (by ref)"))
  (bind _affected_characters (`self.Affected Characters`))
  ;[1 1 1] When an actor begins overlapping the collision check if it is already in the affected characters array and if it isn't then add it to the array and check if it is a character and then update the speed multiplier of the character passing the slow of this AOE persistence as the speed multiplier difference
  (if (not (`KismetArrayLibrary.Array_Contains` _affected_characters OtherActor))
    (`KismetArrayLibrary.Array_Add` _affected_characters OtherActor)
    (if (`KismetSystemLibrary.DoesImplementInterface` OtherActor "/Game/General_Character_Things/Interfaces/BPI_Character.BPI_Character_C")
      (`/Game/Movement/Basic_Movement/BPC_Movement_Manager.Set Speed Multiplier` (`self.GetComponentByClass` OtherActor "/Game/Movement/Basic_Movement/BPC_Movement_Manager.BPC_Movement_Manager_C") (`self.Percentage Slow`)))))

(event `self.Sphere.OnComponentEndOverlap`
  (params (OverlappedComponent :type "PrimitiveComponent Object Reference") (OtherActor :type "Actor Object Reference") (OtherComp :type "PrimitiveComponent Object Reference") (OtherBodyIndex :type Integer))
  ;[1 1 1] When a character leaves the collision remove it from the array of characters and then check if it actually i a character and update the character's speed multiplier by getting the percentage slow and getting the inverse to take away from the character's speed multiplier
  (`KismetArrayLibrary.Array_RemoveItem` (`self.Affected Characters`) OtherActor)
  (if (`KismetSystemLibrary.DoesImplementInterface` OtherActor "/Game/General_Character_Things/Interfaces/BPI_Character.BPI_Character_C")
    (`/Game/Movement/Basic_Movement/BPC_Movement_Manager.Set Speed Multiplier` (`self.GetComponentByClass` OtherActor "/Game/Movement/Basic_Movement/BPC_Movement_Manager.BPC_Movement_Manager_C") (* (`self.Percentage Slow`) -1.0))))

(fn `UserConstructionScript`)