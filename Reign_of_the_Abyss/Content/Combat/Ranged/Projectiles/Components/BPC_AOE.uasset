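; Projectile component that detonates a spell's area-of-effect blast, using the owner's spell info for VFX, sound and distance-scaled camera shake.
; A sphere trace hits each actor once, pushing physics bodies, damaging players, enemies and payloads, and adding status effects to characters.
; Horizontal-distance falloff scales impulse, vertical knockback and character damage (derived from MaximumKnockback), while payload damage stays flat.
; Optionally, a downward trace places a BP_AOE_Persistence zone on the floor.
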(fn `AOE`
  (locals (`Hit Actors` :type "Array of Actor Object Reference"))
  (bind _returnvalue (`self.GetOwner`))
  (bind _returnvalue_2 (`self.GetOwner`))
  (bind _returnvalue_3 (`self.GetOwner`))
  (bind (_returnvalue_x _returnvalue_y) (`KismetMathLibrary.BreakVector` (`Actor.K2_GetActorLocation` (`self.GetOwner`))))
  (bind _returnvalue_4 (`Actor.K2_GetActorLocation` _returnvalue))
  (bind _returnvalue_5 (`Actor.GetOwner` (`self.GetOwner`)))
  (bind _returnvalue_6 (`Actor.K2_GetActorLocation` _returnvalue_3))
  (bind _spell_info (message `/Game/Combat/Ranged/Projectiles/Interfaces/BPI_Spell.Get Spell Info` _returnvalue_2))
  (bind ((`AOEInfo_56_82970EA5401F2C2A7623458E4EEA83C0` _aoeinfo) (`AudioInfo_66_023905E04BEB1D481DE5AAABC05F3EEC` _audioinfo)) (break `/Game/Combat/Ranged/Projectiles/Structs_Tables/Struct_Spell_Info` _spell_info))
  (`NiagaraFunctionLibrary.SpawnSystemAtLocation` (`.AOEVFX_31_6E8C0C784F037F6309478582782FF1DC` (break `/Game/Combat/Ranged/Projectiles/Structs_Tables/Characteristics/Struct_Spell_AOE` _aoeinfo)) (`Actor.K2_GetActorLocation` _returnvalue_2))
  (bind _returnvalue_7 (`GameplayStatics.GetActorOfClass` "/Game/Co-op/Camera/BP_Camera.BP_Camera_C"))
  (`LegacyCameraShake.StartLegacyCameraShake` (`GameplayStatics.GetPlayerCameraManager` 0) "/Game/Combat/Ranged/BPs/BP_Spell_Shoot_Camera_Shake.BP_Spell_Shoot_Camera_Shake_C" (`KismetMathLibrary.FClamp` (- 6.0 (/ (`KismetMathLibrary.Vector_Distance` (`Actor.K2_GetActorLocation` (`self.GetOwner`)) (`Actor.K2_GetActorLocation` _returnvalue_7)) 2000.0)) 0.5 8.0))
  (`GameplayStatics.PlaySoundAtLocation` (`.Explode_Cue_6_4E203B034B028D4C852BA9A06B1C7287` (break `/Game/Combat/Ranged/Projectiles/Structs_Tables/Struct_Spell_Audio` _audioinfo)) (`Actor.K2_GetActorLocation` (`self.GetOwner`)) (struct) 1.0 1.0 0.0 null null null null)
  ;[1 1 1] Clear hit actors array as a precaution
  (`KismetArrayLibrary.Array_Clear` (`local.Hit Actors`))
  ;[1 1 1] Get spell info for this aoe
  (bind _spell_info_2 (message `/Game/Combat/Ranged/Projectiles/Interfaces/BPI_Spell.Get Spell Info` _returnvalue_3))
  (bind ((`BlastRadius_4_3492033443B8005980361DAAA80022D1` _blastradius) (`BlastDamage_5_A273AC134EBF32F6AEFE49ACD4D1C7C2` _blastdamage) (`MaximumPercentageDamageFalloff_8_DD8BAC65409BAE6D6DD3C0BC522A3320` _maximumpercentagedamagefalloff) (`MaximumKnockback_10_040115324DA9D94B03D42588E1406240` _maximumknockback) (`MaximumPercentageKnockbackFalloff_12_D9E3DE2B4E160937D800B2A4571A8C38` _maximumpercentageknockbackfalloff) (`AOEStatusEffect_27_EE2161454CE49DE0DE21E1A99094D592` _aoestatuseffect) (`PersistingAOE?_16_70343A3344CDE3A0B289B8A5D7EA3386` _persistingaoe_) (`PersistingAOEDuration_19_FF5894B54DF6620AD74C339FC6BD57A6` _persistingaoeduration) (`PersistingAOEPercentageSlow_22_459E4DDF466812DEACD21C916C5A24EB` _persistingaoepercentageslow) (`PersistingAOEStatusEffect_28_8FCFD4BC4E13A5687D1EF985A6BA3C0B` _persistingaoestatuseffect) (`AOEPersistenceColour_34_53835C064B50D1EB3ABD04B2961F8EF3` _aoepersistencecolour)) (break `/Game/Combat/Ranged/Projectiles/Structs_Tables/Characteristics/Struct_Spell_AOE` (`.AOEInfo_56_82970EA5401F2C2A7623458E4EEA83C0` (break `/Game/Combat/Ranged/Projectiles/Structs_Tables/Struct_Spell_Info` _spell_info_2))))
  ;[1 1 1] Sphere trace for pawns and physics bodies with radius of blast radius at the projectile's location
  (bind (_outhits _returnvalue_8) (`KismetSystemLibrary.SphereTraceMultiForObjects` _returnvalue_6 _returnvalue_6 _blastradius (`|MakeArray` "ObjectTypeQuery7" "ObjectTypeQuery8" "ObjectTypeQuery9" "ObjectTypeQuery4" :!type "EObjectTypeQuery Enum")))
  (if _returnvalue_8
    (for _array_element _outhits
      (bind (_bblockinghit _binitialoverlap _time _distance _location _impactpoint _normal _impactnormal _physmat _hitactor _hitcomponent) (`GameplayStatics.BreakHitResult` _array_element))
      ;[1 1 1] Check if we've already hit the actor
      (if (not (`KismetArrayLibrary.Array_Contains` (`local.Hit Actors`) _hitactor))
        ;[1 1 1] Add to hit actors
        (`KismetArrayLibrary.Array_Add` (`local.Hit Actors`) _hitactor)
        (switch `ECollisionChannel` (`PrimitiveComponent.GetCollisionObjectType` _hitcomponent)
          (:`ECC_PhysicsBody`
            (bind _z (.z (`Actor.K2_GetActorLocation` _hitactor)))
            (bind _returnvalue_9 (* _maximumknockback (- 1.0 (`KismetMathLibrary.FClamp` (/ (- (`KismetMathLibrary.VSize` (- (`KismetMathLibrary.MakeVector` _returnvalue_x _returnvalue_y _z) (`KismetMathLibrary.MakeVector` (.x (`Actor.K2_GetActorLocation` _hitactor)) (.y (`Actor.K2_GetActorLocation` _hitactor)) _z))) 10.0) _blastradius) 0.0 _maximumpercentageknockbackfalloff))))
            ;[1 1 1] Add impulse to the physics body away from the epicentre of the AOE
            (`PrimitiveComponent.AddImpulse` _hitcomponent (* (`KismetMathLibrary.GetForwardVector` (`KismetMathLibrary.FindLookAtRotation` (`Actor.K2_GetActorLocation` (`self.GetOwner`)) _location)) _returnvalue_9) "None" true))
          (:`ECC_GameTraceChannel1`
            (bind _returnvalue_10 (* _blastdamage (- 1.0 0.0)))
            (`/Game/Health/Components/BPC_Health_V2.Take Damage` (`Actor.GetComponentByClass` _hitactor "/Game/Health/Components/BPC_Health_V2.BPC_Health_V2_C") (/ _returnvalue_9 2.0) _returnvalue_5 _impactnormal _location _returnvalue_10 _returnvalue_9 0.0 :!label _label)
            ;[1 1 1] Applying on hit status effects to the hit targets
            (for _array_element_2 (`.PossibleStatus_23_30BE313C410E5C82B6F330A9E0495AFC` (break `/Game/Combat/Status_Effects/Structs_Tables/Struct_Status_Effects` _aoestatuseffect))
              (`/Game/Combat/Status_Effects/Components/BPC_StatusEffectHandler.Add Status` (`Actor.GetComponentByClass` _hitactor "/Game/Combat/Status_Effects/Components/BPC_StatusEffectHandler.BPC_StatusEffectHandler_C") _array_element_2 _aoestatuseffect (`Actor.GetOwner` (`self.GetOwner`)))))
          (:`ECC_GameTraceChannel2`
            (goto _label))
          (:`ECC_GameTraceChannel3`
            (`/Game/Health/Components/BPC_PayloadHealth.TakeDamage` (`Actor.GetComponentByClass` _hitactor "/Game/Health/Components/BPC_PayloadHealth.BPC_PayloadHealth_C") _returnvalue_10 _returnvalue_5))))))
  ;[1 1 1] Check if we should spawn an aoe persistence
  (if _persistingaoe_
    ;[1 1 1] line trace for world static and world dynamic objects down a lot to find the floor below the projectile which is where the aoe persistence will be spawned
    (bind (_outhit _returnvalue_11) (`KismetSystemLibrary.LineTraceSingleForObjects` _returnvalue_4 (+ (* (`Actor.GetActorUpVector` _returnvalue) -500000.0) _returnvalue_4) (`|MakeArray` "ObjectTypeQuery2" "ObjectTypeQuery1" :!type "EObjectTypeQuery Enum")))
    (bind (_bblockinghit_2 _binitialoverlap_2 _time_2 _distance_2 _location_2 _impactpoint_2 _normal_2 _impactnormal_2 _physmat_2 _hitactor_2 _hitcomponent_2 _hitbonename _bonename _hititem _elementindex _faceindex _tracestart _traceend) (`GameplayStatics.BreakHitResult` _outhit))
    ;[1 1 1] Spawn an aoe persistence either at the trace's hit location or the trace end depending on if the trace hit with the aoe persistence info being passed from the aoe info in the spell info and the owner set as the owner of this spell projectile
    (`|SpawnActorFromClass` "/Game/Combat/Ranged/Projectiles/BPs/BP_AOE_Persistence.BP_AOE_Persistence_C" (`KismetMathLibrary.MakeTransform` (`KismetMathLibrary.SelectVector` _location_2 _traceend _returnvalue_11)) "Undefined" "MultiplyWithRoot" (`Actor.GetOwner` (`self.GetOwner`)) _persistingaoeduration _persistingaoepercentageslow _blastradius _persistingaoestatuseffect _aoepersistencecolour null)))