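; Actor component that gives spell projectiles piercing behaviour, with an optional pierce limit and falloff of damage, speed and scale.
; Each pierce damages a valid character through its health component, or otherwise pushes the physics body with a velocity-change impulse.
; It then counts the pierce and either triggers the projectile's end of life at the limit or rewrites its SpellInfo with the multiplied values.
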(fn `Pierced`
  (params (`Pierced Character` :type "Actor Object Reference") (`Pierced Physics Body` :type "PrimitiveComponent Object Reference"))
  (`/Engine/EditorBlueprintResources/StandardMacros.IsValid` `Pierced Character`
    (:`Is Valid`
      ;[1 1 1] Apply damage to pierced character applying directional normal by subtracing the location of the projectile from the location of the hit actor normalised
      (`KismetSystemLibrary.PrintString` "SPELL PIERCED")
      (bind _spell_info (message `/Game/Combat/Ranged/Projectiles/Interfaces/BPI_Spell.Get Spell Info` (`self.GetOwner`)))
      (`/Game/Health/Components/BPC_Health.Take Damage` (`Actor.GetComponentByClass` `Pierced Character` "/Game/Health/Components/BPC_Health.BPC_Health_C") (break `/Game/Combat/Ranged/Projectiles/Structs_Tables/Struct_Spell_General_Info` (`.GeneralInfo_32_E73347CC461F7538702134BFE7B28D2D` (break `/Game/Combat/Ranged/Projectiles/Structs_Tables/Struct_Spell_Info` _spell_info))) (`Actor.GetOwner` (`self.GetOwner`)) (`KismetMathLibrary.Normal` (- (`Actor.K2_GetActorLocation` (`self.GetOwner`)) (`Actor.K2_GetActorLocation` `Pierced Character`))) (`Actor.K2_GetActorLocation` (`self.GetOwner`)) 100.0 0.0))
    (:`Is Not Valid`
      (`/Engine/EditorBlueprintResources/StandardMacros.IsValid` `Pierced Physics Body`
        (:`Is Valid`
          ;[1 1 1] Add impulse to pierced physics bodies in the direction of the projectile to the hit physics body
          (`PrimitiveComponent.AddImpulse` `Pierced Physics Body` (* (`KismetMathLibrary.GetForwardVector` (`KismetMathLibrary.FindLookAtRotation` (`Actor.K2_GetActorLocation` (`self.GetOwner`)) (`SceneComponent.K2_GetComponentLocation` `Pierced Physics Body`))) 500.0) "None" true))
        (:`Is Not Valid`
          _))))
  ;[1 1 1] Increment active piercings
  (`/Engine/EditorBlueprintResources/StandardMacros.IncrementInt` (`self.Active Piercings`)
    (:`  `
      (if (and (`self.Has Max Number of Piercings?`) (>= (`self.Active Piercings`) (`self.Max Number of Piercings`)))
        ;[1 1 1] Spell end of life
        (bind _asbp_spell_projectile (cast `/Game/Combat/Ranged/Projectiles/BPs/BP_Spell_Projectile` (`self.GetOwner`)))
        (`/Game/Combat/Ranged/Projectiles/BPs/BP_Spell_Projectile.Spell EOL` _asbp_spell_projectile)
        (else
          ;[1 1 1] Update the spell info based on the percentage decreases for each spell piercing
          (bind _spell_info_2 (message `/Game/Combat/Ranged/Projectiles/Interfaces/BPI_Spell.Get Spell Info` (`self.GetOwner`)))
          (bind _asbp_spell_projectile_2 (cast `/Game/Combat/Ranged/Projectiles/BPs/BP_Spell_Projectile` (`self.GetOwner`)))
          (bind (_spellname _generalinfo _uiinfo _spellcharacteristics _chargeinfo _instantinfo _burstinfo _piercinginfo _aoeinfo _splitinfo _hominginfo) (break `/Game/Combat/Ranged/Projectiles/Structs_Tables/Struct_Spell_Info` _spell_info_2))
          (bind (_spelldamage _spellspeed _timetomaxspeed _shouldslowdown _slowdownstarttime _timeforslowdown _spellscale _spellduration _spellcooldown _spellshape) (break `/Game/Combat/Ranged/Projectiles/Structs_Tables/Struct_Spell_General_Info` _generalinfo))
          (set `/Game/Combat/Ranged/Projectiles/BPs/BP_Spell_Projectile.Spell Info` (make `/Game/Combat/Ranged/Projectiles/Structs_Tables/Struct_Spell_Info` _spellname (make `/Game/Combat/Ranged/Projectiles/Structs_Tables/Struct_Spell_General_Info` (* _spelldamage (`self.Damage Percentage`)) (* _spellspeed (`self.Speed Percentage`)) _timetomaxspeed false 0.0 0.0 (* _spellscale (`self.Scale Percentage`)) _spellduration _spellcooldown _spellshape) (struct) _spellcharacteristics _chargeinfo _instantinfo _burstinfo _piercinginfo _aoeinfo _splitinfo _hominginfo) _asbp_spell_projectile_2))))))

(fn `Set Piercing Data`
  (params (`Has Max Number of Piercings?` :type Boolean) (`Max Number of Piercings` :type Integer) (`Damage Percentage Falloff` :type "Float (double-precision)") (`Speed Percentage Falloff` :type "Float (double-precision)") (`Scale Percentage Falloff` :type "Float (double-precision)"))
  ;[1 1 1] Set piercing variables based on passed parameters
  (set `self.Has Max Number of Piercings?` `Has Max Number of Piercings?`)
  (set `self.Max Number of Piercings` `Max Number of Piercings`)
  (set `self.Damage Percentage` `Damage Percentage Falloff`)
  (set `self.Speed Percentage` `Speed Percentage Falloff`)
  (set `self.Scale Percentage` `Scale Percentage Falloff`))