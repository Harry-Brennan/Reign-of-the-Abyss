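; Actor component that splits its owning spell projectile into several smaller projectiles, automatically after a delay for timed splitters.
; Split plays a distance-scaled camera shake, then spawns BP_Spell_Projectiles at stepped yaw angles, optionally reversed.
; Children get percentage-scaled damage, speed and scale, half duration, and no split characteristic, preventing recursive splitting.
; The original projectile then ends through SpellEOL.
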(event `self.ReceiveBeginPlay`
  (bind _spell_info (message `/Game/Combat/Ranged/Projectiles/Interfaces/BPI_Spell.Get Spell Info` (`self.GetOwner`)))
  (bind (_numofsplitspells _timedsplit_ _splittime) (break `/Game/Combat/Ranged/Projectiles/Structs_Tables/Characteristics/Struct_Spell_Split` (`.SplitInfo_46_0BCC21C94072526C07AD3A97FA92EB03` (break `/Game/Combat/Ranged/Projectiles/Structs_Tables/Struct_Spell_Info` _spell_info))))
  (if _timedsplit_
    (`KismetSystemLibrary.PrintString` (`KismetStringLibrary.Conv_DoubleToString` _splittime))
    (`KismetSystemLibrary.Delay` _splittime)
    (`/Engine/EditorBlueprintResources/StandardMacros.IsValid` (`self.GetOwner`)
      (:`Is Valid`
        (`self.Split`))
      (:`Is Not Valid`
        (`KismetSystemLibrary.PrintString` "OWNER IS NOT VALID")))
    (else
      (`KismetSystemLibrary.PrintString` "NOT A TIMED SPLITTER"))))

(fn `Split`
  (locals (Characteristics :type "Array of /Game/Combat/Ranged/Projectiles/Enums/Enum_Spell_Characteristics Enum") (`Current Split Angle` :type "Float (double-precision)"))
  (bind _yaw (.yaw (`Actor.K2_GetActorRotation` (`self.GetOwner`))))
  (bind _returnvalue (+ _yaw 180.0))
  (bind _returnvalue_2 (`GameplayStatics.GetActorOfClass` "/Game/Co-op/Camera/BP_Camera.BP_Camera_C"))
  (`LegacyCameraShake.StartLegacyCameraShake` (`GameplayStatics.GetPlayerCameraManager` 0) "/Game/Combat/Ranged/BPs/BP_Spell_Shoot_Camera_Shake.BP_Spell_Shoot_Camera_Shake_C" (`KismetMathLibrary.FClamp` (- 6.0 (/ (`KismetMathLibrary.Vector_Distance` (`Actor.K2_GetActorLocation` (`self.GetOwner`)) (`Actor.K2_GetActorLocation` _returnvalue_2)) 2000.0)) 0.5 8.0))
  (`KismetSystemLibrary.PrintString` "SPLIT")
  (set `self.Have Split` true)
  ;[1 1 1] Get spell info
  (bind _spell_info (message `/Game/Combat/Ranged/Projectiles/Interfaces/BPI_Spell.Get Spell Info` (`self.GetOwner`)))
  (bind (_spellname _generalinfo _spellvfx _uiinfo _spellcharacteristics _chargeinfo _instantinfo _burstinfo _piercinginfo _aoeinfo _splitinfo _hominginfo _attractinginfo) (break `/Game/Combat/Ranged/Projectiles/Structs_Tables/Struct_Spell_Info` _spell_info))
  ;[1 1 1] Remove the split characteristic from the spell's array of characteristics to be set as a local variable of characteristics to be passed into the split spells so that they in turn don't split further
  (bind _output_get (set `local.Characteristics` _spellcharacteristics))
  (`KismetArrayLibrary.Array_RemoveItem` _output_get "NewEnumerator5")
  (bind (_numofsplitspells _timedsplit_ _splittime _splitradius _splitinoppositedirectiontohit_ _splitpercentagedamage _splitpercentagespeed _splitpercentagescale) (break `/Game/Combat/Ranged/Projectiles/Structs_Tables/Characteristics/Struct_Spell_Split` _splitinfo))
  (bind _returnvalue_3 (- _numofsplitspells 1))
  (bind _returnvalue_4 (/ _splitradius _returnvalue_3))
  ;[1 1 1] Calculate angle to shoot the first split projectile at
  (set `local.Current Split Angle` (- 0.0 _returnvalue_4))
  (for _index (range (+ (`KismetMathLibrary.FTrunc` _returnvalue_3) 1))
    ;[1 1 1] If first in array don't calculate split angle again
    (if (not (== _index 0))
      ;[1 1 1] New split angle for next projectile
      (set `local.Current Split Angle` (+ (`local.Current Split Angle`) _returnvalue_4)))
    (bind _returnvalue_5 (+ (`KismetMathLibrary.SelectFloat` (`KismetMathLibrary.SelectFloat` (- _yaw 360.0) _returnvalue (> _returnvalue 180.0)) _yaw _splitinoppositedirectiontohit_) (`local.Current Split Angle`)))
    (bind (_spelldamage _spellspeed _timetomaxspeed _shouldslowdown _slowdownstarttime _timeforslowdown _spellscale _spellduration _spellcooldown _spellshape _spellaimassistsize _spellcastmethod _spellonhitstatuseffects) (break `/Game/Combat/Ranged/Projectiles/Structs_Tables/Struct_Spell_General_Info` _generalinfo))
    (bind _returnvalue_6 (* _spellscale (/ _splitpercentagescale 100.0)))
    (bind _returnvalue_7 (* _spellspeed (/ _splitpercentagespeed 100.0)))
    ;[1 1 1] Spawn split projectile at the original's location with the current split angle and the new split spell info and with the owner of the projectile as the owner of the original spell
    (`|SpawnActorFromClass` "/Game/Combat/Ranged/Projectiles/BPs/BP_Spell_Projectile.BP_Spell_Projectile_C" (`KismetMathLibrary.MakeTransform` (`Actor.K2_GetActorLocation` (`self.GetOwner`)) (`KismetMathLibrary.MakeRotator` (.roll (`Actor.K2_GetActorRotation` (`self.GetOwner`))) (.pitch (`Actor.K2_GetActorRotation` (`self.GetOwner`))) (`KismetMathLibrary.SelectFloat` (- _returnvalue_5 360.0) _returnvalue_5 (>= _returnvalue_5 180.0))) _returnvalue_6) "AdjustIfPossibleButAlwaysSpawn" "MultiplyWithRoot" (`Actor.GetOwner` (`self.GetOwner`)) (make `/Game/Combat/Ranged/Projectiles/Structs_Tables/Struct_Spell_Info` _spellname (make `/Game/Combat/Ranged/Projectiles/Structs_Tables/Struct_Spell_General_Info` (* _spelldamage (/ _splitpercentagedamage 100.0)) _returnvalue_7 _returnvalue_7 _shouldslowdown _slowdownstarttime _timeforslowdown _returnvalue_6 (/ _spellduration 2.0) _spellcooldown _spellshape _spellaimassistsize _spellcastmethod _spellonhitstatuseffects) _spellvfx _uiinfo (`local.Characteristics`) _chargeinfo _instantinfo _burstinfo _piercinginfo _aoeinfo _splitinfo _hominginfo _attractinginfo) null))
  ;[1 1 1] Spell eol of the original after spawning the required number of split projectiles
  (bind _asbp_spell_projectile (cast `/Game/Combat/Ranged/Projectiles/BPs/BP_Spell_Projectile` (`self.GetOwner`)))
  (`/Game/Combat/Ranged/Projectiles/BPs/BP_Spell_Projectile.Spell EOL` _asbp_spell_projectile))