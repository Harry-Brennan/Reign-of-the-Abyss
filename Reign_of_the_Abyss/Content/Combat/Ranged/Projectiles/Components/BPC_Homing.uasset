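; Projectile component that makes a spell home in on the nearest opposing character, using homing settings from the owning spell's info.
; A sphere trace filters hits by BPI_Enemy or BPI_Player, depending on the caster's side, and feeds the closest to ProjectileMovementComponent.
; With auto-switch on, Tick repeats the search at the switch interval and disables homing when the trace hits nothing; otherwise it searches once on BeginPlay.
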(event `self.ReceiveBeginPlay`
  (bind _returnvalue (`Actor.K2_GetActorLocation` (`self.GetOwner`)))
  (bind _returnvalue_2 (`Actor.K2_GetActorLocation` (`self.GetOwner`)))
  ;[1 1 1] Get the spell's info
  (bind _spell_info (message `/Game/Combat/Ranged/Projectiles/Interfaces/BPI_Spell.Get Spell Info` (`self.GetOwner`)))
  (bind ((`SpellVFX_59_CD8F7D074DE57DBC2EC3EB9DC297560D` _spellvfx) (`UIInfo_51_6745DFF74B6CD39E38C2B6B0065BC998` _uiinfo) (`AOEInfo_56_82970EA5401F2C2A7623458E4EEA83C0` _aoeinfo) (`HomingInfo_48_1BD3D87E46905119AA5AEDAA596C6811` _hominginfo)) (break `/Game/Combat/Ranged/Projectiles/Structs_Tables/Struct_Spell_Info` _spell_info))
  ;[1 1 1] Set homing info variables
  (set `self.Homing Strength` (break `/Game/Combat/Ranged/Projectiles/Structs_Tables/Characteristics/Struct_Spell_Homing` _hominginfo))
  (set `self.Homing Radius` (`.HomingProximityRadius_12_3B703D274D0F406F205C919B08CF2181` (break `/Game/Combat/Ranged/Projectiles/Structs_Tables/Characteristics/Struct_Spell_Homing` _hominginfo)))
  (set `self.Auto Switch Targets?` (`.AutomaticallySwitchTargets?_7_D7F1087A4E51E3EAA1DC25AC747953E1` (break `/Game/Combat/Ranged/Projectiles/Structs_Tables/Characteristics/Struct_Spell_Homing` _hominginfo)))
  (set `self.Time To Switch Targets` (`.TimeToSwitchTargets_10_172422DF49BB562A3C6279963210FFB9` (break `/Game/Combat/Ranged/Projectiles/Structs_Tables/Characteristics/Struct_Spell_Homing` _hominginfo)))
  ;[1 1 1] Set homing acceleration magnitude based on homing strength of the spell
  (set `ProjectileMovementComponent.HomingAccelerationMagnitude` (`self.Homing Strength`) (`Actor.GetComponentByClass` (`self.GetOwner`) "/Script/Engine.ProjectileMovementComponent"))
  (if (`self.Auto Switch Targets?`)
    ;[1 1 1] Set the tick interval based on the time to switch targets
    (`self.SetComponentTickInterval` (`self.Time To Switch Targets`))
    (else
      ;[1 1 1] Set tick disabled since the homing target won't be updated after this one trace
      (`self.SetComponentTickEnabled` false)
      ;[1 1 1] Sphere trace for pawns based on the homing radius of the spell
      (bind (_outhits _returnvalue_3) (`KismetSystemLibrary.SphereTraceMultiForObjects` _returnvalue_2 _returnvalue_2 (`self.Homing Radius`) (`|MakeArray` "ObjectTypeQuery7" "ObjectTypeQuery8" :!type "EObjectTypeQuery Enum")))
      ;[1 1 1] Loop through hit actors and find the closest pawn to then set as the homing target
      (if _returnvalue_3
        (for (_array_element _array_index) _outhits
          (bind (_bblockinghit _binitialoverlap _time _distance _location _impactpoint _normal _impactnormal _physmat _hitactor) (`GameplayStatics.BreakHitResult` _array_element))
          (if (`KismetSystemLibrary.DoesImplementInterface` _hitactor (select `bool` (`KismetSystemLibrary.DoesImplementInterface` (`Actor.GetOwner` (`self.GetOwner`)) "/Game/Player/Interfaces/BPI_Player.BPI_Player_C") :`false` "/Game/Player/Interfaces/BPI_Player.BPI_Player_C" :`true` "/Game/Enemies/Interfaces/BPI_Enemy.BPI_Enemy_C" :!type "Interface Class Reference"))
            (if (== _array_index 0)
              (set `self.Current Homing Target` _hitactor)
              (elif (< (`KismetMathLibrary.Vector_Distance` _returnvalue (`Actor.K2_GetActorLocation` _hitactor)) (`KismetMathLibrary.Vector_Distance` _returnvalue (`Actor.K2_GetActorLocation` (`self.Current Homing Target`))))
                (set `self.Current Homing Target` _hitactor)))))
        (`self.Activate Homing`)
        (`self.Update Homing Target` (`self.Current Homing Target`))))))

(event `self.ReceiveTick`
  (params (DeltaSeconds :type "Float (single-precision)"))
  (bind _returnvalue (`Actor.K2_GetActorLocation` (`self.GetOwner`)))
  (bind _returnvalue_2 (`Actor.K2_GetActorLocation` (`self.GetOwner`)))
  ;[1 1 1] sphere trace for pawns with radius of homing radius to find a homing target
  (bind (_outhits _returnvalue_3) (`KismetSystemLibrary.SphereTraceMultiForObjects` _returnvalue _returnvalue (`self.Homing Radius`) (`|MakeArray` "ObjectTypeQuery8" "ObjectTypeQuery7" :!type "EObjectTypeQuery Enum")))
  ;[1 1 1] Loop through hit actors to find clolsest actor and then set as the homing target of the spell
  (if _returnvalue_3
    (for (_array_element _array_index) _outhits
      (bind (_bblockinghit _binitialoverlap _time _distance _location _impactpoint _normal _impactnormal _physmat _hitactor) (`GameplayStatics.BreakHitResult` _array_element))
      (if (`KismetSystemLibrary.DoesImplementInterface` _hitactor (select `bool` (`KismetSystemLibrary.DoesImplementInterface` (`Actor.GetOwner` (`self.GetOwner`)) "/Game/Player/Interfaces/BPI_Player.BPI_Player_C") :`false` "/Game/Player/Interfaces/BPI_Player.BPI_Player_C" :`true` "/Game/Enemies/Interfaces/BPI_Enemy.BPI_Enemy_C" :!type "Interface Class Reference"))
        (if (== _array_index 0)
          (set `self.Current Homing Target` _hitactor)
          (elif (< (`KismetMathLibrary.Vector_Distance` _returnvalue_2 (`Actor.K2_GetActorLocation` _hitactor)) (`KismetMathLibrary.Vector_Distance` _returnvalue_2 (`Actor.K2_GetActorLocation` (`self.Current Homing Target`))))
            (set `self.Current Homing Target` _hitactor)))))
    (`self.Activate Homing`)
    (`self.Update Homing Target` (`self.Current Homing Target`))
    (else
      ;[1 1 1] If didn't hit anything deactivate homing
      (`self.Deactivate Homing`))))

(fn `Activate Homing`
  (set `ProjectileMovementComponent.bIsHomingProjectile` true (`Actor.GetComponentByClass` (`self.GetOwner`) "/Script/Engine.ProjectileMovementComponent")))

(fn `Deactivate Homing`
  (set `ProjectileMovementComponent.bIsHomingProjectile` false (`Actor.GetComponentByClass` (`self.GetOwner`) "/Script/Engine.ProjectileMovementComponent")))

(fn `Update Homing Target`
  (params (`New Homing Target` :type "Actor Object Reference"))
  ;[1 1 1] Update homing target component of the spell's projectile movement component as long as the new homing target is valid
  (`/Engine/EditorBlueprintResources/StandardMacros.IsValid` `New Homing Target`
    (:`Is Valid`
      (set `ProjectileMovementComponent.HomingTargetComponent` (`Actor.RootComponent` `New Homing Target`) (`Actor.GetComponentByClass` (`self.GetOwner`) "/Script/Engine.ProjectileMovementComponent")))))