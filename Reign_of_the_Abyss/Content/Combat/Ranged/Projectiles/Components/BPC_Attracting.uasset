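; Spell projectile component that pulls nearby characters and physics objects toward its owner, configured by the spell's AttractingInfo.
; BeginPlay handles optional delayed start, tick rate and optional duration.
; Tick sphere-traces for targets, applies status effects to players and enemies, and runs a looping force timer while targets exist.
; The timer applies impulses to characters and forces to static meshes, scaled by clamped horizontal distance, so farther targets pull harder.
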(event `self.ReceiveBeginPlay`
  ;[1 1 1] Get spell info on begin play and check if the attracting should be delayed rather than starting when the projectile is spawned and if so then do a delay before setting the tick enabled then setting the tick interval to be the attracting updating rate and then check if it is a timed attracting and if so do a delay of duration attracting before setting the component tick disabled
  (bind _spell_info (message `/Game/Combat/Ranged/Projectiles/Interfaces/BPI_Spell.Get Spell Info` (`self.GetOwner`)))
  (bind ((`SpellVFX_59_CD8F7D074DE57DBC2EC3EB9DC297560D` _spellvfx) (`AttractingInfo_54_89145D5F4104ACA31D0046B445A80C29` _attractinginfo)) (break `/Game/Combat/Ranged/Projectiles/Structs_Tables/Struct_Spell_Info` _spell_info))
  (if (`.DelayedAttracting?_14_4235F33046BE0756B5BB4BB3DBB5558B` (break `/Game/Combat/Ranged/Projectiles/Structs_Tables/Characteristics/Struct_Spell_Attracting` _attractinginfo))
    (`KismetSystemLibrary.Delay` (`.AttractingStartTime_16_4B3644E9451BAB98D4C823BD39547F14` (break `/Game/Combat/Ranged/Projectiles/Structs_Tables/Characteristics/Struct_Spell_Attracting` _attractinginfo)))
    (`self.SetComponentTickEnabled` true)
    (else
      (`self.SetComponentTickEnabled` true)))
  (`self.SetComponentTickInterval` (`.AttractingUpdatingRate_18_0428CA434CCA5D233F55E89C76EC5C17` (break `/Game/Combat/Ranged/Projectiles/Structs_Tables/Characteristics/Struct_Spell_Attracting` _attractinginfo)))
  (if (`.TimedAttracting?_10_72940C3D47AC3A3C7AD6289159B4FD77` (break `/Game/Combat/Ranged/Projectiles/Structs_Tables/Characteristics/Struct_Spell_Attracting` _attractinginfo))
    (`KismetSystemLibrary.Delay` (`.AttractingDuration_12_10A566424BB81F854BB641BF856D74B9` (break `/Game/Combat/Ranged/Projectiles/Structs_Tables/Characteristics/Struct_Spell_Attracting` _attractinginfo)))
    (`self.SetComponentTickEnabled` false)))

(event `self.ReceiveTick`
  (params (DeltaSeconds :type "Float (single-precision)"))
  (bind _returnvalue (`Actor.K2_GetActorLocation` (`self.GetOwner`)))
  ;[1 1 1] Check for suitable targets for attracting and if there are some then start the function for actually doing the attracting, if there are no targets then the attracting function timer is cleared and invalidated, then loop through the targtets and add them to the affected actors array if they are not alreay contained wtihin them
  (`KismetArrayLibrary.Array_Clear` (`self.Current Affected Actors`))
  (bind ((`SpellVFX_59_CD8F7D074DE57DBC2EC3EB9DC297560D` _spellvfx) (`AttractingInfo_54_89145D5F4104ACA31D0046B445A80C29` _attractinginfo)) (break `/Game/Combat/Ranged/Projectiles/Structs_Tables/Struct_Spell_Info` (stale `self.ReceiveBeginPlay` _spell_info)))
  (bind (_outhits _returnvalue_2) (`KismetSystemLibrary.SphereTraceMultiForObjects` :`Start` _returnvalue :`End` _returnvalue :`Radius` (break `/Game/Combat/Ranged/Projectiles/Structs_Tables/Characteristics/Struct_Spell_Attracting` _attractinginfo) :`ObjectTypes` (`|MakeArray` "ObjectTypeQuery4" "ObjectTypeQuery7" "ObjectTypeQuery8" :!type "EObjectTypeQuery Enum") :`DrawDebugType` "ForDuration"))
  (if _returnvalue_2
    (if (not (`KismetSystemLibrary.K2_IsValidTimerHandle` (`self.Force Event Timer`)))
      (bind _returnvalue_3 (`KismetSystemLibrary.K2_SetTimerDelegate` (delegate `Add Force Event`) 0.1 true))
      (set `self.Force Event Timer` _returnvalue_3))
    (for _array_element _outhits
      (bind (_bblockinghit _binitialoverlap _time _distance _location _impactpoint _normal _impactnormal _physmat _hitactor _hitcomponent) (`GameplayStatics.BreakHitResult` _array_element))
      (if (not (`KismetArrayLibrary.Array_Contains` (`self.Current Affected Actors`) _hitactor))
        (`KismetArrayLibrary.Array_Add` (`self.Current Affected Actors`) _hitactor)
        ;[1 1 1] Applying on attracting status effects to players and enemies
        (switch `ECollisionChannel` (`PrimitiveComponent.GetCollisionObjectType` _hitcomponent)
          (:`ECC_GameTraceChannel1`
            _)
          (:`ECC_GameTraceChannel2`
            _))
        (for _array_element_2 (`.PossibleStatus_23_30BE313C410E5C82B6F330A9E0495AFC` (break `/Game/Combat/Status_Effects/Structs_Tables/Struct_Status_Effects` (`.AttractingStatusEffect_21_E46A7D0C4FC7F95EE3CAA3B4BBEFBC48` (break `/Game/Combat/Ranged/Projectiles/Structs_Tables/Characteristics/Struct_Spell_Attracting` _attractinginfo))))
          (`/Game/Combat/Status_Effects/Components/BPC_StatusEffectHandler.Add Status` (`Actor.GetComponentByClass` _hitactor "/Game/Combat/Status_Effects/Components/BPC_StatusEffectHandler.BPC_StatusEffectHandler_C") _array_element_2 (`.AttractingStatusEffect_21_E46A7D0C4FC7F95EE3CAA3B4BBEFBC48` (break `/Game/Combat/Ranged/Projectiles/Structs_Tables/Characteristics/Struct_Spell_Attracting` _attractinginfo)) (`Actor.GetOwner` (`self.GetOwner`))))))
    (set `self.All Affected Actors` (`self.Current Affected Actors`))
    (else
      (`KismetSystemLibrary.K2_ClearAndInvalidateTimerHandle` (`self.Force Event Timer`))
      (`KismetArrayLibrary.Array_Clear` (`self.All Affected Actors`)))))

(event `Add Force Event`
  (bind (_returnvalue_x _returnvalue_y) (`KismetMathLibrary.BreakVector` (`Actor.K2_GetActorLocation` (`self.GetOwner`))))
  ;[1 1 1] Loop through the affected actors and add impulse to themn in the direction of the epicentre of the attracting  / spell or add a force to physics bodies if the affected actor is a physics body and not a character
  (for _array_element (`self.All Affected Actors`)
    (bind _returnvalue (`Actor.GetComponentByClass` _array_element "/Script/Engine.CharacterMovementComponent"))
    (`/Engine/EditorBlueprintResources/StandardMacros.IsValid` _returnvalue
      (:`Is Valid`
        (bind ((`SpellVFX_59_CD8F7D074DE57DBC2EC3EB9DC297560D` _spellvfx) (`AttractingInfo_54_89145D5F4104ACA31D0046B445A80C29` _attractinginfo)) (break `/Game/Combat/Ranged/Projectiles/Structs_Tables/Struct_Spell_Info` (stale `self.ReceiveBeginPlay` _spell_info)))
        (bind _z (.z (`Actor.K2_GetActorLocation` _array_element)))
        (bind _returnvalue_2 (* (* (`KismetMathLibrary.GetForwardVector` (`KismetMathLibrary.FindLookAtRotation` (`Actor.K2_GetActorLocation` _array_element) (`Actor.K2_GetActorLocation` (`self.GetOwner`)))) (`.AttractingStrength_9_58DF022F4F1D7C12A4FFB78D268F7D43` (break `/Game/Combat/Ranged/Projectiles/Structs_Tables/Characteristics/Struct_Spell_Attracting` _attractinginfo))) (`KismetMathLibrary.FClamp` (/ (- (`KismetMathLibrary.VSize` (- (`KismetMathLibrary.MakeVector` _returnvalue_x _returnvalue_y _z) (`KismetMathLibrary.MakeVector` (.x (`Actor.K2_GetActorLocation` _array_element)) (.y (`Actor.K2_GetActorLocation` _array_element)) _z))) 10.0) (break `/Game/Combat/Ranged/Projectiles/Structs_Tables/Characteristics/Struct_Spell_Attracting` _attractinginfo)) 0.5)))
        (`CharacterMovementComponent.AddImpulse` _returnvalue _returnvalue_2 true))
      (:`Is Not Valid`
        (`PrimitiveComponent.AddForce` (`Actor.GetComponentByClass` _array_element "/Script/Engine.StaticMeshComponent") (* _returnvalue_2 100.0) "None" false)))))