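; Melee weapon component that tracks light attack state through Attacking and Animating flags and an AttackIndex.
; LightAttack is ignored while Attacking and otherwise sets both flags, without playing any animation itself.
; Its index increment and wrap at two sit behind a constant-true branch, so they never run.
; Two reset events print debug messages and clear the flags, with the animation reset also zeroing the index.
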(event `LightAttack`
  (if (`self.Attacking`)
    _
    (elif (`self.Animating?`)
      (if true
        (set `self.Attacking` true)
        (set `self.Animating?` true)
        (else
          (bind _result (`/Engine/EditorBlueprintResources/StandardMacros.IncrementInt` (`self.AttackIndex`))
            (:`  `
              (if (== _result 2)
                (set `self.AttackIndex` 0)
                (set `self.Attacking` true)
                (set `self.Animating?` true)
                (else
                  (set `self.Attacking` true)
                  (set `self.Animating?` true)))))))
      (else
        (set `self.Attacking` true)
        (set `self.Animating?` true)))))

(event `SetAttackingFalse`
  (`KismetSystemLibrary.PrintString` "set attacking false")
  (set `self.Attacking` false))

(event `SetAnimationFalse`
  (`KismetSystemLibrary.PrintString` "set animating false")
  (set `self.Animating?` false)
  (set `self.AttackIndex` 0))