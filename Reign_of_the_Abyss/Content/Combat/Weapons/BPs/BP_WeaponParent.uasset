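; Base melee weapon actor that loads mesh and stats from DT_Melee_Weapon_Info, reducing damage for enemy owners.
; While active, a looping timer box-traces between mesh sockets, hitting each actor once per activation.
; Hits apply damage and hit stop to characters and payloads, plus knockback and status effects to characters, which also heal player owners.
; It also toggles spell Niagara VFX and A Thousand Cuts, a repeating radial damage pulse around the owner.
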(event `/Game/Combat/Weapons/Interfaces/BPI_Melee.Update Hitbox Multiplier`
  (params (`New Multiplier` :type "Float (double-precision)"))
  (set `self.Hitbox Multiplier` `New Multiplier`))

(event `/Game/Combat/Weapons/Interfaces/BPI_Melee.StopNiagara`
  (`ActorComponent.Deactivate` (`self.MeleeSpellVfx`)))

(event `/Game/Combat/Weapons/Interfaces/BPI_Melee.StartNiagara`
  (bind _spell (message `/Game/Combat/Ranged/Interfaces/BPI_Has_Ranged_Attack.Get Current Spell` (`self.GetOwner`)))
  (`NiagaraComponent.SetAsset` (`self.MeleeSpellVfx`) (`.ShootVFX_5_B64024FF4362A1A66CAB479F4C1C380B` (break `/Game/Combat/Ranged/Projectiles/Structs_Tables/Struct_Spell_VFX` (`.SpellVFX_59_CD8F7D074DE57DBC2EC3EB9DC297560D` (break `/Game/Combat/Ranged/Projectiles/Structs_Tables/Struct_Spell_Info` _spell)))) true)
  (`ActorComponent.Activate` (`self.MeleeSpellVfx`) true))

(event `self.ReceiveBeginPlay`
  (`self.Set Weapon Info` (`self.WeaponName`)))

(event `Activate ATC`
  (params (Active :type Boolean))
  (if Active
    (bind _returnvalue (`KismetSystemLibrary.K2_SetTimerDelegate` (delegate `A Thousand Cuts`) 0.2 true))
    (else
      (`KismetSystemLibrary.K2_ClearAndInvalidateTimerHandle` _returnvalue))))

(event `/Game/Combat/Weapons/Interfaces/BPI_Weapon.Set Weapon Info`
  (params (`Weapon Name` :type "/Game/Combat/Weapons/Enums/Enum_Weapon_Names Enum" :default "NewEnumerator2"))
  (bind _returnvalue (`|GetDataTableRow` "/Game/Combat/Weapons/Melee/Struct_Tables/DT_Melee_Weapon_Info.DT_Melee_Weapon_Info" (`KismetStringLibrary.Conv_StringToName` (`|GetEnumeratorNameAsString` `Weapon Name`)))
    (:`then`
      (bind (_weaponname _staticmesh _damage _horizontalknockback _verticalknockback _statuseffects _hitboxmultiplier) (break `/Game/Combat/Weapons/Melee/Struct_Tables/Struct_Melee_Weapon_Info` _returnvalue))
      (set `self.General Info` (select `bool` (`KismetSystemLibrary.DoesImplementInterface` (`self.GetOwner`) "/Game/Enemies/Interfaces/BPI_Enemy.BPI_Enemy_C") :`false` _returnvalue :`true` (make `/Game/Combat/Weapons/Melee/Struct_Tables/Struct_Melee_Weapon_Info` _weaponname _staticmesh (* _damage 0.8) _horizontalknockback _verticalknockback _statuseffects _hitboxmultiplier)))
      (bind ((`StaticMesh_8_ADF467134E9E9C50BAB129A7371EFB1C` _staticmesh_2) (`HitboxMultiplier_26_AB732F544849C919FD9C1A8392F9AF29` _hitboxmultiplier_2)) (break `/Game/Combat/Weapons/Melee/Struct_Tables/Struct_Melee_Weapon_Info` _returnvalue))
      (`StaticMeshComponent.SetStaticMesh` (`self.WeaponMesh`) _staticmesh_2)
      (set `self.WeaponName` `Weapon Name`)
      (set `self.Hitbox Multiplier` _hitboxmultiplier_2))))

(event `/Game/Combat/Weapons/Interfaces/BPI_Melee.SetHitBox`
  (params (`Active?` :type Boolean))
  ;[1 1 1] Enables and disables hit boxes
  (if `Active?`
    (bind _returnvalue (`KismetSystemLibrary.K2_SetTimerDelegate` (delegate `HitBox`) 0.05 true))
    (else
      (`KismetSystemLibrary.K2_ClearAndInvalidateTimerHandle` _returnvalue)
      (`KismetArrayLibrary.Array_Clear` (`self.HitActors`)))))

(event `A Thousand Cuts`
  (bind _returnvalue (`self.K2_GetActorLocation` (`self.GetOwner`)))
  (bind _outhits (`KismetSystemLibrary.SphereTraceMultiForObjects` _returnvalue _returnvalue 1000.0 (`|MakeArray` "ObjectTypeQuery7" "ObjectTypeQuery8" "ObjectTypeQuery9" :!type "EObjectTypeQuery Enum") false (`|MakeArray` (`self.GetOwner`))))
  (for _array_element _outhits
    (bind (_bblockinghit _binitialoverlap _time _distance _location _impactpoint _normal _impactnormal _physmat _hitactor _hitcomponent) (`GameplayStatics.BreakHitResult` _array_element))
    (`KismetSystemLibrary.PrintString` (`KismetSystemLibrary.GetDisplayName` _hitactor))
    (switch `ECollisionChannel` (`PrimitiveComponent.GetCollisionObjectType` _hitcomponent)
      (:`ECC_Pawn`
        _)
      (:`ECC_GameTraceChannel1`
        _)
      (:`ECC_GameTraceChannel2`
        _)
      (:`ECC_GameTraceChannel3`
        _))
    (if (`KismetSystemLibrary.DoesImplementInterface` _hitactor "/Game/Health/Interfaces/BPI_Has_Health.BPI_Has_Health_C")
      (`/Game/Health/Components/BPC_Health_V2.Take Damage` (`self.GetComponentByClass` _hitactor "/Game/Health/Components/BPC_Health_V2.BPC_Health_V2_C") 5.0 (`self.GetOwner`) _normal _location 0.0 0.0 0.01))))

(event `HitBox`
  (bind _returnvalue (`self.GetOwner`))
  (bind _weaponmesh (`self.WeaponMesh`))
  (bind (_weaponname _staticmesh _damage _horizontalknockback _verticalknockback) (break `/Game/Combat/Weapons/Melee/Struct_Tables/Struct_Melee_Weapon_Info` (`self.General Info`)))
  (bind ((`StatusEffects_23_5383A7074E2E49CCE1F8BA9BFA4A696B` _statuseffects)) (break `/Game/Combat/Weapons/Melee/Struct_Tables/Struct_Melee_Weapon_Info` (`self.General Info`)))
  (bind _returnvalue_2 (`self.GetComponentByClass` _returnvalue "/Game/Health/Components/BPC_Health_V2.BPC_Health_V2_C"))
  (bind _returnvalue_3 (`self.GetComponentByClass` (`self.GetOwner`) "/Game/Combat/Components/BPC_HitStop.BPC_HitStop_C"))
  ;[1 0 0] Handles the hitbox of the weapon by getting its bounds with the sockets that are on the mesh.
  (bind _outhits (`KismetSystemLibrary.BoxTraceMultiForObjects` (`SceneComponent.GetSocketLocation` _weaponmesh "Bottom Extent") (`SceneComponent.GetSocketLocation` _weaponmesh "Top Extent") (* (`KismetMathLibrary.Conv_DoubleToVector` (`KismetMathLibrary.Vector_Distance` (`SceneComponent.GetSocketLocation` _weaponmesh "Left Extent") (`SceneComponent.GetSocketLocation` _weaponmesh "Right Extent"))) (`self.Hitbox Multiplier`)) (`SceneComponent.K2_GetComponentRotation` _weaponmesh) (`|MakeArray` "ObjectTypeQuery3" "ObjectTypeQuery4" "ObjectTypeQuery7" "ObjectTypeQuery8" "ObjectTypeQuery9" :!type "EObjectTypeQuery Enum") false (`|MakeArray` (`self.GetOwner`))))
  (for _array_element _outhits
    (bind (_bblockinghit _binitialoverlap _time _distance _location _impactpoint _normal _impactnormal _physmat _hitactor _hitcomponent) (`GameplayStatics.BreakHitResult` _array_element))
    (switch `ECollisionChannel` (`PrimitiveComponent.GetCollisionObjectType` _hitcomponent)
      (:`ECC_Pawn`
        _)
      (:`ECC_GameTraceChannel1`
        _)
      (:`ECC_GameTraceChannel2`
        _)
      (:`ECC_GameTraceChannel3`
        _))
    (if (`KismetSystemLibrary.DoesImplementInterface` _hitactor "/Game/Health/Interfaces/BPI_Has_Health.BPI_Has_Health_C")
      (if (not (`KismetArrayLibrary.Array_Contains` (`self.HitActors`) _hitactor))
        (`/Game/Health/Components/BPC_Health_V2.Take Damage` (`self.GetComponentByClass` _hitactor "/Game/Health/Components/BPC_Health_V2.BPC_Health_V2_C") _damage (`self.GetOwner`) _normal _location _horizontalknockback _verticalknockback 0.0)
        (`KismetArrayLibrary.Array_Add` (`self.HitActors`) _hitactor)
        (bind _returnvalue_4 (`self.GetComponentByClass` _hitactor "/Game/Combat/Components/BPC_HitStop.BPC_HitStop_C"))
        (`/Game/Combat/Components/BPC_HitStop.INITIAITE HIT STOP!` _returnvalue_4 _damage)
        (`/Game/Combat/Components/BPC_HitStop.INITIAITE HIT STOP!` _returnvalue_3 _damage)
        (for _array_element_2 (`.PossibleStatus_23_30BE313C410E5C82B6F330A9E0495AFC` (break `/Game/Combat/Status_Effects/Structs_Tables/Struct_Status_Effects` _statuseffects))
          (`/Game/Combat/Status_Effects/Components/BPC_StatusEffectHandler.Add Status` (`self.GetComponentByClass` _hitactor "/Game/Combat/Status_Effects/Components/BPC_StatusEffectHandler.BPC_StatusEffectHandler_C") _array_element_2 _statuseffects (`self.GetOwner`)))
        ;[1 1 1] HEAL PLAYER THAT HIT THE OTHER CHARACTER BASED ON DAMAGE DEALT
        (if (or (`/Game/Health/Components/BPC_Health_V2.Downed` _returnvalue_2) (`/Game/Health/Components/BPC_Health_V2.DownedTransition` _returnvalue_2))
          _
          (elif (`KismetSystemLibrary.DoesImplementInterface` _returnvalue "/Game/Player/Interfaces/BPI_Player.BPI_Player_C")
            (`/Game/Health/Components/BPC_Health_V2.Heal` _returnvalue_2 (/ _damage 5.0)))))
      (elif (`KismetSystemLibrary.DoesImplementInterface` _hitactor "/Game/Co-op/Interfaces/BPI_Payload.BPI_Payload_C")
        (if (not (`KismetArrayLibrary.Array_Contains` (`self.HitActors`) _hitactor))
          (`/Game/Health/Components/BPC_PayloadHealth.TakeDamage` (`self.GetComponentByClass` _hitactor "/Game/Health/Components/BPC_PayloadHealth.BPC_PayloadHealth_C") _damage (`self.GetOwner`))
          (`KismetArrayLibrary.Array_Add` (`self.HitActors`) _hitactor)
          (`/Game/Combat/Components/BPC_HitStop.INITIAITE HIT STOP!` _returnvalue_4 _damage)
          (`/Game/Combat/Components/BPC_HitStop.INITIAITE HIT STOP!` _returnvalue_3 _damage))))))

(fn `Get Weapon Info`
  (returns (`Weapon Info` :type "/Game/Combat/Weapons/Melee/Struct_Tables/Struct_Melee_Weapon_Info Structure"))
  (return (`self.General Info`)))

(fn `Get Weapon Name`
  (returns (`Weapon Name` :type "/Game/Combat/Weapons/Enums/Enum_Weapon_Names Enum"))
  (return (`self.WeaponName`)))

(fn `UserConstructionScript`)