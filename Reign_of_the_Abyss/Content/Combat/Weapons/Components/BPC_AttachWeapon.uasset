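; Actor component that spawns and attaches a character's ranged and melee weapons and moves them between hand and holster sockets.
; On BeginPlay it reads weapon names from the owner via interface messages, spawns collision-disabled BP_WeaponParent actors, reports them back and equips the primary.
; SwitchWeapon re-attaches the pair to swap the main-hand weapon, using flags to track holster state.
; A separate function holsters both weapons while casting.
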(event `Set Weapons`
  (bind _returnvalue (`self.GetOwner`))
  (bind _character_info (message `/Game/General_Character_Things/Interfaces/BPI_Character.Get Character Info` (`self.GetOwner`) :!label _label))
  (bind ((`MeleeWeaponInfo_39_C677D2A64046D59F138511BD8C2C3485` _meleeweaponinfo) (`RangedWeaponName_38_099615D5498943DC4E4D36A1DCB8226D` _rangedweaponname) (`MeleePrimaryWeapon?_41_6718B5A842DB0EDA5042C1906181B61A` _meleeprimaryweapon_)) (break `/Game/General_Character_Things/Structs_Tables/Struct_Character_Info` _character_info))
  (set `self.Melee Weapon Name` _meleeweaponinfo)
  (set `self.Ranged Weapon Name` _rangedweaponname)
  (`|ExecutionSequence`
    (:`then_0`
      (bind _returnvalue_2 (`|SpawnActorFromClass` "/Game/Combat/Weapons/BPs/BP_WeaponParent.BP_WeaponParent_C" (`KismetMathLibrary.MakeTransform` (0.0 0.0 0.0)) "Undefined" "MultiplyWithRoot" (`self.GetOwner`) (`self.Ranged Weapon Name`) null))
      (bind _mesh (message `/Game/Combat/Interfaces/BPI_Has_Weapon.Get_Character_Mesh` _returnvalue))
      (`Actor.K2_AttachToComponent` _returnvalue_2 _mesh "r_weapon_socket" "SnapToTarget" "SnapToTarget" "KeepWorld" true)
      (message `/Game/Combat/Interfaces/BPI_Has_Weapon.Set_Equipped_Ranged_Weapon` _returnvalue _returnvalue_2)
      (`Actor.SetActorEnableCollision` _returnvalue_2 false)
      (set `self.Ranged Weapon` _returnvalue_2)
      (set `self.Mesh` _mesh))
    (:`then_1`
      (bind _returnvalue_3 (`|SpawnActorFromClass` "/Game/Combat/Weapons/BPs/BP_WeaponParent.BP_WeaponParent_C" (`KismetMathLibrary.MakeTransform` (0.0 0.0 0.0)) "Undefined" "MultiplyWithRoot" (`self.GetOwner`) (`self.Melee Weapon Name`) null))
      (`Actor.K2_AttachToComponent` _returnvalue_3 (`self.Mesh`) "l_weapon_socket" "SnapToTarget" "SnapToTarget" "KeepWorld" true)
      (message `/Game/Combat/Interfaces/BPI_Has_Weapon.Set_Equipped_Melee_Weapon` (`self.GetOwner`) _returnvalue_3)
      (`Actor.SetActorEnableCollision` _returnvalue_3 false)
      (set `self.Melee Weapon` _returnvalue_3))
    (:`then_2`
      (set `self.Melee Holstered?` _meleeprimaryweapon_)
      (`self.Switch Weapon` _meleeprimaryweapon_))))

(event `self.ReceiveBeginPlay`
  (goto _label))

(fn `Holster Ranged Weapon Whilst Casting`
  (bind _ranged_weapon (`self.Ranged Weapon`))
  (`/Engine/EditorBlueprintResources/StandardMacros.IsValid` _ranged_weapon
    (:`Is Valid`
      (`Actor.K2_AttachToComponent` _ranged_weapon (`self.Mesh`) "Holstered_Weapon_Socket_2" "SnapToTarget" "SnapToTarget" "KeepWorld" true)
      (set `self.Ranged Holstered For Casting` true)
      (`Actor.K2_AttachToComponent` (`self.Melee Weapon`) (`self.Mesh`) "Holstered_Weapon_Socket" "SnapToTarget" "SnapToTarget" "KeepWorld" true)
      (set `self.Melee Holstered?` true))))

(fn `Switch Weapon`
  (params (`Melee to Main` :type Boolean))
  (if `Melee to Main`
    (if (`self.Melee Holstered?`)
      (`Actor.K2_AttachToComponent` (`self.Ranged Weapon`) (`self.Mesh`) "Holstered_Weapon_Socket" "SnapToTarget" "SnapToTarget" "KeepWorld" true)
      (`Actor.K2_AttachToComponent` (`self.Melee Weapon`) (`self.Mesh`) "r_weapon_socket" "SnapToTarget" "SnapToTarget" "KeepWorld" true)
      (set `self.Melee Holstered?` false)
      (set `self.Ranged Holstered For Casting` false))
    (elif (`self.Melee Holstered?`)
      (if (`self.Ranged Holstered For Casting`)
        (`Actor.K2_AttachToComponent` (`self.Melee Weapon`) (`self.Mesh`) "Holstered_Weapon_Socket" "SnapToTarget" "SnapToTarget" "KeepWorld" true :!label _label)
        (`Actor.K2_AttachToComponent` (`self.Ranged Weapon`) (`self.Mesh`) "r_weapon_socket" "SnapToTarget" "SnapToTarget" "KeepWorld" true)
        (set `self.Melee Holstered?` true)
        (set `self.Ranged Holstered For Casting` false))
      (else
        (goto _label)))))