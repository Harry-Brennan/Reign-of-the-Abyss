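; Status effect component that applies chance-based Bleed, Burn and Charmed/Turned to its owner, showing them on the player HUD.
; AddStatus tags the owner and starts looping timers; a shared retriggerable delay handles clearing.
; Bleed and Burn deal periodic damage, with Burn spreading through sphere traces to nearby handlers.
; Charm/Turn, limited to opposing-faction sources, overrides control: charmed owners approach the charmer, turned ones attack nearby allies or wander.
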(event `ClearStatusWithTimer`
  (params (Time :type "Float (double-precision)") (Tag :type "GameplayTag Structure"))
  (`KismetSystemLibrary.RetriggerableDelay` Time)
  (`|SwitchGameplayTag` Tag
    (:`Bleed`
      (`KismetSystemLibrary.K2_ClearAndInvalidateTimerHandle` (`self.BleedTimerHandle`)))
    (:`Burn`
      (`KismetSystemLibrary.K2_ClearAndInvalidateTimerHandle` (`self.BurnTimerHandle`)))
    (:`Charmed / Turned`
      (bind _ascharacter (cast `Character` (`self.GetOwner`)))
      (bind _returnvalue (`Pawn.GetController` _ascharacter))
      ;[1 1 1] Activating enemy if the owner of this component is an enemy
      (bind _asac_enemy (cast `/Game/Enemies/AI/Controllers/AC_Enemy` _returnvalue)
        (:`then`
          (`/Game/Enemies/AI/Controllers/AC_Enemy.Activate Enemy` _asac_enemy))
        (:`CastFailed`
          _))
      ;[1 1 1] Allowing move input again
      (`Controller.ResetIgnoreMoveInput` _returnvalue)
      ;[1 1 1] Stopping the charmed / turned timer
      (`KismetSystemLibrary.K2_ClearAndInvalidateTimerHandle` (`self.Charmed / Turned Timer`))
      ;[1 1 1] Stopping the charmed / turned movement functions
      (`self.Stop Charmed / Turned Movement`)
      ;[1 1 1] Resetting the speed back to normal again
      (`/Game/Movement/Basic_Movement/BPC_Movement_Manager.Set Speed Multiplier` (`Actor.GetComponentByClass` (`self.GetOwner`) "/Game/Movement/Basic_Movement/BPC_Movement_Manager.BPC_Movement_Manager_C") (* (`.PercentageMoveSpeedSlow_19_BA2382774A23599A9192E59BD9F26660` (break `/Game/Combat/Status_Effects/Structs_Tables/Struct_Charmed_Turned` (`.CharmedTurned_24_EF1FB2024F9506FF1C949EB01835F961` (break `/Game/Combat/Status_Effects/Structs_Tables/Struct_Status_Effects` (`self.Status Struct Variable`))))) -1.0))
      ;[1 1 1] Resetting the speed bool variable indicator back to false
      (set `self.Set Speed Charmed / Turned` false)))
  (`BlueprintGameplayTagLibrary.RemoveGameplayTag` (`self.StatusEffects`) Tag))

(event `Charmed / Turned Actual Movement`
  (bind (_returnvalue_roll _returnvalue_pitch _returnvalue_yaw) (`KismetMathLibrary.BreakRotator` (`KismetMathLibrary.FindLookAtRotation` (`Actor.K2_GetActorLocation` (`self.GetOwner`)) (`self.Move To Loc`))))
  (if (not (< (`KismetMathLibrary.Vector_Distance` (`Actor.K2_GetActorLocation` (`self.GetOwner`)) (`self.Move To Loc`)) 135.0))
    (bind _aspawn (cast `Pawn` (`self.GetOwner`)))
    (`Actor.K2_SetActorRotation` (`self.GetOwner`) (`KismetMathLibrary.MakeRotator` 0.0 0.0 _returnvalue_yaw) true)
    (`Pawn.AddMovementInput` _aspawn (`Actor.GetActorForwardVector` (`self.GetOwner`)) 1.0 true)))

(event `Start Charmed / Turned Movement`
  (if (not (`KismetSystemLibrary.K2_IsValidTimerHandle` (`self.Charmed / Turned Movement Timer`)))
    (bind _returnvalue (`KismetSystemLibrary.K2_SetTimerDelegate` (delegate `Charmed / Turned Actual Movement`) 0.01 true))
    (set `self.Charmed / Turned Movement Timer` _returnvalue)))

(event `Stop Charmed / Turned Movement`
  (`KismetSystemLibrary.K2_ClearAndInvalidateTimerHandle` (`self.Charmed / Turned Movement Timer`)))

(fn `Add Status`
  (params (`Status Effect` :type "GameplayTag Structure") (`Status Struct` :type "/Game/Combat/Status_Effects/Structs_Tables/Struct_Status_Effects Structure") (`Damage Dealer` :type "Actor Object Reference"))
  (bind ((`Burn_2_A31ADAD5466B6E04845AB7BDAFECC735` _burn) (`Bleeding_13_B61CBB8C42FA68FFED01288F5A225E45` _bleeding) (`CharmedTurned_24_EF1FB2024F9506FF1C949EB01835F961` _charmedturned)) (break `/Game/Combat/Status_Effects/Structs_Tables/Struct_Status_Effects` `Status Struct`))
  (bind _damage_dealer (`self.Damage Dealer`))
  (bind _status_struct_variable (`self.Status Struct Variable`))
  (bind _damage_dealer_2 (`self.Damage Dealer`))
  (bind ((`BleedDuration_8_7F742F6C480905803B3A8986EE73C504` _bleedduration) (`Chance_12_E8F417AA4EB7F5199495D99D141F612B` _chance)) (break `/Game/Combat/Status_Effects/Structs_Tables/Struct_Bleeding` (`.Bleeding_13_B61CBB8C42FA68FFED01288F5A225E45` (break `/Game/Combat/Status_Effects/Structs_Tables/Struct_Status_Effects` _status_struct_variable))))
  (bind ((`Duration_17_639C84964633395F9125BE8130B45740` _duration)) (break `/Game/Combat/Status_Effects/Structs_Tables/Struct_Charmed_Turned` (`.CharmedTurned_24_EF1FB2024F9506FF1C949EB01835F961` (break `/Game/Combat/Status_Effects/Structs_Tables/Struct_Status_Effects` (`self.Status Struct Variable`)))))
  (bind ((`Chance_15_16F3BD6A416F412D410206BE34FB0D85` _chance_2) (`Duration_17_639C84964633395F9125BE8130B45740` _duration_2)) (break `/Game/Combat/Status_Effects/Structs_Tables/Struct_Charmed_Turned` (`.CharmedTurned_24_EF1FB2024F9506FF1C949EB01835F961` (break `/Game/Combat/Status_Effects/Structs_Tables/Struct_Status_Effects` (`self.Status Struct Variable`)))))
  (bind ((`BleedDuration_8_7F742F6C480905803B3A8986EE73C504` _bleedduration_2) (`Chance_12_E8F417AA4EB7F5199495D99D141F612B` _chance_3)) (break `/Game/Combat/Status_Effects/Structs_Tables/Struct_Bleeding` (`.Bleeding_13_B61CBB8C42FA68FFED01288F5A225E45` (break `/Game/Combat/Status_Effects/Structs_Tables/Struct_Status_Effects` _status_struct_variable))))
  (bind ((`BleedDuration_8_7F742F6C480905803B3A8986EE73C504` _bleedduration_3)) (break `/Game/Combat/Status_Effects/Structs_Tables/Struct_Bleeding` (`.Bleeding_13_B61CBB8C42FA68FFED01288F5A225E45` (break `/Game/Combat/Status_Effects/Structs_Tables/Struct_Status_Effects` (`self.Status Struct Variable`)))))
  (bind ((`BurnDuration_19_CC3019BB477E49886AFAA1A45E0B295E` _burnduration)) (break `/Game/Combat/Status_Effects/Structs_Tables/Struct_Burned` (`.Burn_2_A31ADAD5466B6E04845AB7BDAFECC735` (break `/Game/Combat/Status_Effects/Structs_Tables/Struct_Status_Effects` (`self.Status Struct Variable`)))))
  (set `self.Status Struct Variable` `Status Struct`)
  (set `self.Damage Dealer` `Damage Dealer`)
  (if (`BlueprintGameplayTagLibrary.HasTag` (`self.StatusEffects`) `Status Effect`)
    (`|SwitchGameplayTag` `Status Effect`
      (:`Bleed`
        (if (`KismetMathLibrary.RandomBoolWithWeight` _chance)
          (`self.ClearStatusWithTimer` _bleedduration (struct :`TagName` "Bleed"))
          (`self.Add Status Effect To HUD` "NewEnumerator3" _bleedduration)))
      (:`Burn`
        (if (`KismetMathLibrary.RandomBoolWithWeight` _chance_3)
          (`self.ClearStatusWithTimer` _bleedduration_2 (struct :`TagName` "Burn"))
          (`self.Add Status Effect To HUD` "NewEnumerator2" _bleedduration_2)))
      (:`Charmed / Turned`
        (if (and (`KismetMathLibrary.RandomBoolWithWeight` _chance_2) (select `bool` (`KismetSystemLibrary.DoesImplementInterface` (`self.GetOwner`) "/Game/Player/Interfaces/BPI_Player.BPI_Player_C") :`false` (`KismetSystemLibrary.DoesImplementInterface` _damage_dealer_2 "/Game/Player/Interfaces/BPI_Player.BPI_Player_C") :`true` (`KismetSystemLibrary.DoesImplementInterface` _damage_dealer_2 "/Game/Enemies/Interfaces/BPI_Enemy.BPI_Enemy_C")))
          ;[1 1 1] Clearing turned target and potential turned targets array
          (set `self.Turned Target` null)
          (`KismetArrayLibrary.Array_Clear` (`self.Potential Turned Targets`))
          ;[1 1 1] Call the clear status timer function again to add to the retriggerable delay
          (`self.ClearStatusWithTimer` _duration_2 (struct :`TagName` "Charmed / Turned"))
          (`self.Add Status Effect To HUD` "NewEnumerator5" _duration_2))))
    (else
      (`|SwitchGameplayTag` `Status Effect`
        (:`Bleed`
          (if (`KismetMathLibrary.RandomBoolWithWeight` (`.Chance_12_E8F417AA4EB7F5199495D99D141F612B` (break `/Game/Combat/Status_Effects/Structs_Tables/Struct_Bleeding` _bleeding)))
            ;[1 1 1] Bleeding
            (`BlueprintGameplayTagLibrary.AddGameplayTag` (`self.StatusEffects`) (struct :`TagName` "Bleed"))
            (bind _returnvalue (`KismetSystemLibrary.K2_SetTimer` null "Bleeding" 1.0 true))
            (set `self.BleedTimerHandle` _returnvalue)
            (`self.ClearStatusWithTimer` _bleedduration_3 (struct :`TagName` "Bleed"))
            (`self.Add Status Effect To HUD` "NewEnumerator3" _bleedduration_3)))
        (:`Burn`
          (if (`KismetMathLibrary.RandomBoolWithWeight` (`.Chance_24_7F084E7144864765DBA1258CFC08CB7A` (break `/Game/Combat/Status_Effects/Structs_Tables/Struct_Burned` _burn)))
            (`BlueprintGameplayTagLibrary.AddGameplayTag` (`self.StatusEffects`) (struct :`TagName` "Burn"))
            ;[1 1 1] Burning
            (bind _returnvalue_2 (`KismetSystemLibrary.K2_SetTimer` null "Burning" 1.0 true))
            (set `self.BleedTimerHandle` _returnvalue_2)
            (`self.ClearStatusWithTimer` _burnduration (struct :`TagName` "Burn"))
            (`self.Add Status Effect To HUD` "NewEnumerator2" _burnduration)))
        (:`Charmed / Turned`
          ;[1 1 1] Add the gameplay tag
          (if (and (`KismetMathLibrary.RandomBoolWithWeight` (`.Chance_15_16F3BD6A416F412D410206BE34FB0D85` (break `/Game/Combat/Status_Effects/Structs_Tables/Struct_Charmed_Turned` _charmedturned))) (select `bool` (`KismetSystemLibrary.DoesImplementInterface` (`self.GetOwner`) "/Game/Player/Interfaces/BPI_Player.BPI_Player_C") :`false` (`KismetSystemLibrary.DoesImplementInterface` _damage_dealer "/Game/Player/Interfaces/BPI_Player.BPI_Player_C") :`true` (`KismetSystemLibrary.DoesImplementInterface` _damage_dealer "/Game/Enemies/Interfaces/BPI_Enemy.BPI_Enemy_C")))
            (`BlueprintGameplayTagLibrary.AddGameplayTag` (`self.StatusEffects`) (struct :`TagName` "Charmed / Turned"))
            ;[1 1 1] Reset the turned target and potential turned targets array
            (set `self.Turned Target` null)
            (`KismetArrayLibrary.Array_Clear` (`self.Potential Turned Targets`))
            ;[1 1 1] Start the charmed / turned function
            (bind _returnvalue_3 (`KismetSystemLibrary.K2_SetTimer` null "Charmed / Turned" 0.3 true))
            ;[1 1 1] Set the charmed / turned timer
            (set `self.Charmed / Turned Timer` _returnvalue_3)
            ;[1 1 1] Start the timer for clearing the timer for the charmed / turned function
            (`self.ClearStatusWithTimer` _duration (struct :`TagName` "Charmed / Turned"))
            (`self.Add Status Effect To HUD` "NewEnumerator5" _duration)))))))

(fn `Bleeding`
  (bind _returnvalue (`self.GetOwner`))
  (bind (_bleeddamage _bleedduration _hitstop) (break `/Game/Combat/Status_Effects/Structs_Tables/Struct_Bleeding` (`.Bleeding_13_B61CBB8C42FA68FFED01288F5A225E45` (break `/Game/Combat/Status_Effects/Structs_Tables/Struct_Status_Effects` (`self.Status Struct Variable`)))))
  (`/Game/Health/Components/BPC_Health_V2.Take Damage` (`Actor.GetComponentByClass` (`self.GetOwner`) "/Game/Health/Components/BPC_Health_V2.BPC_Health_V2_C") _bleeddamage (`self.Damage Dealer`) (`KismetMathLibrary.RandomUnitVector`) (`Actor.K2_GetActorLocation` _returnvalue) 0.0 0.0)
  (if _hitstop
    (`/Game/Combat/Components/BPC_HitStop.INITIAITE HIT STOP!` (`Actor.GetComponentByClass` _returnvalue "/Game/Combat/Components/BPC_HitStop.BPC_HitStop_C") _bleeddamage)))

(fn `Burning`
  (bind _returnvalue (`self.GetOwner`))
  (bind _returnvalue_2 (`Actor.K2_GetActorLocation` _returnvalue))
  (bind (_burndamage _burnduration _damagemultiplier _speedmultiplier _spreadchance) (break `/Game/Combat/Status_Effects/Structs_Tables/Struct_Burned` (`.Burn_2_A31ADAD5466B6E04845AB7BDAFECC735` (break `/Game/Combat/Status_Effects/Structs_Tables/Struct_Status_Effects` (`self.Status Struct Variable`)))))
  (`/Game/Health/Components/BPC_Health_V2.Take Damage` (`Actor.GetComponentByClass` _returnvalue "/Game/Health/Components/BPC_Health_V2.BPC_Health_V2_C") _burndamage (`self.Damage Dealer`) (0.0 0.0 0.0) (0.0 0.0 0.0) 0.0 0.0)
  (bind _outhits (`KismetSystemLibrary.SphereTraceMultiForObjects` :`Start` _returnvalue_2 :`End` _returnvalue_2 :`Radius` 250.0 :`ObjectTypes` (`|MakeArray` "ObjectTypeQuery8" "ObjectTypeQuery7" :!type "EObjectTypeQuery Enum") :`DrawDebugType` "ForDuration"))
  (for _array_element _outhits
    (bind _returnvalue_3 (`Actor.GetComponentByClass` (`.HitActor` (`GameplayStatics.BreakHitResult` _array_element)) "BPC_StatusEffectHandler_C"))
    (if (`BlueprintGameplayTagLibrary.HasTag` (`/Game/Combat/Status_Effects/Components/BPC_StatusEffectHandler.StatusEffects` _returnvalue_3) (struct :`TagName` "Burn"))
      _
      (elif (`KismetMathLibrary.RandomBoolWithWeight` _spreadchance)
        (`self.Add Status` _returnvalue_3 (struct :`TagName` "Burn") (`self.Status Struct Variable`) (`self.GetOwner`))))))

(fn `Charmed / Turned`
  (bind _returnvalue (`Actor.K2_GetActorLocation` (`self.GetOwner`)))
  (bind _returnvalue_2 (`Actor.GetComponentByClass` (`self.GetOwner`) "/Game/Combat/Components/BPC_AttackHandler.BPC_AttackHandler_C"))
  (bind _returnvalue_3 (`Actor.K2_GetActorLocation` (`self.GetOwner`)))
  (bind ((`Duration_17_639C84964633395F9125BE8130B45740` _duration) (`UpdateTargetCount_22_1A7A193D4165F324FC4F87AA58A64C4C` _updatetargetcount)) (break `/Game/Combat/Status_Effects/Structs_Tables/Struct_Charmed_Turned` (`.CharmedTurned_24_EF1FB2024F9506FF1C949EB01835F961` (break `/Game/Combat/Status_Effects/Structs_Tables/Struct_Status_Effects` (`self.Status Struct Variable`)))))
  ;[1 1 1] Calculate whether we should do another target calculation based on the duration of the status effect, the update target count in the status effect info and the current game time in seconds as well as the last time that the calculation was done and also that the target count isn't 0
  (if (and (>= (`KismetSystemLibrary.GetGameTimeInSeconds`) (+ (`self.Last Turned / Charmed Calc Time`) (/ _duration _updatetargetcount))) (!= _updatetargetcount 0))
    ;[1 1 1] Get game time as seconds since this is now the last time that the pass should be done for the turned / charmed target detection and then also clear the turned target
    (set `self.Last Turned / Charmed Calc Time` (`KismetSystemLibrary.GetGameTimeInSeconds`))
    (set `self.Turned Target` null))
  (if (not (`self.Set Speed Charmed / Turned`))
    ;[1 1 1] If we haven't already set the speed to the new speed percentage then do that and set the bool variable to indicate this to be true
    (`/Game/Movement/Basic_Movement/BPC_Movement_Manager.Set Speed Multiplier` (`Actor.GetComponentByClass` (`self.GetOwner`) "/Game/Movement/Basic_Movement/BPC_Movement_Manager.BPC_Movement_Manager_C") (`.PercentageMoveSpeedSlow_19_BA2382774A23599A9192E59BD9F26660` (break `/Game/Combat/Status_Effects/Structs_Tables/Struct_Charmed_Turned` (`.CharmedTurned_24_EF1FB2024F9506FF1C949EB01835F961` (break `/Game/Combat/Status_Effects/Structs_Tables/Struct_Status_Effects` (`self.Status Struct Variable`))))))
    (set `self.Set Speed Charmed / Turned` true))
  (`/Engine/EditorBlueprintResources/StandardMacros.IsValid` (`self.Turned Target`)
    (:`Is Valid`
      ;[1 1 1] If no potential targets in area then we go in a random direction
      (if (`KismetArrayLibrary.Array_IsEmpty` (`self.Potential Turned Targets`)) :!label _label
        ;[1 1 1] Charmed movement as well as ignoring move input and deactivating enemy if the owner of this component is an enemy
        (`|ExecutionSequence`
          (:`then_0`
            (bind _ascharacter (cast `Character` (`self.GetOwner`)))
            (bind _returnvalue_4 (`Pawn.GetController` _ascharacter))
            (`Controller.SetIgnoreMoveInput` _returnvalue_4 true)
            (bind _asac_enemy (cast `/Game/Enemies/AI/Controllers/AC_Enemy` _returnvalue_4))
            (`/Game/Enemies/AI/Controllers/AC_Enemy.Deactivate Enemy` _asac_enemy))
          (:`then_1`
            (if (or (== (`Actor.K2_GetActorLocation` (`self.GetOwner`)) (`self.Move To Loc`) :`ErrorTolerance` 100.0) (`KismetMathLibrary.EqualExactly_VectorVector` (`self.Move To Loc`)))
              (bind _randomlocation (`NavigationSystemV1.K2_GetRandomLocationInNavigableRadius` (`Actor.K2_GetActorLocation` (`self.GetOwner`)) 250.0 null null))
              (set `self.Move To Loc` _randomlocation)
              (set `self.Last Turned / Charmed Calc Time` (`KismetSystemLibrary.GetGameTimeInSeconds`))
              (else
                (`self.Start Charmed / Turned Movement`)))))
        (else
          ;[1 1 1] Since there are potential targets we get the closest and that is the turned target
          (set `self.Turned Target` (`.ReturnValue` (`GameplayStatics.FindNearestActor` (`Actor.K2_GetActorLocation` (`self.GetOwner`)) (`self.Potential Turned Targets`))))
          (`|ExecutionSequence`
            (:`then_0`
              ;[1 1 1] Setting the move input to be ignored and if it is an enemy then to deactivate the enemy
              (bind _ascharacter_2 (cast `Character` (`self.GetOwner`)))
              (bind _returnvalue_5 (`Pawn.GetController` _ascharacter_2))
              (`Controller.SetIgnoreMoveInput` _returnvalue_5 true)
              (bind _asac_enemy_2 (cast `/Game/Enemies/AI/Controllers/AC_Enemy` _returnvalue_5))
              (`/Game/Enemies/AI/Controllers/AC_Enemy.Deactivate Enemy` _asac_enemy_2))
            (:`then_1`
              ;[1 1 1] Setting location to move to and starting the movement function and then also the process of constantly attacking with dependencies on whether the owner of this component is a player or enemy and then depending on the enemy info if the owner is an enemy
              (set `self.Move To Loc` (`Actor.K2_GetActorLocation` (`self.Turned Target`)))
              (`self.Start Charmed / Turned Movement`)
              (if (`KismetSystemLibrary.DoesImplementInterface` (`self.GetOwner`) "/Game/Player/Interfaces/BPI_Player.BPI_Player_C")
                (`/Game/Combat/Components/BPC_AttackHandler.Melee Attack Start` _returnvalue_2)
                (else
                  (bind _enemy_info (message `/Game/Enemies/Interfaces/BPI_Enemy.Get Enemy Info` (`self.GetOwner`)))
                  (bind ((`RangedEnemy?_9_5A91CDBB41D4361B9D352C81F4000FF9` _rangedenemy_) (`CanMelee?_11_84FB58B845678B6142122A89E5E526DB` _canmelee_)) (break `/Game/Enemies/Structs_Tables/Struct_Enemy_Info` _enemy_info))
                  (if _canmelee_
                    (`/Game/Combat/Components/BPC_AttackHandler.Melee Attack Start` _returnvalue_2)
                    (elif _rangedenemy_
                      (`/Game/Combat/Components/BPC_AttackHandler.Ranged Attack Start` _returnvalue_2)
                      (`KismetSystemLibrary.K2_SetTimer` _returnvalue_2 "Ranged Attack End" (`KismetMathLibrary.RandomFloatInRange` 0.5 2.5)))))))))))
    (:`Is Not Valid`
      (if (`.Charmed?_10_9E206C954EE994DA7CFF5B8129D2F809` (break `/Game/Combat/Status_Effects/Structs_Tables/Struct_Charmed_Turned` (`.CharmedTurned_24_EF1FB2024F9506FF1C949EB01835F961` (break `/Game/Combat/Status_Effects/Structs_Tables/Struct_Status_Effects` (`self.Status Struct Variable`)))))
        ;[1 1 1] Get location of the character that charmed this character and then set that to be the move to loc and then call the start charmed / turned movement function
        (set `self.Move To Loc` (`Actor.K2_GetActorLocation` (`self.Damage Dealer`)))
        (`self.Start Charmed / Turned Movement`)
        (else
          (`KismetArrayLibrary.Array_Clear` (`self.Potential Turned Targets`))
          (if (`KismetSystemLibrary.DoesImplementInterface` (`self.Damage Dealer`) "/Game/Player/Interfaces/BPI_Player.BPI_Player_C")
            ;[1 1 1] Detect other enemies within a certain range and add them to the potential turned targets array
            (bind (_outhits _returnvalue_6) (`KismetSystemLibrary.SphereTraceMultiForObjects` _returnvalue_3 _returnvalue_3 1500.0 (`|MakeArray` "ObjectTypeQuery8" :!type "EObjectTypeQuery Enum") false (`|MakeArray` (`self.GetOwner`)) "Persistent"))
            (if _returnvalue_6
              (for _array_element _outhits
                (bind (_bblockinghit _binitialoverlap _time _distance _location _impactpoint _normal _impactnormal _physmat _hitactor) (`GameplayStatics.BreakHitResult` _array_element))
                (if (not (`KismetArrayLibrary.Array_Contains` (`self.Potential Turned Targets`) _hitactor))
                  (`KismetArrayLibrary.Array_Add` (`self.Potential Turned Targets`) _hitactor)))
              (goto _label)
              (else
                (goto _label)))
            (else
              ;[1 1 1] Detect other players within a certain range and add them to the potential turned targets array
              (bind (_outhits_2 _returnvalue_7) (`KismetSystemLibrary.SphereTraceMultiForObjects` _returnvalue _returnvalue 1500.0 (`|MakeArray` "ObjectTypeQuery7" :!type "EObjectTypeQuery Enum") false (`|MakeArray` (`self.GetOwner`)) "ForOneFrame"))
              (if _returnvalue_7
                (for _array_element_2 _outhits_2
                  (bind (_bblockinghit_2 _binitialoverlap_2 _time_2 _distance_2 _location_2 _impactpoint_2 _normal_2 _impactnormal_2 _physmat_2 _hitactor_2) (`GameplayStatics.BreakHitResult` _array_element_2))
                  (if (not (`KismetArrayLibrary.Array_Contains` (`self.Potential Turned Targets`) _hitactor_2))
                    (`KismetArrayLibrary.Array_Add` (`self.Potential Turned Targets`) _hitactor_2)))
                (goto _label)
                (else
                  (goto _label))))))))))