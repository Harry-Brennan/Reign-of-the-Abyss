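; Actor component that tracks whether its owner is in combat and passively regenerates health while out of combat.
; DelayInCombatReset sets InCombat and clears it after a retriggerable delay, so repeated calls extend combat.
; Tick stops the looping heal timer while in combat, downed or in downed transition, and starts it otherwise.
; Each heal picks the payload or player health component and amount by the owner's interface.
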(event `Delay In Combat Reset`
  ;[1 1 1] Delays the setting of the incombat variable to false so keeping the owner "in combat"
  (set `self.In Combat` true)
  (`KismetSystemLibrary.RetriggerableDelay` (`self.Combat Delay`))
  (set `self.In Combat` false))

(event `self.ReceiveTick`
  (params (DeltaSeconds :type "Float (single-precision)"))
  (bind _in_combat (`self.In Combat`))
  (bind _returnvalue (`Actor.GetComponentByClass` (`self.GetOwner`) "/Game/Health/Components/BPC_Health_V2.BPC_Health_V2_C"))
  ;[1 1 1] Constantly checkinf if in combat or downed or downed transition and if so then we check if the heal timer is valid and if so we clear and invalidate it, if we are out of combat then we check if the timer is valid and if not then we start the timer by the heal event with the time for the loop being the heal interval variable and we set the heal timer variable to be this timer we just set
  (`/Engine/EditorBlueprintResources/StandardMacros.IsValid` _returnvalue
    (:`Is Valid`
      (if (or _in_combat (or (`/Game/Health/Components/BPC_Health_V2.Downed` _returnvalue) (`/Game/Health/Components/BPC_Health_V2.DownedTransition` _returnvalue)))
        (if (`KismetSystemLibrary.K2_IsValidTimerHandle` (`self.Heal Timer`)) :!label _label
          (`KismetSystemLibrary.K2_ClearAndInvalidateTimerHandle` (`self.Heal Timer`)))
        (else
          (if (not (`KismetSystemLibrary.K2_IsValidTimerHandle` (`self.Heal Timer`))) :!label _label_2
            (bind _returnvalue_2 (`KismetSystemLibrary.K2_SetTimerDelegate` (delegate `Heal`) (`self.Heal Interval`) true))
            (set `self.Heal Timer` _returnvalue_2)))))
    (:`Is Not Valid`
      (if _in_combat
        (goto _label)
        (else
          (goto _label_2))))))

(event `Heal`
  (bind _returnvalue (`self.GetOwner`))
  (bind _returnvalue_2 (`self.GetOwner`))
  ;[1 1 1] Heal the owning character or payload depending on implementation of interfaces healing the amount of the heal amount variables
  (if (`KismetSystemLibrary.DoesImplementInterface` _returnvalue_2 "/Game/Co-op/Interfaces/BPI_Payload.BPI_Payload_C")
    (`/Game/Health/Components/BPC_PayloadHealth.Heal` (`Actor.GetComponentByClass` _returnvalue "/Game/Health/Components/BPC_PayloadHealth.BPC_PayloadHealth_C") (`self.Heal Amount Payload`))
    (elif (`KismetSystemLibrary.DoesImplementInterface` _returnvalue_2 "/Game/Player/Interfaces/BPI_Player.BPI_Player_C")
      (`/Game/Health/Components/BPC_Health_V2.Heal` (`Actor.GetComponentByClass` _returnvalue "/Game/Health/Components/BPC_Health_V2.BPC_Health_V2_C") (`self.Heal Amount Player`)))))