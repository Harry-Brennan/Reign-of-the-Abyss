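; BPC_AttackHandler is an attack component that routes ranged and melee input to its owner's combat components.
; Tick sets CanAttack whenever neither BPC_Ranged_Attack is firing nor BPC_LightAttacks is attacking.
; Ranged input, gated by CanAttack and the current BPC_Spells cooldown, starts the spell on Triggered, then finishes and resets charge on Canceled or Completed.
; Melee input triggers a light attack, also serving as ranged characters' last resort.
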(event `self.ReceiveTick`
  (params (DeltaSeconds :type "Float (single-precision)"))
  ;[1 1 1] SETTING IF CAN ATTACK
  (set `self.Can Attack` (and (not (`/Game/Combat/Ranged/Components/BPC_Ranged_Attack.Firing Spell` (`Actor.GetComponentByClass` (`self.GetOwner`) "/Game/Combat/Ranged/Components/BPC_Ranged_Attack.BPC_Ranged_Attack_C"))) (not (`/Game/Combat/Weapons/Melee/Components/BPC_LightAttacks.Attacking` (`Actor.GetComponentByClass` (`self.GetOwner`) "/Game/Combat/Weapons/Melee/Components/BPC_LightAttacks.BPC_LightAttacks_C"))))))

(event `EnhancedInput|/Game/Player/Input/Actions/Ranged/IA_Ranged_Attack`
  (params (ActionValue :type Boolean) (ElapsedSeconds :type "Float (double-precision)") (TriggeredSeconds :type "Float (double-precision)") (InputAction :type "InputAction Object Reference" :default "/Game/Player/Input/Actions/Ranged/IA_Ranged_Attack.IA_Ranged_Attack"))
  (bind _returnvalue (`Actor.GetComponentByClass` (`self.GetOwner`) "/Game/Combat/Ranged/Components/BPC_Spells.BPC_Spells_C"))
  (bind _returnvalue_2 (`Actor.GetComponentByClass` (`self.GetOwner`) "/Game/Combat/Ranged/Components/BPC_Ranged_Attack.BPC_Ranged_Attack_C"))
  (bind _returnvalue_3 (and (not (`|GetArrayItem` (`/Game/Combat/Ranged/Components/BPC_Spells.Spell Cooldowns Active` _returnvalue) (`/Game/Combat/Ranged/Components/BPC_Spells.Current Spell Index` _returnvalue))) (`self.Can Attack`)))
  ;[1 1 1] Ranged attack input
  (:`Triggered`
    ;[1 1 1] Set bool for attempting to ranged attack depending on input action
    (set `self.Attempting to Ranged Attack` true)
    (if _returnvalue_3
      ;[1 1 1] Get the current spell's info
      (bind _spell (message `/Game/Combat/Ranged/Interfaces/BPI_Has_Ranged_Attack.Get Current Spell` (`self.GetOwner`)))
      ;[1 1 1] Call start ranged attack from the owner's ranged attack component passing the triggered seconds of the input action and the current spell as the attempting spell
      (`/Game/Combat/Ranged/Components/BPC_Ranged_Attack.Start Ranged Attack` (`Actor.GetComponentByClass` (`self.GetOwner`) "/Game/Combat/Ranged/Components/BPC_Ranged_Attack.BPC_Ranged_Attack_C") TriggeredSeconds _spell)))
  (:`Canceled`
    (set `self.Attempting to Ranged Attack` false :!label _label)
    (if _returnvalue_3
      ;[1 1 1] Call the finish ranged attack function from the owner's ranged attack component passing the triggered seconds of the input action as the elapsed seconds parameter and then calling the reset charge function in the same component
      (`/Game/Combat/Ranged/Components/BPC_Ranged_Attack.Finish Ranged Attack` _returnvalue_2 TriggeredSeconds)
      (`/Game/Combat/Ranged/Components/BPC_Ranged_Attack.Reset Charge` _returnvalue_2)))
  (:`Completed`
    (goto _label)))

(event `EnhancedInput|/Game/Player/Input/Actions/Melee/IA_MeleeInput`
  (params (ActionValue :type Boolean) (ElapsedSeconds :type "Float (double-precision)") (TriggeredSeconds :type "Float (double-precision)") (InputAction :type "InputAction Object Reference" :default "/Game/Player/Input/Actions/Melee/IA_MeleeInput.IA_MeleeInput"))
  ;[1 1 1] Melee input for general melee attacking that ranged characters will also have access to as a last resort for melee combat
  (:`Triggered`
    (if (`self.Can Attack`)
      (`/Game/Combat/Weapons/Melee/Components/BPC_LightAttacks.LightAttack` (`Actor.GetComponentByClass` (`self.GetOwner`) "/Game/Combat/Weapons/Melee/Components/BPC_LightAttacks.BPC_LightAttacks_C")))))