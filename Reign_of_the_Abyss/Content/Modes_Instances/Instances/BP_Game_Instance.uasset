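; Game instance Blueprint that holds player setup and audio volume settings.
; SetupPlayers stores the active players and their info on the instance.
; UpdateSound applies the stored Master, Music, Menu and VFX volumes as sound class overrides, each through its own sound mix.
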(fn `Setup Players`
  (params (`Active Players` :type "Array of Boolean") (`Players Info` :type "Array of /Game/General_Character_Things/Enums/Enum_Character_Names Enum"))
  (set `self.Active Players` `Active Players`)
  (set `self.Players Info` `Players Info`))

(fn `Update Sound`
  (`GameplayStatics.SetSoundMixClassOverride` "/Game/SFX/Classes/Sound_MIX_Classes/SCM_Master.SCM_Master" "/Game/SFX/Classes/Sound_Classes/SC_Master.SC_Master" (`self.Master Volume`))
  (`GameplayStatics.SetSoundMixClassOverride` "/Game/SFX/Classes/Sound_MIX_Classes/SCM_Music.SCM_Music" "/Game/SFX/Classes/Sound_Classes/SC_Music.SC_Music" (`self.Music Volume`))
  (`GameplayStatics.SetSoundMixClassOverride` "/Game/SFX/Classes/Sound_MIX_Classes/SCM_Menu.SCM_Menu" "/Game/SFX/Classes/Sound_Classes/SC_Menu.SC_Menu" (`self.Menu Volume`))
  (`GameplayStatics.SetSoundMixClassOverride` "/Game/SFX/Classes/Sound_MIX_Classes/SCM_VFX.SCM_VFX" "/Game/SFX/Classes/Sound_Classes/SC_VFX.SC_VFX" (`self.VFX Volume`)))