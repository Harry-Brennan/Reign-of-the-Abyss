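; BPC_LightAttacks is a melee weapon component that plays light attack montages.
; LightAttack looks up WeaponName in DT_MeleeWeapons and uses AttackIndex, which this graph never changes, to pick one of the row's three montages.
; An Attacking flag blocks re-entry until the montage's Attack End notify clears it.
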(event `LightAttack`
  (if (not (`self.Attacking`))
    (bind _returnvalue (`|GetDataTableRow` "/Game/Weapons/Melee/Structs_Tables/DT_MeleeWeapons.DT_MeleeWeapons" (`self.WeaponName`))
      (:`then`
        (set `self.Attacking` true)
        (bind (_attackmontage1 _attackmontage2 _attackmontage3) (break `/Game/Weapons/Melee/Structs_Tables/S_MeleeWeapon` _returnvalue))
        (bind _notifyname (`|PlayMontage` null (select `int` (`self.AttackIndex`) :`0` _attackmontage1 :`1` _attackmontage2 :`2` _attackmontage3))
          (:`OnNotifyBegin`
            (switch `name` _notifyname
              (:`AttackEnd`
                (set `self.Attacking` false)))))))))