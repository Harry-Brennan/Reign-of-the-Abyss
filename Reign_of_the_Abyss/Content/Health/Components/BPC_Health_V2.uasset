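; Health component for players, enemies and bosses that handles damage, death, downing and revival, initialised from owner health info.
; TakeDamage plays hit feedback, applies knockback, reduces damage for rolling or same-faction hits and triggers boss phase two.
; Death either explodes the owner, alerting nearby AI when an enemy dies, or downs it, ending the game once all players are down.
; StartRevive half-heals the nearest downed character; older input-based revive logic is disconnected.
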(event `self.ReceiveBeginPlay`
  (bind _health_info (message `/Game/Health/Interfaces/BPI_Has_Health.Get Health Info` (`self.GetOwner`)))
  (bind _output_get (set `self.Owner Health Info` _health_info))
  (bind ((`StartingHealth_4_91E796F8462112FCE066E8B01D9FBC5F` _startinghealth) (`MaximumHealth_5_44F73FCC42A9E13C8ACBC398ED91715C` _maximumhealth)) (break `/Game/Health/Structs_Tables/Struct_Health_Info` _output_get))
  (set `self.Current Health` _startinghealth)
  (set `self.Maximum Health` _maximumhealth))

(event `EnhancedInput|/Game/Player/Input/Actions/Miscellaneous/IA_Revive`
  (params (ActionValue :type Boolean) (ElapsedSeconds :type "Float (double-precision)") (TriggeredSeconds :type "Float (double-precision)") (InputAction :type "InputAction Object Reference" :default "/Game/Player/Input/Actions/Miscellaneous/IA_Revive.IA_Revive")))

(fn `Death`
  (params (`Character Responsible For Death` :type "Actor Object Reference"))
  (locals (`Game Over?` :type Boolean))
  (bind _returnvalue (`Actor.K2_GetActorLocation` (`self.GetOwner`)))
  (`KismetSystemLibrary.PrintString` "DEATH")
  (if (`KismetSystemLibrary.DoesImplementInterface` (`self.GetOwner`) "/Game/Enemies/Interfaces/BPI_Boss.BPI_Boss_C")
    (bind _asbp_third_person_game_mode (cast `/Game/Modes_Instances/Modes/BP_ThirdPersonGameMode` (`GameplayStatics.GetGameMode`))
      (:`then`
        (`/Game/UI/HUD/Widgets/WBP_HUD.Play Boss Death Animation` (`/Game/Modes_Instances/Modes/BP_ThirdPersonGameMode.HUD Ref` _asbp_third_person_game_mode)))
      (:`CastFailed`
        _)))
  (switch `/Game/Health/Enums/Enum_Death_Types` (`.DeathType_18_4504017348CFBE64097445804BB9B65E` (break `/Game/Health/Structs_Tables/Struct_Health_Info` (`self.Owner Health Info`)))
    (:`NewEnumerator0`
      (`|SpawnActorFromClass` "/Game/VFX/Bloodsplosion/BPs/BP_BloodSplosion.BP_BloodSplosion_C" (`KismetMathLibrary.MakeTransform` (`Actor.K2_GetActorLocation` (`self.GetOwner`))) "AlwaysSpawn" "MultiplyWithRoot" (`self.GetOwner`) (`KismetMathLibrary.Clamp` (* (`self.Maximum Health`) 2) 0 500) null)
      (`Actor.SetActorHiddenInGame` (`self.GetOwner`) true)
      (`KismetSystemLibrary.K2_SetTimer` null "Destroy Owning Actor & Associated Weapons" 0.2)
      (if (`KismetSystemLibrary.DoesImplementInterface` (`self.GetOwner`) "/Game/Enemies/Interfaces/BPI_Enemy.BPI_Enemy_C")
        (bind (_outhits _returnvalue_2) (`KismetSystemLibrary.SphereTraceMultiForObjects` _returnvalue _returnvalue 500.0 (`|MakeArray` "ObjectTypeQuery8" :!type "EObjectTypeQuery Enum") false (`|MakeArray` (`self.GetOwner`)) "ForDuration"))
        (if _returnvalue_2
          (for _array_element _outhits
            (bind _asac_enemy (cast `/Game/Enemies/AI/Controllers/AC_Enemy` (`AIBlueprintHelperLibrary.GetAIController` (`.HitActor` (`GameplayStatics.BreakHitResult` _array_element)))))
            (`/Game/Enemies/Interfaces/BPI_Enemy_Controller.Update State` _asac_enemy "NewEnumerator1")
            (bind _output_get (set `/Game/Enemies/AI/Controllers/AC_Enemy.Chasing_Character` (`local.Character Responsible For Death`) _asac_enemy))
            (`AIController.K2_SetFocus` _asac_enemy _output_get)))))
    (:`NewEnumerator1`
      (set `self.DownedTransition` true)
      (`/Game/Movement/Basic_Movement/BPC_Movement_Manager.Set Speed Multiplier` (`Actor.GetComponentByClass` (`self.GetOwner`) "/Game/Movement/Basic_Movement/BPC_Movement_Manager.BPC_Movement_Manager_C") 0.9)
      (`CapsuleComponent.SetCapsuleHalfHeight` (`Actor.GetComponentByClass` (`self.GetOwner`) "/Script/Engine.CapsuleComponent") 35.0 true)
      (`SceneComponent.K2_SetRelativeLocation` (`Actor.GetComponentByClass` (`self.GetOwner`) "/Script/Engine.SkeletalMeshComponent") (0.0 0.0 0.0) false false)
      (`SceneComponent.K2_SetRelativeLocation` (`Actor.GetComponentByClass` (`self.GetOwner`) "/Script/UMG.WidgetComponent") (0.0 0.0 -10.0) false false)
      (bind _asbp_third_person_game_mode_2 (cast `/Game/Modes_Instances/Modes/BP_ThirdPersonGameMode` (`GameplayStatics.GetGameMode`)))
      (set `local.Game Over?` true)
      (for _array_element_2 (`/Game/Modes_Instances/Modes/BP_ThirdPersonGameMode.Players` _asbp_third_person_game_mode_2)
        (bind _returnvalue_3 (`Actor.GetComponentByClass` _array_element_2 "BPC_Health_V2_C"))
        (if (not (or (`/Game/Health/Components/BPC_Health_V2.Downed` _returnvalue_3) (`/Game/Health/Components/BPC_Health_V2.DownedTransition` _returnvalue_3)))
          (set `local.Game Over?` false)))
      (if (`local.Game Over?`)
        (`KismetSystemLibrary.K2_SetTimer` _asbp_third_person_game_mode_2 "Game Over" 2.0)))))

(fn `Destroy Owning Actor & Associated Weapons`
  (bind _returnvalue (`self.GetOwner`))
  (`|ExecutionSequence`
    (:`then_0`
      (bind _weapon_parent (message `/Game/Combat/Interfaces/BPI_Has_Weapon.Get_Equipped_Melee_Weapon` _returnvalue))
      (`/Engine/EditorBlueprintResources/StandardMacros.IsValid` _weapon_parent
        (:`Is Valid`
          (`Actor.K2_DestroyActor` _weapon_parent))))
    (:`then_1`
      (bind _weapon_parent_2 (message `/Game/Combat/Interfaces/BPI_Has_Weapon.Get_Equipped_Ranged_Weapon` _returnvalue))
      (`/Engine/EditorBlueprintResources/StandardMacros.IsValid` _weapon_parent_2
        (:`Is Valid`
          (`Actor.K2_DestroyActor` _weapon_parent_2))))
    (:`then_2`
      (`Actor.K2_DestroyActor` (`self.GetOwner`)))))

(fn `Finish Revive`)

(fn `Heal`
  (params (`Amount To Heal` :type "Float (double-precision)"))
  (set `self.Current Health` (`KismetMathLibrary.FClamp` (+ (`self.Current Health`) `Amount To Heal`) 0.0 (`self.Maximum Health`))))

(fn `Start Revive`
  (params (PlayerLocation :type "Vector Structure"))
  (locals (OverlappingActors :type "Array of Actor Object Reference"))
  (bind _returnvalue (`Actor.GetComponentByClass` (`.ReturnValue` (`GameplayStatics.FindNearestActor` PlayerLocation (`local.OverlappingActors`))) "BPC_Health_V2_C"))
  (`KismetArrayLibrary.Array_Clear` (`local.OverlappingActors`))
  (bind (_outhits _returnvalue_2) (`KismetSystemLibrary.SphereTraceMultiForObjects` :`Start` PlayerLocation :`End` PlayerLocation :`Radius` 100.0 :`ObjectTypes` (`|MakeArray` "ObjectTypeQuery7" :!type "EObjectTypeQuery Enum") :`DrawDebugType` "ForDuration"))
  (if _returnvalue_2
    (for _array_element _outhits
      (bind (_bblockinghit _binitialoverlap _time _distance _location _impactpoint _normal _impactnormal _physmat _hitactor) (`GameplayStatics.BreakHitResult` _array_element))
      (if (not (== _hitactor (`self.GetOwner`)))
        (`KismetArrayLibrary.Array_Add` (`local.OverlappingActors`) _hitactor)))
    (for _array_element_2 (`local.OverlappingActors`)
      (if (not (`/Game/Health/Components/BPC_Health_V2.Downed` (`Actor.GetComponentByClass` _array_element_2 "BPC_Health_V2_C")))
        (`KismetArrayLibrary.Array_RemoveItem` (`local.OverlappingActors`) _array_element_2)))
    (if (`KismetArrayLibrary.Array_IsEmpty` (`local.OverlappingActors`))
      _
      (elif (`/Game/Health/Components/BPC_Health_V2.Downed` _returnvalue)
        (`self.Heal` _returnvalue (/ (`/Game/Health/Components/BPC_Health_V2.Maximum Health` _returnvalue) 2.0))
        (set `/Game/Health/Components/BPC_Health_V2.DownedTransition` true _returnvalue)
        (set `/Game/Health/Components/BPC_Health_V2.Downed` false _returnvalue)))))

(fn `Take Damage`
  (params (`Damage To Take` :type "Float (double-precision)") (`Damage Dealer` :type "Actor Object Reference") (`Direction Normal Of Damage` :type "Vector Structure") (`Location Of Damage` :type "Vector Structure") (`Knockback Strength Horizontal` :type "Float (double-precision)") (`Knockback Strength Vertical` :type "Float (double-precision)"))
  (bind _returnvalue (`Actor.GetComponentByClass` (`self.GetOwner`) "/Game/Combat/Components/BPC_In_Combat_Checker.BPC_In_Combat_Checker_C"))
  (bind _returnvalue_2 (`KismetSystemLibrary.DoesImplementInterface` (`self.GetOwner`) "/Game/Player/Interfaces/BPI_Player.BPI_Player_C"))
  (bind (_returnvalue_x _returnvalue_y) (`KismetMathLibrary.BreakVector` (* (`KismetMathLibrary.GetForwardVector` (`KismetMathLibrary.FindLookAtRotation` (`local.Location Of Damage`) (`Actor.K2_GetActorLocation` (`self.GetOwner`)))) (`local.Knockback Strength Horizontal`))))
  (bind _returnvalue_3 (- (`self.Current Health`) (`KismetMathLibrary.SelectFloat` (* `Damage To Take` 0.25) (`KismetMathLibrary.SelectFloat` (* `Damage To Take` 0.5) (`KismetMathLibrary.SelectFloat` (* `Damage To Take` 0.75) `Damage To Take` (and (`KismetSystemLibrary.DoesImplementInterface` (`self.GetOwner`) "/Game/Enemies/Interfaces/BPI_Enemy.BPI_Enemy_C") (`KismetSystemLibrary.DoesImplementInterface` `Damage Dealer` "/Game/Enemies/Interfaces/BPI_Enemy.BPI_Enemy_C"))) (and _returnvalue_2 (`KismetSystemLibrary.DoesImplementInterface` `Damage Dealer` "/Game/Player/Interfaces/BPI_Player.BPI_Player_C"))) (`/Game/Movement/Roll/Components/BPC_Roll.Rolling` (`Actor.GetComponentByClass` (`self.GetOwner`) "/Game/Movement/Roll/Components/BPC_Roll.BPC_Roll_C")))))
  (bind _returnvalue_4 (`KismetMathLibrary.FClamp` _returnvalue_3 0.0 (`self.Maximum Health`)))
  (`KismetSystemLibrary.PrintString` (`KismetStringLibrary.Conv_BoolToString` _returnvalue_2))
  (`GameplayStatics.PlayWorldCameraShake` "/Game/Health/BPs/BP_Take_Damage_Camera_Shake.BP_Take_Damage_Camera_Shake_C" (`Actor.K2_GetActorLocation` (`self.GetOwner`)) 0.0 9600.0)
  (`GameplayStatics.PlaySoundAtLocation` "/Game/VFX/Blood_Splatter/Audio/Impact_Audio/Body_Impact_SC.Body_Impact_SC" (`Actor.K2_GetActorLocation` (`self.GetOwner`)) (struct) 2.0 1.0 0.0 "/Game/VFX/Blood_Splatter/Audio/SA_Blood.SA_Blood" null null null)
  (`/Game/VFX/Blood_Splatter/BPS/BPC_Blood_Effect.Blood_Effect` (`Actor.GetComponentByClass` (`self.GetOwner`) "/Game/VFX/Blood_Splatter/BPS/BPC_Blood_Effect.BPC_Blood_Effect_C") (`Actor.K2_GetActorLocation` (`self.GetOwner`)) (`local.Direction Normal Of Damage`) (`self.GetOwner`) (`local.Damage To Take`))
  (`/Game/VFX/Blood_Splatter/BPS/BPC_Blood_Effect.Blood_Effect` (`Actor.GetComponentByClass` (`self.GetOwner`) "/Game/VFX/Blood_Splatter/BPS/BPC_Blood_Effect.BPC_Blood_Effect_C") (`Actor.K2_GetActorLocation` (`self.GetOwner`)) (* (`local.Direction Normal Of Damage`) -1.0) (`self.GetOwner`) (`local.Damage To Take`))
  (bind _ascharacter (cast `Character` (`self.GetOwner`)))
  (`Character.LaunchCharacter` _ascharacter (`KismetMathLibrary.MakeVector` _returnvalue_x _returnvalue_y (`local.Knockback Strength Vertical`)) true true)
  (bind _asbp_third_person_game_mode (cast `/Game/Modes_Instances/Modes/BP_ThirdPersonGameMode` (`GameplayStatics.GetGameMode`)))
  (`/Game/UI/HUD/Widgets/WBP_HUD.Play Hit Animation` (`/Game/Modes_Instances/Modes/BP_ThirdPersonGameMode.HUD Ref` _asbp_third_person_game_mode) (`KismetArrayLibrary.Array_Find` (`/Game/Modes_Instances/Modes/BP_ThirdPersonGameMode.Players` _asbp_third_person_game_mode) (`self.GetOwner`)))
  (if (<= _returnvalue_3 0.0)
    (if (not (or (`self.DownedTransition`) (`self.Downed`)))
      (set `self.Current Health` _returnvalue_4)
      (`self.Death` (`local.Damage Dealer`)))
    (else
      (set `self.Current Health` _returnvalue_4)
      (if (`KismetSystemLibrary.DoesImplementInterface` (`self.GetOwner`) "/Game/Enemies/Interfaces/BPI_Boss.BPI_Boss_C")
        (bind _asbp_third_person_game_mode_2 (cast `/Game/Modes_Instances/Modes/BP_ThirdPersonGameMode` (`GameplayStatics.GetGameMode`)))
        (`/Game/UI/HUD/Widgets/WBP_HUD.Play Boss Hit Animation` (`/Game/Modes_Instances/Modes/BP_ThirdPersonGameMode.HUD Ref` _asbp_third_person_game_mode_2))
        (bind _enemy_info (message `/Game/Enemies/Interfaces/BPI_Enemy.Get Enemy Info` (`self.GetOwner`)))
        (if (<= (`self.Current Health`) (* (`self.Maximum Health`) (`.BOSS-PercentageHealthPhase2_32_3F9D2E2F41A3AFFDCBF44797F6B08EF4` (break `/Game/Enemies/Structs_Tables/Struct_Enemy_Info` _enemy_info))))
          (message `/Game/Enemies/Interfaces/BPI_Boss.Activate 2nd Phase` (`self.GetOwner`)))
        (else
          (`/Engine/EditorBlueprintResources/StandardMacros.IsValid` _returnvalue
            (:`Is Valid`
              (`/Game/Combat/Components/BPC_In_Combat_Checker.Delay In Combat Reset` _returnvalue))))))))