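; Health component for the escort payload that tracks damage and healing and triggers game over when the payload is destroyed.
; TakeDamage halves damage from BPI_Player dealers, plays camera shake, sound and HUD hit feedback, and delays the owner's in-combat reset.
; Each hit also slows BP_Payload temporarily, with duration and speed multiplier scaled by damage.
; At zero health, PayloadDestroyed stops the payload and calls the game mode's Game Over on a timer.
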(event `self.ReceiveBeginPlay`
  (set `self.MaximumHealth` 500.0)
  (set `self.CurrentHealth` 500.0))

(fn `Heal`
  (params (`Amount To Heal` :type "Float (double-precision)"))
  (set `self.CurrentHealth` (`KismetMathLibrary.FClamp` (+ (`self.CurrentHealth`) `Amount To Heal`) 0.0 (`self.MaximumHealth`))))

(fn `PayloadDestroyed`
  (`GameplayStatics.PlaySoundAtLocation` "/Game/_UE_Content/StarterContent/Audio/Explosion01.Explosion01" (`Actor.K2_GetActorLocation` (`self.GetOwner`)) (struct) 1.0 1.0 0.0 null null null null)
  (bind _asbp_payload (cast `/Game/Co-op/Payload/BP_Payload` (`self.GetOwner`)))
  (`/Game/Co-op/Payload/BP_Payload.Slow Payload` _asbp_payload false 0.0 0.0)
  (bind _asbp_third_person_game_mode (cast `/Game/Modes_Instances/Modes/BP_ThirdPersonGameMode` (`GameplayStatics.GetGameMode`)))
  (`KismetSystemLibrary.K2_SetTimer` _asbp_third_person_game_mode "Game Over" 2.0))

(fn `TakeDamage`
  (params (`Damage to take` :type "Float (double-precision)") (`Damage Dealer` :type "Actor Object Reference"))
  (bind _returnvalue (/ `Damage to take` 5.0))
  (bind _returnvalue_2 (`Actor.GetComponentByClass` (`self.GetOwner`) "/Game/Combat/Components/BPC_In_Combat_Checker.BPC_In_Combat_Checker_C"))
  (bind _returnvalue_3 (`Actor.K2_GetActorLocation` (`self.GetOwner`)))
  (bind _returnvalue_4 (- (`self.CurrentHealth`) (`KismetMathLibrary.SelectFloat` (* `Damage to take` 0.5) `Damage to take` (`KismetSystemLibrary.DoesImplementInterface` `Damage Dealer` "/Game/Player/Interfaces/BPI_Player.BPI_Player_C"))))
  (`|ExecutionSequence`
    (:`then_0`
      (`GameplayStatics.PlayWorldCameraShake` "/Game/Health/BPs/BP_Take_Damage_Camera_Shake.BP_Take_Damage_Camera_Shake_C" _returnvalue_3 0.0 9600.0)
      (`GameplayStatics.PlaySoundAtLocation` "/Game/VFX/Blood_Splatter/Audio/Impact_Audio/Bone_Break_1.Bone_Break_1" _returnvalue_3 (struct) 2.0 1.0 0.0 "/Game/VFX/Blood_Splatter/Audio/SA_Blood.SA_Blood" null null null)
      (bind _asbp_third_person_game_mode (cast `/Game/Modes_Instances/Modes/BP_ThirdPersonGameMode` (`GameplayStatics.GetGameMode`)))
      (`/Game/UI/HUD/Widgets/WBP_HUD.Play Payload Hit Animation` (`/Game/Modes_Instances/Modes/BP_ThirdPersonGameMode.HUD Ref` _asbp_third_person_game_mode))
      (if (<= _returnvalue_4 0.0)
        (set `self.CurrentHealth` _returnvalue_4)
        (`self.PayloadDestroyed`)
        (else
          (set `self.CurrentHealth` _returnvalue_4)))
      (`/Engine/EditorBlueprintResources/StandardMacros.IsValid` _returnvalue_2
        (:`Is Valid`
          (`/Game/Combat/Components/BPC_In_Combat_Checker.Delay In Combat Reset` _returnvalue_2))))
    (:`then_1`
      (bind _asbp_payload (cast `/Game/Co-op/Payload/BP_Payload` (`self.GetOwner`)))
      (`/Game/Co-op/Payload/BP_Payload.Slow Payload` _asbp_payload true _returnvalue (/ _returnvalue 10.0)))))