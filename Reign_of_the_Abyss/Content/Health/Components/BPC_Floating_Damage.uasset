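; Health component that shows floating damage numbers as Niagara effects at a given world location.
; MakeFloatingNumber floors the damage and spawns one NS_Floating_Numbers_FX per character, stopping at the decimal point.
; Each digit gets its texture through a Niagara parameter and a sideways offset, with size and spacing scaled by clamped damage.
; All digits share a random colour and roll, and take their yaw from BP_Camera.
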(fn `Make_Floating_Number`
  (params (Location :type "Vector Structure") (Damage_Amount :type "Float (double-precision)"))
  (locals (Digit_System :type "NiagaraComponent Object Reference") (Text_Offset :type "Float (double-precision)" :default 0.0) (Random_Roll :type "Float (double-precision)") (Random_Colour :type "LinearColor Structure"))
  (bind _returnvalue (`KismetMathLibrary.FFloor` Damage_Amount))
  (bind _returnvalue_2 (/ (`KismetMathLibrary.Conv_IntToDouble` _returnvalue) 15))
  (bind _returnvalue_3 (`KismetMathLibrary.FClamp` _returnvalue_2 0.5 25.0))
  (set `local.Random_Roll` (`KismetMathLibrary.RandomFloatInRange` -25.0 25.0))
  (set `local.Random_Colour` (make `LinearColor` (`KismetMathLibrary.RandomFloat`) (`KismetMathLibrary.RandomFloat`) (`KismetMathLibrary.RandomFloat`) 0.8))
  (bind _returnvalue_4 (`GameplayStatics.GetActorOfClass` "/Game/Co-op/Camera/BP_Camera.BP_Camera_C"))
  (for _array_element (`KismetStringLibrary.GetCharacterArrayFromString` (`KismetStringLibrary.Conv_DoubleToString` (`KismetMathLibrary.Conv_IntToDouble` _returnvalue)))
    (if (`KismetStringLibrary.EqualEqual_StrStr` _array_element ".")
      (break)
      (else
        (bind (_returnvalue_roll _returnvalue_pitch _returnvalue_yaw) (`KismetMathLibrary.BreakRotator` (`SceneComponent.K2_GetComponentRotation` (`/Game/Co-op/Camera/BP_Camera.Camera` _returnvalue_4))))
        (bind _returnvalue_5 (`NiagaraFunctionLibrary.SpawnSystemAtLocation` "/Game/VFX/Damage_Niumber/NS_Floating_Numbers_FX.NS_Floating_Numbers_FX" Location (`KismetMathLibrary.MakeRotator` (`local.Random_Roll`) 180.0 _returnvalue_yaw) (`KismetMathLibrary.MakeVector` _returnvalue_3 (`KismetMathLibrary.FClamp` _returnvalue_2 0.5 25.0) (`KismetMathLibrary.FClamp` _returnvalue_2 0.5 25.0))))
        (set `local.Digit_System` _returnvalue_5)
        (`SceneComponent.K2_AddLocalOffset` (`local.Digit_System`) (`KismetMathLibrary.MakeVector` 0.0 (`local.Text_Offset`)) false false)
        (`NiagaraComponent.SetVariableLinearColor` (`local.Digit_System`) "user.Damage_Colour" (`local.Random_Colour`))
        (set `local.Text_Offset` (+ (`local.Text_Offset`) (* 30.0 _returnvalue_3)))
        (switch `string` _array_element
          (:`0`
            (`NiagaraFunctionLibrary.SetTextureObject` (`local.Digit_System`) "user.Digit" "/Game/VFX/Damage_Niumber/Digits/0.0"))
          (:`1`
            (`NiagaraFunctionLibrary.SetTextureObject` (`local.Digit_System`) "user.Digit" "/Game/VFX/Damage_Niumber/Digits/1.1"))
          (:`2`
            (`NiagaraFunctionLibrary.SetTextureObject` (`local.Digit_System`) "user.Digit" "/Game/VFX/Damage_Niumber/Digits/2.2"))
          (:`3`
            (`NiagaraFunctionLibrary.SetTextureObject` (`local.Digit_System`) "user.Digit" "/Game/VFX/Damage_Niumber/Digits/3.3"))
          (:`4`
            (`NiagaraFunctionLibrary.SetTextureObject` (`local.Digit_System`) "user.Digit" "/Game/VFX/Damage_Niumber/Digits/4.4"))
          (:`5`
            (`NiagaraFunctionLibrary.SetTextureObject` (`local.Digit_System`) "user.Digit" "/Game/VFX/Damage_Niumber/Digits/5.5"))
          (:`6`
            (`NiagaraFunctionLibrary.SetTextureObject` (`local.Digit_System`) "user.Digit" "/Game/VFX/Damage_Niumber/Digits/6.6"))
          (:`7`
            (`NiagaraFunctionLibrary.SetTextureObject` (`local.Digit_System`) "user.Digit" "/Game/VFX/Damage_Niumber/Digits/7.7"))
          (:`8`
            (`NiagaraFunctionLibrary.SetTextureObject` (`local.Digit_System`) "user.Digit" "/Game/VFX/Damage_Niumber/Digits/8.8"))
          (:`9`
            (`NiagaraFunctionLibrary.SetTextureObject` (`local.Digit_System`) "user.Digit" "/Game/VFX/Damage_Niumber/Digits/9.9"))
          (:`.`
            (`NiagaraFunctionLibrary.SetTextureObject` (`local.Digit_System`) "user.Digit" "/Game/VFX/Damage_Niumber/Digits/_._")))))))