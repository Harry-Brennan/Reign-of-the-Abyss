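; BPC_Health is an actor component that tracks current and maximum health for its owner.
; On BeginPlay it pulls starting and maximum values from the owner through a GetHealthInfoMessage call.
; TakeDamage subtracts damage without clamping, prints the result and calls Death at zero or below; dealer and direction inputs are unused.
; Death only prints a debug string, while Heal, StartRevive and FinishRevive are empty stubs.
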(event `self.ReceiveBeginPlay`
  (bind _health_info (message `/Game/Health/Interfaces/BPI_Has_Health.Get Health Info` (`self.GetOwner`)))
  (bind _output_get (set `self.Owner Health Info` _health_info))
  (bind (_startinghealth _maximumhealth) (break `/Game/Health/Structs_Tables/Struct_Health_Info` _output_get))
  (set `self.Current Health` _startinghealth)
  (set `self.Maximum Health` _maximumhealth))

(fn `Death`
  (`KismetSystemLibrary.PrintString` "DEATH"))

(fn `Finish Revive`)

(fn `Heal`
  (params (`Amount To Heal` :type "Float (double-precision)")))

(fn `Start Revive`)

(fn `Take Damage`
  (params (`Damage To Take` :type "Float (double-precision)") (`Damage Dealer` :type "Actor Object Reference") (`Direction Normal Of Damage` :type "Vector Structure"))
  (bind _returnvalue (- (`self.Current Health`) `Damage To Take`))
  (`KismetSystemLibrary.PrintString` (`KismetStringLibrary.Conv_DoubleToString` _returnvalue))
  (if (<= _returnvalue 0.0)
    (set `self.Current Health` _returnvalue)
    (`self.Death`)
    (else
      (set `self.Current Health` _returnvalue))))